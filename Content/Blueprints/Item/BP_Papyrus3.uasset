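; BP_Papyrus3 is a one-time papyrus pickup for the player, identified by the item key "Papyrus3".
; On BeginPlay it destroys itself if RXGameInstance already records that key as acquired.
; When RXPlayer overlaps its Box, it increments the game instance's papyrus count and marks the key acquired.
; It then shows a WBP_PopupNewItem with a Korean or non-Korean image variant chosen by IsKorean, and destroys itself.
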(event `self.ReceiveBeginPlay`
  (bind _asrxgame_instance (cast `RXGameInstance` (`GameplayStatics.GetGameInstance`)))
  (if (`RXGameInstance.IsItemStatusAcquired` _asrxgame_instance "Papyrus3")
    (`self.K2_DestroyActor`)))

(event `self.Box.OnComponentBeginOverlap`
  (params (OverlappedComponent :type "PrimitiveComponent Object Reference") (OtherActor :type "Actor Object Reference") (OtherComp :type "PrimitiveComponent Object Reference") (OtherBodyIndex :type Integer) (bFromSweep :type Boolean) (SweepResult :type "HitResult Structure (by ref)"))
  ;[1 1 1] 플레이어 트리거시 게임인스턴스 파피루스 갯수 증가
  (cast `RXPlayer` OtherActor)
  (bind _asrxgame_instance (cast `RXGameInstance` (`GameplayStatics.GetGameInstance`)))
  (`/Engine/EditorBlueprintResources/StandardMacros.IncrementInt` (`RXGameInstance.AcquiredPapyrusNum` _asrxgame_instance)
    (:`  `
      (`RXGameInstance.SetItemStatusAcquired` _asrxgame_instance "Papyrus3")
      (bind _returnvalue (`|CreateWidget` "/Game/UI/Popup/WBP_PopupNewItem.WBP_PopupNewItem_C"))
      (`UserWidget.AddToViewport` _returnvalue 0)
      (bind _asrxgame_instance_2 (cast `RXGameInstance` (`GameplayStatics.GetGameInstance`)))
      (if (`RXGameInstance.bIsKorean` _asrxgame_instance_2)
        (`/Game/UI/Popup/WBP_PopupNewItem.SetImageWithItemType` _returnvalue "NewEnumerator27")
        (else
          (`/Game/UI/Popup/WBP_PopupNewItem.SetImageWithItemType` _returnvalue "NewEnumerator28")))
      (`self.K2_DestroyActor`))))

(fn `UserConstructionScript`)
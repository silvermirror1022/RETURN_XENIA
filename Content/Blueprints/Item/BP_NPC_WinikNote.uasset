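; BP_NPC_WinikNote is the NPC logic at Winik's house that gives the player the HintPaper note once.
; On BeginPlay it destroys itself if RXGameInstance already records HintPaper as acquired.
; DialoguePopupEvent shows the new-item widget, marks HintPaper acquired, picks the widget image by the IsKorean language flag, then destroys the actor immediately.
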(event `self.ReceiveBeginPlay`
  ;[1 1 1] 위닉집 노트주는 로직 : 힌트페이퍼있으면 걍 파괴
  (bind _asrxgame_instance (cast `RXGameInstance` (`GameplayStatics.GetGameInstance`)))
  (if (`RXGameInstance.IsItemStatusAcquired` _asrxgame_instance "HintPaper")
    (`self.K2_DestroyActor`)))

(event `self.DialoguePopupEvent`
  (bind _newitemwidget (`self.NewItemWidget`))
  ;[1 1 1] 추가 대화 후 사라지는 이벤트 페이드 후 디스트로이엑터 구현
  (bind _asrxgame_instance (cast `RXGameInstance` (`GameplayStatics.GetGameInstance`)))
  (`UserWidget.AddToViewport` (`self.NewItemWidget`) 0)
  (`RXGameInstance.SetItemStatusAcquired` _asrxgame_instance "HintPaper")
  (if (`RXGameInstance.bIsKorean` _asrxgame_instance)
    (`/Game/UI/Popup/WBP_PopupNewItem.SetImageWithItemType` _newitemwidget "NewEnumerator4")
    (else
      (`/Game/UI/Popup/WBP_PopupNewItem.SetImageWithItemType` _newitemwidget "NewEnumerator5")))
  (`self.K2_DestroyActor`))

(fn `UserConstructionScript`)
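; Water volume that switches the player between swimming and falling, with underwater audio and a breath gauge widget.
; Overlapping the underwater box starts the swim state, and overlapping the upper box ends it, acting as paired enter/exit triggers.
; While inside, Tick reapplies swim mode, toggles the physics volume's water flag on and uses a hardcoded world height to signal treading versus diving.
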(event `SetPlayerSwimMode`
  (bind _charactermovement (`Character.CharacterMovement` (`self. RXPlayer`)))
  (`CharacterMovementComponent.SetMovementMode` _charactermovement "MOVE_Swimming" 0)
  (set `PhysicsVolume.bWaterVolume` true (`MovementComponent.GetPhysicsVolume` _charactermovement)))

(event `self.ReceiveBeginPlay`
  (bind _asrxplayer (cast `RXPlayer` (`GameplayStatics.GetPlayerCharacter` 0)))
  (set `self. RXPlayer` _asrxplayer))

(event `SetPlayerWalkMode`
  (bind _charactermovement (`Character.CharacterMovement` (`self. RXPlayer`)))
  (`CharacterMovementComponent.SetMovementMode` _charactermovement "MOVE_Falling" 0)
  (set `PhysicsVolume.bWaterVolume` false (`MovementComponent.GetPhysicsVolume` _charactermovement)))

(event `self.ReceiveTick`
  (params (DeltaSeconds :type "Float (single-precision)"))
  (bind __rxplayer (`self. RXPlayer`))
  (bind (_returnvalue_x _returnvalue_y _returnvalue_z) (`KismetMathLibrary.BreakVector` (`self.K2_GetActorLocation` (`self. RXPlayer`))))
  (if (`self.IsPlayerInWaterVolume`)
    (`self.SetPlayerSwimMode`)
    (if (> _returnvalue_z 7540.0)
      (set `RXPlayer.bIsThreadingWater` true __rxplayer)
      (`self.PlayerThreadingWater`)
      (else
        (set `RXPlayer.bIsThreadingWater` false __rxplayer)
        (`self.PlayerDivingWater`)))))

(event `self.UnderWaterBox.OnComponentBeginOverlap`
  (params (OverlappedComponent :type "PrimitiveComponent Object Reference") (OtherActor :type "Actor Object Reference") (OtherComp :type "PrimitiveComponent Object Reference") (OtherBodyIndex :type Integer) (bFromSweep :type Boolean) (SweepResult :type "HitResult Structure (by ref)"))
  (cast `RXPlayer` OtherActor)
  (set `self.IsPlayerInWaterVolume` true)
  (`AudioComponent.Play` (`self.SFX_UnderWater`) 0.0)
  (`GameplayStatics.PlaySound2D` "/Game/Audio/SFX/Player/SFX_Footstep_Water2.SFX_Footstep_Water2" 1.0 1.0 0.0 null null)
  (if (not (`self.IsUIGenerated`))
    (bind _returnvalue (`|CreateWidget` "/Game/UI/WBP_BreatheGauge.WBP_BreatheGauge_C" (`GameplayStatics.GetPlayerController` 0)))
    (`UserWidget.AddToViewport` _returnvalue 0)
    (set `self.IsUIGenerated` true)))

(event `self.UpperWaterBox.OnComponentBeginOverlap`
  (params (OverlappedComponent :type "PrimitiveComponent Object Reference") (OtherActor :type "Actor Object Reference") (OtherComp :type "PrimitiveComponent Object Reference") (OtherBodyIndex :type Integer) (bFromSweep :type Boolean) (SweepResult :type "HitResult Structure (by ref)"))
  (cast `RXPlayer` OtherActor)
  (if (`self.IsPlayerInWaterVolume`)
    (set `self.IsPlayerInWaterVolume` false)
    (`self.SetPlayerWalkMode`)
    (`GameplayStatics.PlaySound2D` "/Game/Audio/SFX/Player/SFX_Footstep_Water2.SFX_Footstep_Water2" 1.0 1.0 0.0 null null)
    (`AudioComponent.Stop` (`self.SFX_UnderWater`))
    (set `RXPlayer.bIsThreadingWater` false (`self. RXPlayer`))
    (`Widget.RemoveFromParent` (stale `self.UnderWaterBox.OnComponentBeginOverlap` _returnvalue))
    (set `self.IsUIGenerated` false)))

(fn `UserConstructionScript`)
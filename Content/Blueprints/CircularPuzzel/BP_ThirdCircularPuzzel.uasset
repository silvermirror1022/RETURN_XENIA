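; Third circular puzzle, where the player selects and rotates outer, middle and inner wheels to reach a correct answer.
; Starting it swaps Enhanced Input contexts, disables player movement and shows fade and notify widgets, extending parent puzzle events.
; Selection highlights a wheel by material; timelines lerp each 36-degree turn, guarded by IsRotating, alongside a player pulling animation.
; Solving records completion in BP_GameInstance, restores controls and removes interaction, which BeginPlay also removes if already solved.
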(event `ResetAllWheelColor`
  ;[1 1 1] 모든 휠 색 초기화
  (`PrimitiveComponent.SetMaterial` (`self.SM_Inner`) 0 (`self.OriginalMaterial`))
  (`PrimitiveComponent.SetMaterial` (`self.SM_Outer`) 0 (`self.OriginalMaterial`))
  (`PrimitiveComponent.SetMaterial` (`self.SM_Middle`) 0 (`self.OriginalMaterial`)))

(event `EnablePlayerInput`
  (bind _asbp_player (cast `/Game/Blueprints/Player/BP_Player` (`GameplayStatics.GetPlayerCharacter` 0)))
  (`CharacterMovementComponent.SetMovementMode` (`Character.CharacterMovement` _asbp_player) "MOVE_Walking" 0))

(event `ShowSelectedOuter`
  ;[1 1 1] 외곽 원판 퍼즐 선택 모드 함수
  (`PrimitiveComponent.SetMaterial` (`self.SM_Outer`) 0 "/Game/Material/puzzel/MI_QuipuPuzzle_B03.MI_QuipuPuzzle_B03")
  (`PrimitiveComponent.SetMaterial` (`self.SM_Inner`) 0 (`self.OriginalMaterial`))
  (`PrimitiveComponent.SetMaterial` (`self.SM_Middle`) 0 (`self.OriginalMaterial`)))

(event `DisablePlayerInput`
  (bind _asbp_player (cast `/Game/Blueprints/Player/BP_Player` (`GameplayStatics.GetPlayerCharacter` 0)))
  (`CharacterMovementComponent.SetMovementMode` (`Character.CharacterMovement` _asbp_player) "MOVE_None" 0))

(event `RotateOuterToCCW`
  (bind (_outercurrentrotation_roll _outercurrentrotation_pitch _outercurrentrotation_yaw) (`KismetMathLibrary.BreakRotator` (`self.OuterCurrentRotation`)))
  (bind _output_get (set `self.OuterTargetRotation` (`KismetMathLibrary.MakeRotator` 0.0 0.0 (+ _outercurrentrotation_yaw 36.0))))
  (bind (_direction _newtrack_0) (`Timeline|Timeline` :!via `PlayFromStart`)
    (:`Update`
      (`SceneComponent.K2_SetRelativeRotation` (`self.SM_Outer`) (`KismetMathLibrary.RLerp` (`SceneComponent.RelativeRotation` (`self.SM_Outer`)) (`self.OuterTargetRotation`) _newtrack_0 true) false false))
    (:`Finished`
      (set `self.OuterCurrentRotation` _output_get)
      (set `self.isRotating` false))))

(event `ShowSelectedMiddle`
  ;[1 1 1] 중간 원형 퍼즐 선택 모드 함수
  (`PrimitiveComponent.SetMaterial` (`self.SM_Middle`) 0 "/Game/Material/puzzel/MI_QuipuPuzzle_B03.MI_QuipuPuzzle_B03")
  (`PrimitiveComponent.SetMaterial` (`self.SM_Outer`) 0 (`self.OriginalMaterial`))
  (`PrimitiveComponent.SetMaterial` (`self.SM_Inner`) 0 (`self.OriginalMaterial`)))

(event `self.ReceiveBeginPlay`
  (bind _asbp_game_instance (cast `/Game/Blueprints/System/BP_GameInstance` (`GameplayStatics.GetGameInstance`)))
  (if (`RXGameInstance.IsPuzzelStatusAcquired` _asbp_game_instance "ThirdCircularPuzzel")
    (`self.DestroyComponents`)
    (else
      (bind _returnvalue (`|CreateWidget` "/Game/UI/WBP_FadeAnimWidget.WBP_FadeAnimWidget_C"))
      (set `self.FadeWidget` _returnvalue)
      (`self.ResetPuzzel`)
      (bind _asbp_player (cast `/Game/Blueprints/Player/BP_Player` (`GameplayStatics.GetPlayerCharacter` 0)))
      (bind _asabp_player (cast `/Game/Animation/Player/ABP_Player` (`SkeletalMeshComponent.GetAnimInstance` (`Character.Mesh` _asbp_player))))
      (set `self.PlayerABP` _asabp_player))))

(event `DestroyComponents`
  (`ActorComponent.K2_DestroyComponent` (`self.RXInteractionVisibility`))
  (`Widget.RemoveFromParent` (`self.FadeWidget`))
  (`Widget.RemoveFromParent` (`self.NotifyWidget`)))

(event `RotateMiddleToCCW`
  (bind (_middlecurrentrotation_roll _middlecurrentrotation_pitch _middlecurrentrotation_yaw) (`KismetMathLibrary.BreakRotator` (`self.MiddleCurrentRotation`)))
  (bind _output_get (set `self.MiddleTargetRotation` (`KismetMathLibrary.MakeRotator` 0.0 0.0 (+ _middlecurrentrotation_yaw 36.0))))
  (bind (_direction _newtrack_0) (`Timeline|Timeline_0` :!via `PlayFromStart`)
    (:`Update`
      (`SceneComponent.K2_SetRelativeRotation` (`self.SM_Middle`) (`KismetMathLibrary.RLerp` (`SceneComponent.RelativeRotation` (`self.SM_Middle`)) (`self.MiddleTargetRotation`) _newtrack_0 true) false false))
    (:`Finished`
      (set `self.MiddleCurrentRotation` _output_get)
      (set `self.isRotating` false))))

(event `ShowSelectedInner`
  ;[1 1 1] 안쪽 원형 퍼즐 선택 모드 함수
  (`PrimitiveComponent.SetMaterial` (`self.SM_Inner`) 0 "/Game/Material/puzzel/MI_QuipuPuzzle_B03.MI_QuipuPuzzle_B03")
  (`PrimitiveComponent.SetMaterial` (`self.SM_Middle`) 0 (`self.OriginalMaterial`))
  (`PrimitiveComponent.SetMaterial` (`self.SM_Outer`) 0 (`self.OriginalMaterial`)))

(event `self.RotateToClockWise`
  (if (not (`self.isRotating`))
    (`parent.RotateToClockWise`)
    (`/Game/UI/Puzzel/WBP_2NDCP_NotifyWidget.CWRotateWithChangingUI` (`self.NotifyWidget`))
    (set `self.isRotating` true)
    ;[1 1 1] 0 : outer, 1: middle, 2 : inner
    (switch `int` (`self.CurrentSelectedWheel`)
      (:`0`
        (`self.RotateOuterToCW`))
      (:`1`
        (`self.RotateMiddleToCW`))
      (:`2`
        (`self.RotateInnerToCW`)))
    (`self.PlayPlayerAnim`)
    (if (`self.IsCorrectAnswer`)
      (`KismetSystemLibrary.Delay` 0.8)
      (`self.PuzzelEventFinish`)
      (bind _asbp_game_instance (cast `/Game/Blueprints/System/BP_GameInstance` (`GameplayStatics.GetGameInstance`) :!label _label))
      (`RXGameInstance.SetPuzzelStatusAcquired` _asbp_game_instance "ThirdCircularPuzzel"))))

(event `self.SwitchSelectedWheel`
  ;[1 1 1] Tab을 통해 이동할 때마다 머터리얼 색 맞추어 변경하여 Focus
  (`parent.SwitchSelectedWheel`)
  (`/Game/UI/Puzzel/WBP_2NDCP_NotifyWidget.ChangeWheelWithUI` (`self.NotifyWidget`))
  ;;[1 1 1] 0 : outer, 1: middle, 2 : inner
  (switch `int` (`self.CurrentSelectedWheel`)
    (:`0`
      (`self.ShowSelectedOuter`))
    (:`1`
      (`self.ShowSelectedMiddle`))
    (:`2`
      (`self.ShowSelectedInner`))))

(event `RotateInnerToCCW`
  (bind (_innercurrentrotation_roll _innercurrentrotation_pitch _innercurrentrotation_yaw) (`KismetMathLibrary.BreakRotator` (`self.InnerCurrentRotation`)))
  (bind _output_get (set `self.InnerTargetRotation` (`KismetMathLibrary.MakeRotator` 0.0 0.0 (+ _innercurrentrotation_yaw 36.0))))
  (bind (_direction _newtrack_0) (`Timeline|Timeline_1` :!via `PlayFromStart`)
    (:`Update`
      (`SceneComponent.K2_SetRelativeRotation` (`self.SM_Inner`) (`KismetMathLibrary.RLerp` (`SceneComponent.RelativeRotation` (`self.SM_Inner`)) (`self.InnerTargetRotation`) _newtrack_0 true) false false))
    (:`Finished`
      (set `self.InnerCurrentRotation` _output_get)
      (set `self.isRotating` false))))

(event `ResetPuzzel`
  ;[1 1 1] 초기화 퍼즐 관련 변수들 리셋
  (`|ExecutionSequence`
    (:`then_0`
      (set `self.OuterCurrentRotation` (struct))
      (set `self.OuterTargetRotation` (struct))
      (`SceneComponent.K2_SetRelativeRotation` :`self` (`self.SM_Outer`)))
    (:`then_1`
      (set `self.CurrentSelectedWheel` 0)
      (set `self.MiddleCurrentRotation` (struct))
      (set `self.MiddleTargetRotation` (struct))
      (`SceneComponent.K2_SetRelativeRotation` :`self` (`self.SM_Middle`)))
    (:`then_2`
      (set `self.OuterIndex` 0))
    (:`then_3`
      (set `self.MiddleIndex` 0)
      (set `self.InnerCurrentRotation` (struct))
      (set `self.InnerTargetRotation` (struct))
      (`SceneComponent.K2_SetRelativeRotation` :`self` (`self.SM_Inner`)))
    (:`then_4`
      (set `self.InnerIndex` 0)
      (`self.ResetAllWheelColor`)
      (`Widget.RemoveFromParent` (`self.NotifyWidget`)))))

(event `self.RotateToCounterClockWise`
  (if (not (`self.isRotating`))
    (`parent.RotateToCounterClockWise`)
    (`/Game/UI/Puzzel/WBP_2NDCP_NotifyWidget.CCWRotateWithChangingUI` (`self.NotifyWidget`))
    (set `self.isRotating` true)
    ;[1 1 1] 0 : outer, 1: middle, 2 : inner
    (switch `int` (`self.CurrentSelectedWheel`)
      (:`0`
        (`self.RotateOuterToCCW`))
      (:`1`
        (`self.RotateMiddleToCCW`))
      (:`2`
        (`self.RotateInnerToCCW`)))
    (`self.PlayPlayerAnim`)
    (if (`self.IsCorrectAnswer`)
      (`KismetSystemLibrary.Delay` 0.8)
      (`self.PuzzelEventFinish`)
      (goto _label))))

(event `RotateOuterToCW`
  (bind (_outercurrentrotation_roll _outercurrentrotation_pitch _outercurrentrotation_yaw) (`KismetMathLibrary.BreakRotator` (`self.OuterCurrentRotation`)))
  (bind _output_get (set `self.OuterTargetRotation` (`KismetMathLibrary.MakeRotator` 0.0 0.0 (+ _outercurrentrotation_yaw -36.0))))
  (bind (_direction _newtrack_0) (`Timeline|Timeline_2` :!via `PlayFromStart`)
    (:`Update`
      (`SceneComponent.K2_SetRelativeRotation` (`self.SM_Outer`) (`KismetMathLibrary.RLerp` (`SceneComponent.RelativeRotation` (`self.SM_Outer`)) (`self.OuterTargetRotation`) _newtrack_0 true) false false))
    (:`Finished`
      (set `self.OuterCurrentRotation` _output_get)
      (set `self.isRotating` false))))

(event `self.PuzzelEventStart`
  (bind _fadewidget (`self.FadeWidget`))
  ;[1 1 1] 퍼즐모드 시작 : BlueprintNativeEvent
  (bind _asrxplayer_controller (cast `RXPlayerController` (`GameplayStatics.GetPlayerController` 0)))
  (`parent.PuzzelEventStart`)
  (bind _returnvalue (pcsubsystem `EnhancedInputLocalPlayerSubsystem` _asrxplayer_controller))
  (`EnhancedInputSubsystemInterface.RemoveMappingContext` _returnvalue "/Game/Input/IMC_Default.IMC_Default" (struct))
  ;[1 1 1] 컨트롤러 퍼즐전용으로 교체
  (`EnhancedInputSubsystemInterface.AddMappingContext` _returnvalue "/Game/Input/IMC_CircularPuzzel.IMC_CircularPuzzel" 0 (struct))
  ;[1 1 1] 페이드이벤트발생
  (`UserWidget.AddToViewport` _fadewidget 0)
  (`/Game/UI/WBP_FadeAnimWidget.PlayFadeOut` _fadewidget)
  (`self.DisablePlayerInput`)
  (`self.ShowSelectedOuter`)
  (`RXInteractionVisibilityComponent.SetVisibilityFalse` (`self.RXInteractionVisibility`))
  (`UserWidget.AddToViewport` (`self.NotifyWidget`) 0))

(event `self.MovePlayerLocation`
  (bind _returnvalue (`GameplayStatics.GetPlayerCharacter` 0))
  (`parent.MovePlayerLocation`)
  (`self.K2_SetActorLocationAndRotation` _returnvalue (`SceneComponent.K2_GetComponentLocation` (`self.PlayerPos`)) (`KismetMathLibrary.FindLookAtRotation` (`SceneComponent.K2_GetComponentLocation` (`Actor.RootComponent` _returnvalue)) (`SceneComponent.K2_GetComponentLocation` (`self.CenterPos`))) true true))

(event `RotateMiddleToCW`
  (bind (_middlecurrentrotation_roll _middlecurrentrotation_pitch _middlecurrentrotation_yaw) (`KismetMathLibrary.BreakRotator` (`self.MiddleCurrentRotation`)))
  (bind _output_get (set `self.MiddleTargetRotation` (`KismetMathLibrary.MakeRotator` 0.0 0.0 (+ _middlecurrentrotation_yaw -36.0))))
  (bind (_direction _newtrack_0) (`Timeline|Timeline_3` :!via `PlayFromStart`)
    (:`Update`
      (`SceneComponent.K2_SetRelativeRotation` (`self.SM_Middle`) (`KismetMathLibrary.RLerp` (`SceneComponent.RelativeRotation` (`self.SM_Middle`)) (`self.MiddleTargetRotation`) _newtrack_0 true) false false))
    (:`Finished`
      (set `self.MiddleCurrentRotation` _output_get)
      (set `self.isRotating` false))))

(event `self.PuzzelEventFinish`
  (bind _fadewidget (`self.FadeWidget`))
  ;[1 1 1] 퍼즐모드 해제 : BlueprintNativeEvent
  (bind _asrxplayer_controller (cast `RXPlayerController` (`GameplayStatics.GetPlayerController` 0)))
  (`parent.PuzzelEventFinish`)
  (bind _returnvalue (pcsubsystem `EnhancedInputLocalPlayerSubsystem` _asrxplayer_controller))
  (`EnhancedInputSubsystemInterface.RemoveMappingContext` _returnvalue "/Game/Input/IMC_CircularPuzzel.IMC_CircularPuzzel" (struct))
  (`EnhancedInputSubsystemInterface.AddMappingContext` _returnvalue "/Game/Input/IMC_Default.IMC_Default" 0 (struct))
  (`UserWidget.AddToViewport` _fadewidget 0)
  (`/Game/UI/WBP_FadeAnimWidget.PlayFadeOut` _fadewidget)
  (`self.EnablePlayerInput`)
  (`self.ResetPuzzel`)
  (`KismetSystemLibrary.Delay` 1.5)
  (`self.DestroyComponents`))

(event `RotateInnerToCW`
  (bind (_innercurrentrotation_roll _innercurrentrotation_pitch _innercurrentrotation_yaw) (`KismetMathLibrary.BreakRotator` (`self.InnerCurrentRotation`)))
  (bind _output_get (set `self.InnerTargetRotation` (`KismetMathLibrary.MakeRotator` 0.0 0.0 (+ _innercurrentrotation_yaw -36.0))))
  (bind (_direction _newtrack_0) (`Timeline|Timeline_4` :!via `PlayFromStart`)
    (:`Update`
      (`SceneComponent.K2_SetRelativeRotation` (`self.SM_Inner`) (`KismetMathLibrary.RLerp` (`SceneComponent.RelativeRotation` (`self.SM_Inner`)) (`self.InnerTargetRotation`) _newtrack_0 true) false false))
    (:`Finished`
      (set `self.InnerCurrentRotation` _output_get)
      (set `self.isRotating` false))))

(event `PlayPlayerAnim`
  (set `/Game/Animation/Player/ABP_Player.IsPulling` true (`self.PlayerABP`))
  (`KismetSystemLibrary.Delay` 1.0)
  (set `/Game/Animation/Player/ABP_Player.IsPulling` false (`self.PlayerABP`)))

(fn `UserConstructionScript`)
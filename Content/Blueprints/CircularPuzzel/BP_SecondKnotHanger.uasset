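; BP_SecondKnotHanger is a knot-hanger interactable in the circular puzzle that switches the player to a puzzle camera view when interacted with.
; Entering the view runs the parent logic, plays a fade-out, adds the knot widget and hides the interaction visibility.
; Returning to the player view runs the parent logic and restores that visibility.
; HangKnotAction, noted as a player input handler, is an empty stub.
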(event `self.ChangeToCamView`
  (bind _fadewidget (`self.Fadewidget`))
  ;[1 1 1] 플레이어가 E 인터렉션 할 경우 호출되는 함수
  (`parent.ChangeToCamView`)
  (`UserWidget.AddToViewport` _fadewidget 0)
  (`/Game/UI/WBP_FadeAnimWidget.PlayFadeOut` _fadewidget)
  (`UserWidget.AddToViewport` (`self.KnotWidget`) 0)
  (`RXInteractionVisibilityComponent.SetInteractionVisibility` (`self.RXInteractionVisibility`) false))

(event `self.HangKnotAction`
  ;[1 1 1] 상단에서 하단으로 플레이어 Q, B 버튼 인풋 함수
)

(event `self.ReturnToPlayerView`
  ;[1 1 1] 상단에서 하단으로 플레이어 Q, B 버튼 인풋 함수
  (`parent.ReturnToPlayerView`)
  (`RXInteractionVisibilityComponent.SetInteractionVisibility` (`self.RXInteractionVisibility`) true))

(fn `UserConstructionScript`)
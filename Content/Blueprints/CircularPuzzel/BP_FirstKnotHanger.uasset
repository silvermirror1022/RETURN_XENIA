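; First knot hanger puzzle actor, where the player interacts to enter a camera view and hang the tutorial knot.
; Camera view swaps the default Enhanced Input context for a knot-hanger one, shows fade and knot widgets, and reverses this on return.
; Hanging checks for the tutorial knot, consumes it, reveals a widget and records completion in RXGameInstance.
; On BeginPlay, a completed puzzle replaces itself with BP_EmptyKnotHanger.
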(event `self.ReceiveBeginPlay`
  (`parent.ReceiveBeginPlay`)
  (`SceneComponent.SetVisibility` (`self.Widget`) false false)
  (bind _asrxgame_instance (cast `RXGameInstance` (`GameplayStatics.GetGameInstance`)))
  (if (`RXGameInstance.IsPuzzelStatusAcquired` _asrxgame_instance "FirstKnotHanger")
    (`self.K2_DestroyActor`)
    (`|SpawnActorFromClass` "/Game/Blueprints/CircularPuzzel/BP_EmptyKnotHanger.BP_EmptyKnotHanger_C" (`self.GetTransform`) "Undefined" "MultiplyWithRoot" null null)))

(event `self.ChangeToCamView`
  (bind _fadewidget (`self.Fadewidget`))
  ;[1 1 1] 플레이어가 E 인터렉션 할 경우 호출되는 함수
  (`parent.ChangeToCamView`)
  (`UserWidget.AddToViewport` _fadewidget 0)
  (`/Game/UI/WBP_FadeAnimWidget.PlayFadeOut` _fadewidget)
  (`UserWidget.AddToViewport` (`self.KnotWidget`) 0)
  (`RXInteractionVisibilityComponent.SetInteractionVisibility` (`self.RXInteractionVisibility`) false)
  (`self.ChangeKnotHangPC`)
  (`KismetSystemLibrary.Delay` 1.5)
  (set `self.isCamView` true)
  (`GameplayStatics.PlaySound2D` "/Game/Audio/SFX/Puzzel/SFX_EventStart.SFX_EventStart" 1.0 1.0 0.0 null null))

(event `self.HangKnotAction`
  ;[1 1 1] 상단에서 하단으로 플레이어 Q, B 버튼 인풋 함수
  (`parent.HangKnotAction`)
  (bind _returnvalue (`self.IsAcquiredKnot_Tutorial`))
  (if _returnvalue
    (`GameplayStatics.PlaySound2D` "/Game/Audio/SFX/SFX_Interacted.SFX_Interacted" 1.0 1.0 0.0 null null)
    (`SceneComponent.SetVisibility` (`self.Widget`) true false)
    (bind _asrxgame_instance (cast `RXGameInstance` (`GameplayStatics.GetGameInstance`)))
    (`RXGameInstance.SetPuzzelStatusAcquired` _asrxgame_instance "FirstKnotHanger")
    (`self.UseKnotItem` "Tutorial")
    (`/Game/UI/Puzzel/WBP_KnotFirstHanger.ChangeQImageColor` (`self.KnotWidget`))
    (else
      (`GameplayStatics.PlaySound2D` "/Game/Audio/SFX/Puzzel/SFX_CannotIneract.SFX_CannotIneract" 1.0 1.0 0.0 null null))))

(event `self.ReturnToPlayerView`
  (bind _fadewidget (`self.Fadewidget`))
  ;[1 1 1] 상단에서 하단으로 플레이어 Q, B 버튼 인풋 함수
  (`parent.ReturnToPlayerView`)
  (`RXInteractionVisibilityComponent.SetInteractionVisibility` (`self.RXInteractionVisibility`) true)
  (`self.ReturnPC`)
  (`Widget.RemoveFromParent` (`self.KnotWidget`))
  (`UserWidget.AddToViewport` _fadewidget 0)
  (`/Game/UI/WBP_FadeAnimWidget.PlayFadeOut` _fadewidget))

(event `ChangeKnotHangPC`
  (bind _asrxplayer_controller (cast `RXPlayerController` (`GameplayStatics.GetPlayerController` 0)))
  (bind _returnvalue (pcsubsystem `EnhancedInputLocalPlayerSubsystem` _asrxplayer_controller))
  (`EnhancedInputSubsystemInterface.RemoveMappingContext` _returnvalue "/Game/Input/IMC_Default.IMC_Default" (struct))
  (`EnhancedInputSubsystemInterface.AddMappingContext` _returnvalue "/Game/Input/IMC_KnotHanger.IMC_KnotHanger" 0 (struct)))

(event `ReturnPC`
  (bind _asrxplayer_controller (cast `RXPlayerController` (`GameplayStatics.GetPlayerController` 0)))
  (bind _returnvalue (pcsubsystem `EnhancedInputLocalPlayerSubsystem` _asrxplayer_controller))
  (`EnhancedInputSubsystemInterface.RemoveMappingContext` _returnvalue "/Game/Input/IMC_KnotHanger.IMC_KnotHanger" (struct))
  (`EnhancedInputSubsystemInterface.AddMappingContext` _returnvalue "/Game/Input/IMC_Default.IMC_Default" 0 (struct)))

(fn `UserConstructionScript`)
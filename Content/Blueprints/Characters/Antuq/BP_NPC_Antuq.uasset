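; BP_NPC_Antuq is the Antuq NPC as it appears before its one-time dialogue event finishes.
; On BeginPlay it caches BP_GameInstance and destroys itself if IsAntuqDialogueEventFinished is already set, so it does not reappear on re-entry.
; DialoguePopupEvent, run when dialogue ends, sets that flag, spawns BP_NPC_Antuq_AfterEvent at the same transform and destroys this actor.
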(event `self.ReceiveBeginPlay`
  ;[1 1 1] 안XN크대화 인스턴스변수 처리 / 대화가 끝났으면 재진입시 엑터 파괴
  (bind _asbp_game_instance (cast `/Game/Blueprints/System/BP_GameInstance` (`GameplayStatics.GetGameInstance`)))
  (if (`RXGameInstance.bIsAntuqDialogueEventFinished` _asbp_game_instance)
    (`self.K2_DestroyActor`)))

(event `self.DialoguePopupEvent`
  ;[1 1 1] 대화가 끝났을 때 시퀀스 실행 노드
  (set `RXGameInstance.bIsAntuqDialogueEventFinished` true (stale `self.ReceiveBeginPlay` _asbp_game_instance))
  (`|SpawnActorFromClass` "/Game/Blueprints/Characters/Antuq/BP_NPC_Antuq_AfterEvent.BP_NPC_Antuq_AfterEvent_C" (`SceneComponent.K2_GetComponentToWorld` (`self.RootComponent`)) "AlwaysSpawn" "MultiplyWithRoot" null null)
  (`self.K2_DestroyActor`))

(fn `UserConstructionScript`)
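; Pachamama NPC in the boss battle whose dialogue popup event runs the game's ending sequence.
; It stops the boss music, then plays a video through BP_MediaPlayer, picked by the game instance's Korean-language flag.
; Holding exactly three papyri adds a second video, with fixed delays timing each one.
; Afterward it plays a fade widget, async-loads the main menu and opens that level.
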(event `self.DialoguePopupEvent`
  (bind _returnvalue (`GameplayStatics.GetActorOfClass` "/Game/Blueprints/ETC/BP_BossMusicPlayer.BP_BossMusicPlayer_C"))
  (`/Game/Blueprints/ETC/BP_BossMusicPlayer.StopMusic` _returnvalue)
  (bind _asrxgame_instance (cast `RXGameInstance` (`GameplayStatics.GetGameInstance`)))
  (bind _output_get (set `self.As RXGame Instance` _asrxgame_instance))
  (if (== (`RXGameInstance.AcquiredPapyrusNum` _output_get) 3)
    ;[1 1 1] 파피루스3->true / rest: false
    (bind _returnvalue_2 (`GameplayStatics.GetActorOfClass` "/Game/Blueprints/System/BP_MediaPlayer.BP_MediaPlayer_C"))
    (if (`RXGameInstance.bIsKorean` (`self.As RXGame Instance`))
      (`/Game/Blueprints/System/BP_MediaPlayer.PlayWithWidget` _returnvalue_2 "NewEnumerator4")
      (`KismetSystemLibrary.Delay` 84.0)
      (`/Game/Blueprints/System/BP_MediaPlayer.PlayWithWidget` _returnvalue_2 "NewEnumerator6")
      (`KismetSystemLibrary.Delay` 89.0)
      (`self.OpenMainMenu`)
      (else
        (`/Game/Blueprints/System/BP_MediaPlayer.PlayWithWidget` _returnvalue_2 "NewEnumerator5")
        (`KismetSystemLibrary.Delay` 84.0)
        (`/Game/Blueprints/System/BP_MediaPlayer.PlayWithWidget` _returnvalue_2 "NewEnumerator7")
        (`KismetSystemLibrary.Delay` 89.0)
        (`self.OpenMainMenu`)))
    (else
      (bind _returnvalue_3 (`GameplayStatics.GetActorOfClass` "/Game/Blueprints/System/BP_MediaPlayer.BP_MediaPlayer_C"))
      (if (`RXGameInstance.bIsKorean` (`self.As RXGame Instance`))
        (`/Game/Blueprints/System/BP_MediaPlayer.PlayWithWidget` _returnvalue_3 "NewEnumerator4")
        (`KismetSystemLibrary.Delay` 84.0)
        (`self.OpenMainMenu`)
        (else
          (`/Game/Blueprints/System/BP_MediaPlayer.PlayWithWidget` _returnvalue_3 "NewEnumerator5")
          (`KismetSystemLibrary.Delay` 84.0)
          (`self.OpenMainMenu`))))))

(event `OpenMainMenu`
  (bind _returnvalue (`|CreateWidget` "/Game/UI/WBP_FadeAnimWidget.WBP_FadeAnimWidget_C"))
  (`UserWidget.AddToViewport` _returnvalue 0)
  (`/Game/UI/WBP_FadeAnimWidget.PlayFadeIn` _returnvalue)
  (`KismetSystemLibrary.Delay` 2.5)
  (bind _object (`|LoadAsset` "/Game/Maps/MainMenu.MainMenu")
    (:`Completed`
      (`GameplayStatics.OpenLevel` (`KismetStringLibrary.Conv_StringToName` (`KismetSystemLibrary.GetDisplayName` _object))))))

(fn `UserConstructionScript`
  (`parent.UserConstructionScript`))
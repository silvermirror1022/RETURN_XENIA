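; BP_TestNPC is a test NPC that the player can talk to inside a trigger volume.
; DialogueStartTrigger overlaps with RXPlayer track whether the player is in range, and leaving also clears the in-dialogue flag.
; While in range, IA_Interact calls StartDialogue and IA_Enter calls DisplayDialogue once dialogue is active; neither function is defined in this graph.
; IA_Interact also has "Hello" debug prints that ignore the trigger check.
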(event `EnhancedInput|/Game/Input/IA_Interact`
  (params (ActionValue :type Boolean) (ElapsedSeconds :type "Float (double-precision)") (TriggeredSeconds :type "Float (double-precision)") (InputAction :type "InputAction Object Reference" :default "/Game/Input/IA_Interact.IA_Interact"))
  (:`Triggered`
    (`KismetSystemLibrary.PrintString` "Hello"))
  (:`Started`
    (`KismetSystemLibrary.PrintString` "Hello")))

(event `self.ReceiveBeginPlay`
  (set `self.IsPlayerInTrigger` false)
  (set `self.IsPlayerOnDialogue` false))

(event `EnhancedInput|/Game/Input/IA_Interact`
  (params (ActionValue :type Boolean) (ElapsedSeconds :type "Float (double-precision)") (TriggeredSeconds :type "Float (double-precision)") (InputAction :type "InputAction Object Reference" :default "/Game/Input/IA_Interact.IA_Interact"))
  (:`Started`
    (if (`self.IsPlayerInTrigger`)
      (`self.StartDialogue`)
      (set `self.IsPlayerOnDialogue` true))))

(event `self.DialogueStartTrigger.OnComponentBeginOverlap`
  (params (OverlappedComponent :type "PrimitiveComponent Object Reference") (OtherActor :type "Actor Object Reference") (OtherComp :type "PrimitiveComponent Object Reference") (OtherBodyIndex :type Integer) (bFromSweep :type Boolean) (SweepResult :type "HitResult Structure (by ref)"))
  (cast `RXPlayer` OtherActor)
  (set `self.IsPlayerInTrigger` true))

(event `self.DialogueStartTrigger.OnComponentEndOverlap`
  (params (OverlappedComponent :type "PrimitiveComponent Object Reference") (OtherActor :type "Actor Object Reference") (OtherComp :type "PrimitiveComponent Object Reference") (OtherBodyIndex :type Integer))
  (cast `RXPlayer` OtherActor)
  (set `self.IsPlayerInTrigger` false)
  (set `self.IsPlayerOnDialogue` false))

(event `EnhancedInput|/Game/Input/IA_Enter`
  (params (ActionValue :type Boolean) (ElapsedSeconds :type "Float (double-precision)") (TriggeredSeconds :type "Float (double-precision)") (InputAction :type "InputAction Object Reference" :default "/Game/Input/IA_Enter.IA_Enter"))
  (:`Started`
    (if (and (`self.IsPlayerInTrigger`) (`self.IsPlayerOnDialogue`))
      (`self.DisplayDialogue` null))))

(fn `UserConstructionScript`)
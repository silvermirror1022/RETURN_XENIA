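; Post-disaster Amarka NPC that gives the player the Red Cloak through a one-time dialogue event.
; On BeginPlay it creates the item popup and destroys itself unless the disaster has happened and the event is unfinished.
; DialoguePopupEvent records completion and RedCloak acquisition in the game instance, then shows a Korean or alternate popup image.
; OnRemovedItemWidget disables input, fades, then async-loads and opens NoahHouse_AfterDisaster; the replacement-NPC spawn is unconnected.
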(event `OnRemovedItemWidget`
  (bind _fadewidget (`self.FadeWidget`))
  (`self.DisableInput` (`GameplayStatics.GetPlayerPawn` 0) (`GameplayStatics.GetPlayerController` 0))
  (`UserWidget.AddToViewport` _fadewidget 0)
  (`/Game/UI/WBP_FadeAnimWidget.PlayFadeIn` _fadewidget)
  (`KismetSystemLibrary.Delay` 2.5)
  (bind _object (`|LoadAsset` "/Game/Maps/BeforeMaps/NoahHouse_AfterDisaster.NoahHouse_AfterDisaster")
    (:`Completed`
      (`GameplayStatics.OpenLevel` (`KismetStringLibrary.Conv_StringToName` (`KismetSystemLibrary.GetDisplayName` _object))))))

(event `self.ReceiveBeginPlay`
  ;[1 1 1] 재앙후에 스폰해야할 엑터들은 변수확인후 재앙안일어났으면 파괴처리
  (bind _returnvalue (`|CreateWidget` "/Game/UI/Popup/WBP_PopupNewItem.WBP_PopupNewItem_C"))
  (bind _output_get (set `self.ItemWidget` _returnvalue))
  (add `/Game/UI/Popup/WBP_PopupNewItem.SpecialEvent` _output_get (`|CreateDelegate` :!event `OnRemovedItemWidget`))
  (bind _asbp_game_instance (cast `/Game/Blueprints/System/BP_GameInstance` (`GameplayStatics.GetGameInstance`)))
  ;[1 1 1] 망토 주는 이벤트가 끝나고 다시 들어왔을 경우 에대한 예외처리
  (if (`RXGameInstance.bIsAfterDisaster` _asbp_game_instance)
    (if (`RXGameInstance.bIsAmarkaDialogueItemEventFinished` _asbp_game_instance)
      (`self.K2_DestroyActor`))
    (else
      (`self.K2_DestroyActor`))))

(event `self.DialoguePopupEvent`
  (bind _itemwidget (`self.ItemWidget`))
  ;[1 1 1] 추가 망토 주는 이벤트 구현
  (bind _asrxgame_instance (cast `RXGameInstance` (`GameplayStatics.GetGameInstance`)))
  (set `RXGameInstance.bIsAmarkaDialogueItemEventFinished` true _asrxgame_instance)
  (`RXGameInstance.SetProfileStatusAcquired` _asrxgame_instance "RedCloak")
  (`UserWidget.AddToViewport` (`self.ItemWidget`) 0)
  (if (`RXGameInstance.bIsKorean` _asrxgame_instance)
    (`/Game/UI/Popup/WBP_PopupNewItem.SetImageWithItemType` _itemwidget "NewEnumerator8")
    (else
      (`/Game/UI/Popup/WBP_PopupNewItem.SetImageWithItemType` _itemwidget "NewEnumerator9"))))

(fn `UserConstructionScript`
  (`parent.UserConstructionScript`))
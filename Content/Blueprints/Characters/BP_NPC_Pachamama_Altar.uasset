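; Pachamama altar NPC whose dialogue event triggers the disaster transition to the NoahHouse_AfterDisaster level.
; DialoguePopupEvent, meant to fire when the Pachamama dialogue ends, plays a rock camera shake, an earthquake sound and a WBP_WhiteOut white-in.
; After a short delay it async-loads the level asset, then opens the level by the loaded asset's display name.
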(event `self.DialoguePopupEvent`
  (`PlayerCameraManager.StartCameraShake` :`self` (`GameplayStatics.GetPlayerCameraManager` 0) :`ShakeClass` "/Game/Blueprints/RockEvent/BP_CameraShake_Rock.BP_CameraShake_Rock_C" :`Scale` 2.0)
  (`GameplayStatics.PlaySound2D` "/Game/Audio/SFX/Boss/SFX_BossEarthquake.SFX_BossEarthquake" 1.0 1.0 0.0 null null)
  (bind _returnvalue (`|CreateWidget` "/Game/UI/Boss/WBP_WhiteOut.WBP_WhiteOut_C"))
  (`UserWidget.AddToViewport` _returnvalue 0)
  (`/Game/UI/Boss/WBP_WhiteOut.PlayWhiteIn` _returnvalue)
  (`KismetSystemLibrary.Delay` 1.0)
  ;[1 1 1] 파차 마마 대화 종료시 화이트 인& 지진 후 Mainmap_AfterDisaster Load
  (bind _object (`|LoadAsset` "/Game/Maps/BeforeMaps/NoahHouse_AfterDisaster.NoahHouse_AfterDisaster")
    (:`Completed`
      (`GameplayStatics.OpenLevel` (`KismetStringLibrary.Conv_StringToName` (`KismetSystemLibrary.GetDisplayName` _object))))))

(fn `UserConstructionScript`
  (`parent.UserConstructionScript`))
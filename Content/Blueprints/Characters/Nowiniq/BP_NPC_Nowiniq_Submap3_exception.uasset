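; Nowiniq NPC variant for Submap 3 that grants a knot character item and returns the player to the main map.
; It destroys itself on BeginPlay unless the PatternPuzzel status is already acquired.
; Its dialogue event records puzzle and item status in two GameInstance classes and shows a Korean or alternate item popup.
; Popup removal disables input, sets the exit teleport tag, fades, then async-loads and opens MainMap_1F_AfterDisaster.
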(event `OnRemovedItemWidget`
  ;[1 0.4896 0.4896] 뉴아이템팝업을 껐을 경우 실행된 이벤트 디스페쳐 바인딩 함수(DisableInput,Fadein,OpenLevel)
  (`self.DisableInput` (`GameplayStatics.GetPlayerCharacter` 0) (`GameplayStatics.GetPlayerController` 0))
  (`self.SetDestinationTag`)
  (`/Game/UI/WBP_FadeAnimWidget.PlayFadeIn` (`self.FadeWidget`))
  (`KismetSystemLibrary.Delay` 2.5)
  (bind _object (`|LoadAsset` "/Game/Maps/MainMaps/MainMap_1F_AfterDisaster.MainMap_1F_AfterDisaster")
    (:`Completed`
      (`GameplayStatics.OpenLevel` (`KismetStringLibrary.Conv_StringToName` (`KismetSystemLibrary.GetDisplayName` _object))))))

(event `self.ReceiveBeginPlay`
  (add `/Game/UI/Popup/WBP_PopupNewItem.SpecialEvent` (`self.NewItemWidget`) (`|CreateDelegate` :!event `OnRemovedItemWidget`))
  (bind _asbp_game_instance (cast `/Game/Blueprints/System/BP_GameInstance` (`GameplayStatics.GetGameInstance`)))
  (if (not (`RXGameInstance.IsPuzzelStatusAcquired` _asbp_game_instance "PatternPuzzel"))
    (`self.K2_DestroyActor`)))

(event `SetDestinationTag`
  (bind _asrxgame_instance (cast `RXGameInstance` (`GameplayStatics.GetGameInstance`)))
  (`RXGameInstance.SetDestinationTag` _asrxgame_instance (struct :`TagName` "Teleport.1stFloor.NoinikSecretarea.Exit")))

(event `self.DialoguePopupEvent`
  ;[1 1 1] 서브맵3 정령 매드문자 획득, 페이드 후 각각 서브맵 입구로 노아 스폰
  (bind _asbp_game_instance (cast `/Game/Blueprints/System/BP_GameInstance` (`GameplayStatics.GetGameInstance`)))
  (`RXGameInstance.SetPuzzelStatusAcquired` _asbp_game_instance "PatternPuzzel")
  (`UserWidget.AddToViewport` (`self.NewItemWidget`) 0)
  (bind _asrxgame_instance (cast `RXGameInstance` (`GameplayStatics.GetGameInstance`)))
  (`RXGameInstance.SetItemStatusAcquired` _asrxgame_instance "KnotChar1F_3")
  (if (`RXGameInstance.bIsKorean` _asrxgame_instance)
    (`/Game/UI/Popup/WBP_PopupNewItem.SetImageWithItemType` (`self.NewItemWidget`) "NewEnumerator14")
    (else
      (`/Game/UI/Popup/WBP_PopupNewItem.SetImageWithItemType` (`self.NewItemWidget`) "NewEnumerator15"))))

(fn `UserConstructionScript`)
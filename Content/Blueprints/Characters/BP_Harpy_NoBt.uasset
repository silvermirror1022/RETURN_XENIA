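; BP_Harpy_NoBt is a harpy character that wanders in the air around its spawn point while the player is undetected.
; Each Tick, a debug-drawn line trace checks for RXPlayer within DetectedDistance; detection only halts the wandering, as no chase is implemented.
; Otherwise it interpolates toward a freshly randomized point near home, falling back to home when a trace is blocked.
; Random values are re-rolled after that trace, and state-selection logic is unwired.
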(event `self.ReceiveBeginPlay`
  (set `self.HomeTrans` (`self.K2_GetActorLocation`)))

(event `self.ReceiveTick`
  (params (DeltaSeconds :type "Float (single-precision)"))
  ;[1 1 1] 플레이어를 감지(ture): Chase / 감지X(false) : Patrol or Idle
  (bind _isdetectedplayer (`self.IsDetectedPlayer`))
  (if (not _isdetectedplayer)
    (bind _newparam (`self.MakeRandomTrans`))
    (`self.K2_SetActorLocationAndRotation` (`KismetMathLibrary.VInterpTo` (`self.K2_GetActorLocation`) _newparam 0.1 0.1) (`KismetMathLibrary.RInterpTo` (`self.K2_GetActorRotation`) (`KismetMathLibrary.FindLookAtRotation` (`self.K2_GetActorLocation`) _newparam) 0.1 0.1))))

(fn `IsDetectedPlayer`
  (returns (IsDetectedPlayer :type Boolean))
  (bind _returnvalue (`GameplayStatics.GetActorOfClass` "/Game/Blueprints/Player/BP_RXPlayer.BP_RXPlayer_C"))
  (bind (_outhit _returnvalue_2) (`KismetSystemLibrary.LineTraceSingle` :`Start` (`self.K2_GetActorLocation`) :`End` (`self.K2_GetActorLocation` _returnvalue) :`TraceChannel` "TraceTypeQuery3" :`DrawDebugType` "ForDuration" :`DrawTime` 2.0))
  (if _returnvalue_2
    (bind (_bblockinghit _binitialoverlap _time _distance _location _impactpoint _normal _impactnormal _physmat _hitactor) (`GameplayStatics.BreakHitResult` _outhit))
    (cast `RXPlayer` _hitactor)
    (return (<= _distance (`self.DetectedDistance`)))))

(fn `MakeRandomTrans`
  (returns (NewParam :type "Vector Structure"))
  (bind _returnvalue (`KismetMathLibrary.RandomFloatInRange` 500.0 -500.0))
  (bind (_returnvalue_x _returnvalue_y _returnvalue_z) (`KismetMathLibrary.BreakVector` (`KismetMathLibrary.MakeVector` _returnvalue _returnvalue (`KismetMathLibrary.RandomFloatInRange` 250.0 -250.0))))
  (bind _returnvalue_2 (+ (`self.HomeTrans`) (`KismetMathLibrary.MakeVector` _returnvalue_x _returnvalue_y _returnvalue_z)))
  (bind (_outhit _returnvalue_3) (`KismetSystemLibrary.LineTraceSingle` (`self.K2_GetActorLocation`) _returnvalue_2 "TraceTypeQuery3"))
  (if _returnvalue_3
    (return (`self.HomeTrans`))
    (else
      (return _returnvalue_2))))

(fn `RandomState`
  (returns (HarpyState :type "/Game/Blueprints/Characters/E_HarpyState Enum"))
  (switch `int` (`KismetMathLibrary.RandomIntegerInRange` 0 3)))

(fn `UserConstructionScript`)
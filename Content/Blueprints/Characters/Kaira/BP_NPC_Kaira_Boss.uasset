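; Kaira boss NPC Blueprint, currently with no active logic of its own.
; Its DialoguePopupEvent and construction script are empty.
; Disconnected leftover nodes would show an item widget with an image chosen by the game instance's Korean-language flag, then play a fade-in after a short delay.
; A separate unconnected node stops camera shake.
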(event `self.DialoguePopupEvent`)

(fn `UserConstructionScript`)
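; BP_NPC_Kaira is the version of NPC Kaira present before the disaster and before her dialogue event completes.
; On BeginPlay it reads BP_GameInstance flags and destroys itself if the disaster has happened or the dialogue event is already finished.
; DialoguePopupEvent sets the finished flag, spawns BP_NPC_Kaira_AfterEvent at its own root transform, then destroys itself, swapping the NPC in place.
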(event `self.ReceiveBeginPlay`
  ;[1 1 1] 재앙후에 스폰해야할 엑터들은 변수확인후 재앙안일어났으면 파괴처리
  (bind _asbp_game_instance (cast `/Game/Blueprints/System/BP_GameInstance` (`GameplayStatics.GetGameInstance`)))
  (if (`RXGameInstance.bIsAfterDisaster` _asbp_game_instance)
    (`self.K2_DestroyActor`)
    (elif (`RXGameInstance.bIsKairaDialogueEventFinished` _asbp_game_instance)
      (`self.K2_DestroyActor`))))

(event `self.DialoguePopupEvent`
  ;[1 1 1] 대화가 끝났을 때 시퀀스 실행 노드
  (set `RXGameInstance.bIsKairaDialogueEventFinished` true (stale `self.ReceiveBeginPlay` _asbp_game_instance))
  (`|SpawnActorFromClass` "/Game/Blueprints/Characters/Kaira/BP_NPC_Kaira_AfterEvent.BP_NPC_Kaira_AfterEvent_C" (`SceneComponent.K2_GetComponentToWorld` (`self.RootComponent`)) "AlwaysSpawn" "MultiplyWithRoot" null null)
  (`self.K2_DestroyActor`))

(fn `UserConstructionScript`)
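; Kaira NPC for the top boss encounter that shows an item popup from a dialogue event and leads into the boss's dialogue.
; It creates the popup widget on BeginPlay with interaction visibility off, choosing its image by the GameInstance's Korean-language flag when shown.
; The popup's special event shakes the camera and starts BP_BossTalk dialogue as the player's detected NPC.
; The actor destroys itself when BP_Boss changes to phase 1.
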(event `self.DialoguePopupEvent`
  (`UserWidget.AddToViewport` (`self.ItemWidget`) 0)
  (bind _asbp_game_instance (cast `/Game/Blueprints/System/BP_GameInstance` (`GameplayStatics.GetGameInstance`)))
  (if (`RXGameInstance.bIsKorean` _asbp_game_instance)
    (`/Game/UI/Popup/WBP_PopupNewItem.SetImageWithItemType` (`self.ItemWidget`) "NewEnumerator2")
    (else
      (`/Game/UI/Popup/WBP_PopupNewItem.SetImageWithItemType` (`self.ItemWidget`) "NewEnumerator3"))))

(event `self.ReceiveBeginPlay`
  (`RXInteractionVisibilityComponent.SetInteractionVisibility` (`self.RXInteractionVisibility`) false)
  (bind _returnvalue (`|CreateWidget` "/Game/UI/Popup/WBP_PopupNewItem.WBP_PopupNewItem_C"))
  (bind _output_get (set `self.ItemWidget` _returnvalue))
  (add `/Game/UI/Popup/WBP_PopupNewItem.SpecialEvent` _output_get (delegate `BossDialogueStartFunc`))
  (bind _returnvalue_2 (`GameplayStatics.GetActorOfClass` "/Game/Blueprints/Boss/BP_Boss.BP_Boss_C"))
  (add `/Game/Blueprints/Boss/BP_Boss.ChangedToPhase1` _returnvalue_2 (delegate `DestroyActor`)))

(event `BossDialogueStartFunc`
  (`PlayerCameraManager.StartCameraShake` :`self` (`GameplayStatics.GetPlayerCameraManager` 0) :`ShakeClass` "/Game/Blueprints/Boss/BP_CameraShake.BP_CameraShake_C")
  (bind _asrxplayer (cast `RXPlayer` (`GameplayStatics.GetPlayerCharacter` 0)))
  (bind _returnvalue (`GameplayStatics.GetActorOfClass` "/Game/Blueprints/Boss/BP_BossTalk.BP_BossTalk_C"))
  (set `RXPlayer.DetectedNPC` _returnvalue _asrxplayer)
  (`self.StartDialogue` _returnvalue))

(event `DestroyActor`
  (`self.K2_DestroyActor`))

(fn `UserConstructionScript`)
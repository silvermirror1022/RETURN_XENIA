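; Kaira NPC Blueprint whose dialogue popup event stages the transition into a boss battle.
; The event disables player input and movement, then plays a camera shake, earthquake sound and white-out widget fade.
; It records the Kaira necklace as acquired in the game instance, waits briefly, then async-loads the BossStartBattle asset and opens that level by the loaded object's name.
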(event `self.DialoguePopupEvent`
  (bind _whiteoutwidget (`self.WhiteOutWidget`))
  (`self.DisableInput` (`GameplayStatics.GetPlayerPawn` 0) (`GameplayStatics.GetPlayerController` 0))
  (`PlayerCameraManager.StartCameraShake` :`self` (`GameplayStatics.GetPlayerCameraManager` 0) :`ShakeClass` "/Game/Blueprints/Boss/BP_CameraShake.BP_CameraShake_C")
  (`GameplayStatics.PlaySound2D` "/Game/Audio/SFX/Boss/SFX_BossEarthquake.SFX_BossEarthquake" 1.0 1.0 0.0 null null)
  (`UserWidget.AddToViewport` _whiteoutwidget 0)
  (`/Game/UI/Boss/WBP_WhiteOut.PlayWhiteIn` _whiteoutwidget)
  (`CharacterMovementComponent.SetMovementMode` (`Character.CharacterMovement` (`GameplayStatics.GetPlayerCharacter` 0)) "MOVE_None" 0)
  (bind _asrxgame_instance (cast `RXGameInstance` (`GameplayStatics.GetGameInstance`)))
  (`RXGameInstance.SetProfileStatusAcquired` _asrxgame_instance "Kaira_necklace")
  (`KismetSystemLibrary.Delay` 4.0)
  (bind _object (`|LoadAsset` "/Game/Maps/BossMaps/BossStartBattle.BossStartBattle")
    (:`Completed`
      (`GameplayStatics.OpenLevel` (`KismetStringLibrary.Conv_StringToName` (`KismetSystemLibrary.GetObjectName` _object))))))

(fn `UserConstructionScript`)
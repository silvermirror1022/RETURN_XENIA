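; Harpy enemy character that patrols a spline route, chases the player and attacks with fireballs.
; Tick, throttled to DetectSecond, uses a line trace's hit distance for detection, halting the timeline-driven patrol to chase when out of attack range.
; In range, it chains detect and attack montages, then spawns a player-targeting fireball.
; After an attack, losing detection sends it toward the spline actor's location, resuming patrol when close.
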(event `ReturnHomeSplineRoute`
  (`self.AddMovementInput` (`KismetMathLibrary.Normal` (- (`self.HomeLocation`) (`self.K2_GetActorLocation`))) (`self.ChasingSpeed`))
  (`self.K2_SetActorRotation` (`KismetMathLibrary.FindLookAtRotation` (`self.K2_GetActorLocation`) (`self.HomeLocation`))))

(event `self.ReceiveBeginPlay`
  (set `self.HomeLocation` (`self.K2_GetActorLocation` (`self.SplineRef`)))
  (`self.SetActorTickInterval` (`self.DetectSecond`)))

(event `StopSplineRoute`
  (bind _spline (`/Game/AI/Harpy/BP_SplineActor.Spline` (`self.SplineRef`)))
  (bind (_direction _move) (`Timeline|RotateTimeline` :!via `Stop` :!label _label)
    (:`Update`
      (bind _returnvalue (`KismetMathLibrary.Lerp` 0.0 (`SplineComponent.GetSplineLength` (`/Game/AI/Harpy/BP_SplineActor.Spline` (`self.SplineRef`))) _move))
      (`self.K2_SetActorTransform` (`KismetMathLibrary.MakeTransform` (`SplineComponent.GetLocationAtDistanceAlongSpline` _spline _returnvalue "World") (`SplineComponent.GetRotationAtDistanceAlongSpline` _spline _returnvalue "Local"))))))

(event `RotateSplineRoute`
  (`/Engine/EditorBlueprintResources/StandardMacros.IsValid` (`self.SplineRef`)
    (:`Is Valid`
      (`TimelineComponent.SetPlayRate` (`self.RotateTimeline`) (/ 1.0 (`self.TimeToComplete(InSeconds)`)))
      (goto _label))))

(event `self.ReceiveTick`
  (params (DeltaSeconds :type "Float (single-precision)"))
  (bind _mesh (`self.Mesh`))
  (bind _isdetectedplayer (`self.IsDetectedPlayer` (`self.DetectedDistance`)))
  (if _isdetectedplayer
    (bind _isinattackrange (`self.IsInAttackRange` (`self.AttackRange`)))
    (if _isinattackrange
      (if (not (`self.bAttacking`))
        (set `self.bAttacking` true)
        (`self.K2_SetActorRotation` (`KismetMathLibrary.FindLookAtRotation` (`self.K2_GetActorLocation`) (`self.K2_GetActorLocation` (`GameplayStatics.GetPlayerCharacter` 0))))
        (`|PlayMontage` _mesh "/Game/Animation/Harpy/AM_HarpyDetect.AM_HarpyDetect"
          (:`OnCompleted`
            (`|PlayMontage` _mesh "/Game/Animation/Harpy/AM_HarpyAttack.AM_HarpyAttack"
              (:`OnCompleted`
                (bind _returnvalue (`|SpawnActorFromClass` "/Game/Blueprints/Characters/Harpy/BP_HarpyFireball.BP_HarpyFireball_C" (`SceneComponent.K2_GetComponentToWorld` (`self.SpawnPos`)) "AlwaysSpawn" "MultiplyWithRoot" null null))
                (`/Game/Blueprints/Characters/Harpy/BP_HarpyFireball.RotateToTarget` _returnvalue)
                (set `self.bAttacking` false)
                (set `self.bIsAttacked` true))))))
      (else
        (`self.StopSplineRoute`)
        (`self.ChasePlayer` (`self.ChasingSpeed`))))
    (elif (`self.bIsAttacked`)
      (`self.ReturnHomeSplineRoute`)
      (bind _isreached_ (`self.Is Reached Patrol Pos`))
      (if _isreached_
        (`self.RotateSplineRoute`))
      (else
        (`self.RotateSplineRoute`)))))

(fn `ChasePlayer`
  (params (ChasingSpeed :type "Float (double-precision)"))
  (bind _normalizedirection (`self.GetPlayerDirection`))
  (`self.AddMovementInput` _normalizedirection ChasingSpeed)
  (`self.K2_SetActorRotation` (`KismetMathLibrary.FindLookAtRotation` (`self.K2_GetActorLocation`) (`self.K2_GetActorLocation` (`GameplayStatics.GetPlayerCharacter` 0)))))

(fn `GetPlayerDirection`
  (returns (NormalizeDirection :type "Vector Structure"))
  (return (`KismetMathLibrary.Normal` (- (`self.K2_GetActorLocation` (`GameplayStatics.GetPlayerCharacter` 0)) (`self.K2_GetActorLocation`)))))

(fn `GetPlayerDistance`
  (returns (PlayerDistance :type "Float (double-precision)"))
  (return (`KismetMathLibrary.VSize` (- (`self.K2_GetActorLocation` (`GameplayStatics.GetPlayerCharacter` 0)) (`self.K2_GetActorLocation`)))))

(fn `Is Reached Patrol Pos`
  (returns (`IsReached?` :type Boolean))
  (bind _returnvalue (`KismetMathLibrary.Vector_Distance` (`self.K2_GetActorLocation`) (`self.HomeLocation`)))
  (bind _returnvalue_2 (<= _returnvalue 30.0))
  (`KismetSystemLibrary.PrintText` (`KismetTextLibrary.Conv_BoolToText` _returnvalue_2))
  (`KismetSystemLibrary.PrintText` (`KismetTextLibrary.Conv_DoubleToText` _returnvalue "HalfToEven"))
  (return _returnvalue_2))

(fn `IsDetectedPlayer`
  (params (DetectedDistance :type "Float (double-precision)"))
  (returns (IsDetectedPlayer :type Boolean))
  (bind _outactors (`GameplayStatics.GetAllActorsOfClass` "BP_Harpy_C"))
  (bind _outhit (`KismetSystemLibrary.LineTraceSingle` (`self.K2_GetActorLocation`) (`self.K2_GetActorLocation` (`GameplayStatics.GetPlayerCharacter` 0)) "TraceTypeQuery3" false _outactors "ForDuration" true (struct :`R` 1.0 :`A` 1.0) (struct :`G` 1.0 :`A` 1.0) 2.0))
  (return (<= (`.Distance` (`GameplayStatics.BreakHitResult` _outhit)) DetectedDistance)))

(fn `IsInAttackRange`
  (params (AttackRange :type "Float (double-precision)"))
  (returns (IsInAttackRange :type Boolean))
  (bind _playerdistance (`self.GetPlayerDistance`))
  (return (<= _playerdistance AttackRange)))

(fn `UserConstructionScript`)
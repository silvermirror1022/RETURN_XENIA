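; Harpy character, built without a behavior tree going by its name, that flies along the spline of a BP_SplineActor found at BeginPlay.
; A timeline, rate-scaled by TimeToCompleteInSeconds, lerps distance along the spline and sets world location and local-space spline rotation.
; Line-trace player detection, random wandering and random state selection exist only as disconnected or unfinished experiments, so only the spline movement runs.
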(event `self.ReceiveBeginPlay`
  (bind _returnvalue (`GameplayStatics.GetActorOfClass` "/Game/Blueprints/Characters/Harpy/BP_SplineActor.BP_SplineActor_C"))
  (set `self.SplineRef` _returnvalue)
  (`self.RotateSplineRoute`))

(event `RotateSplineRoute`
  (bind _spline (`/Game/Blueprints/Characters/Harpy/BP_SplineActor.Spline` (`self.SplineRef`)))
  (`TimelineComponent.SetPlayRate` (`self.RotateTimeline`) (/ 1.0 (`self.TimeToComplete(InSeconds)`)))
  (bind (_direction _move) (`Timeline|RotateTimeline`)
    (:`Update`
      (bind _returnvalue (`KismetMathLibrary.Lerp` 0.0 (`SplineComponent.GetSplineLength` (`/Game/Blueprints/Characters/Harpy/BP_SplineActor.Spline` (`self.SplineRef`))) _move))
      (`self.K2_SetActorTransform` (`KismetMathLibrary.MakeTransform` (`SplineComponent.GetLocationAtDistanceAlongSpline` _spline _returnvalue "World") (`SplineComponent.GetRotationAtDistanceAlongSpline` _spline _returnvalue "Local"))))))

(event `self.ReceiveTick`
  (params (DeltaSeconds :type "Float (single-precision)")))

(fn `IsDetectedPlayer`
  (returns (IsDetectedPlayer :type Boolean))
  (bind _returnvalue (`GameplayStatics.GetActorOfClass` "/Game/Blueprints/Player/BP_RXPlayer.BP_RXPlayer_C"))
  (bind (_outhit _returnvalue_2) (`KismetSystemLibrary.LineTraceSingle` :`Start` (`self.K2_GetActorLocation`) :`End` (`self.K2_GetActorLocation` _returnvalue) :`TraceChannel` "TraceTypeQuery3" :`DrawDebugType` "ForDuration" :`DrawTime` 2.0))
  (if _returnvalue_2
    (bind (_bblockinghit _binitialoverlap _time _distance _location _impactpoint _normal _impactnormal _physmat _hitactor) (`GameplayStatics.BreakHitResult` _outhit))
    (cast `RXPlayer` _hitactor)
    (return (<= _distance (`self.DistanceAlongSpline`)))))

(fn `MakeRandomTrans`
  (returns (NewParam :type "Vector Structure"))
  (bind _returnvalue (`KismetMathLibrary.RandomFloatInRange` 500.0 -500.0))
  (bind (_returnvalue_x _returnvalue_y _returnvalue_z) (`KismetMathLibrary.BreakVector` (`KismetMathLibrary.MakeVector` _returnvalue _returnvalue (`KismetMathLibrary.RandomFloatInRange` 250.0 -250.0))))
  (bind _returnvalue_2 (+ (0.0 0.0 0.0) (`KismetMathLibrary.MakeVector` _returnvalue_x _returnvalue_y _returnvalue_z)))
  (bind (_outhit _returnvalue_3) (`KismetSystemLibrary.LineTraceSingle` (`self.K2_GetActorLocation`) _returnvalue_2 "TraceTypeQuery3"))
  (if _returnvalue_3
    (return (0.0 0.0 0.0))
    (else
      (return _returnvalue_2))))

(fn `RandomState`
  (returns (HarpyState :type "/Game/Blueprints/Characters/E_HarpyState Enum"))
  (switch `int` (`KismetMathLibrary.RandomIntegerInRange` 0 3)))

(fn `UserConstructionScript`)
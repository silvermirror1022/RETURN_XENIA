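; Harpy fireball projectile that damages the player or leaves fire where it hits scenery.
; On BeginPlay it aims its ProjectileMovement velocity once at the player's current position, with no further homing.
; Sphere overlap with BP_Player applies damage through RXPlayerStatComponent, while a StaticMeshActor overlap spawns BP_HarpySplineFire at the sweep location.
; Both hits play explosion effects and destroy the fireball; static meshes need overlap-enabled WorldStatic collision.
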(event `self.ReceiveBeginPlay`
  (`self.RotateToTarget`))

(event `RotateToTarget`
  (set `MovementComponent.Velocity` (* (`KismetMathLibrary.GetDirectionUnitVector` (`self.K2_GetActorLocation`) (`self.K2_GetActorLocation` (`GameplayStatics.GetPlayerCharacter` 0))) (`self.Speed`)) (`self.ProjectileMovement`)))

(event `self.Sphere.OnComponentBeginOverlap`
  (params (OverlappedComponent :type "PrimitiveComponent Object Reference") (OtherActor :type "Actor Object Reference") (OtherComp :type "PrimitiveComponent Object Reference") (OtherBodyIndex :type Integer) (bFromSweep :type Boolean) (SweepResult :type "HitResult Structure (by ref)"))
  (`|ExecutionSequence`
    (:`then_0`
      (bind _asbp_player (cast `/Game/Blueprints/Player/BP_Player` OtherActor))
      (`RXPlayerStatComponent.ApplyDamage` (`self.GetComponentByClass` _asbp_player "/Script/RETURN_XENIA.RXPlayerStatComponent") 1)
      (`GameplayStatics.SpawnEmitterAtLocation` "/Game/ImportedAsset/StarterContent/Particles/P_Explosion.P_Explosion" SweepResult_Location)
      (`GameplayStatics.PlaySoundAtLocation` "/Game/Audio/SFX/Boss/SFX_HitFire.SFX_HitFire" SweepResult_Location (struct) 1.0 1.0 0.0 null null null null)
      (`self.K2_DestroyActor`))
    (:`then_1`
      ;[1 1 1] 해당 스태틱메시 엑터가 Generate Overlap Event On, Collision Enabled, WorldStatic Object Type
      (cast `StaticMeshActor` OtherActor)
      (`GameplayStatics.SpawnEmitterAtLocation` "/Game/ImportedAsset/StarterContent/Particles/P_Explosion.P_Explosion" SweepResult_Location)
      (`|SpawnActorFromClass` "/Game/Blueprints/Characters/Harpy/BP_HarpySplineFire.BP_HarpySplineFire_C" (`KismetMathLibrary.MakeTransform` SweepResult_Location) "Undefined" "MultiplyWithRoot" null null)
      (`GameplayStatics.PlaySoundAtLocation` "/Game/Audio/SFX/Boss/SFX_HitFire.SFX_HitFire" SweepResult_Location (struct) 1.0 1.0 0.0 null null null null)
      (`self.K2_DestroyActor`))))

(fn `UserConstructionScript`)
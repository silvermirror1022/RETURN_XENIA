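; First-floor map transition portal that plays a cutscene of itself appearing when PlayPortalAppearance is called.
; The event disables player movement, plays a screen fade and switches the view to CameraActor.
; A timeline drives the mesh's world Z, with a rock-moving sound and camera shake at its start event.
; After completion and a short delay, it fades again, restores walking and player view, then calls DestroyBox on BP_PlayerTeleport1F.
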(event `self.ReceiveBeginPlay`)

(event `PlayPortalAppearance`
  (bind (_returnvalue_x _returnvalue_y) (`KismetMathLibrary.BreakVector` (`self.K2_GetActorLocation`)))
  (bind _fadewidget (`self.FadeWidget`))
  (bind _fadewidget_2 (`self.FadeWidget`))
  (`CharacterMovementComponent.SetMovementMode` (`Character.CharacterMovement` (`GameplayStatics.GetPlayerCharacter` 0)) "MOVE_None" 0)
  (`UserWidget.AddToViewport` _fadewidget 0)
  (`/Game/UI/WBP_FadeAnimWidget.PlayFadeOut` _fadewidget)
  (`PlayerController.SetViewTargetWithBlend` (`GameplayStatics.GetPlayerController` 0) (`self.CameraActor`) 0.0 "VTBlend_Linear" 0.0 false)
  (bind (_direction _vectortrack) (`Timeline|Timeline_2`)
    (:`Update`
      (`SceneComponent.K2_SetWorldLocation` (`self.StaticMesh`) (`KismetMathLibrary.MakeVector` _returnvalue_x _returnvalue_y (.z _vectortrack)) false false))
    (:`MovingCompleted`
      (`KismetSystemLibrary.Delay` 1.0)
      (`UserWidget.AddToViewport` _fadewidget_2 0)
      (`/Game/UI/WBP_FadeAnimWidget.PlayFadeOut` _fadewidget_2)
      (`CharacterMovementComponent.SetMovementMode` (`Character.CharacterMovement` (`GameplayStatics.GetPlayerCharacter` 0)) "MOVE_Walking" 0)
      (`PlayerController.SetViewTargetWithBlend` (`GameplayStatics.GetPlayerController` 0) (`GameplayStatics.GetPlayerCharacter` 0) 0.0 "VTBlend_Linear" 0.0 false)
      (bind _returnvalue (`GameplayStatics.GetActorOfClass` "/Game/Blueprints/Teleport/BP_PlayerTeleport1F.BP_PlayerTeleport1F_C"))
      (`/Game/Blueprints/Teleport/BP_PlayerTeleport1F.DestroyBox` _returnvalue))
    (:`MovingStart`
      (`GameplayStatics.PlaySound2D` "/Game/Audio/SFX/SFX_MoveRock.SFX_MoveRock" 1.0 1.0 0.0 null null)
      (`PlayerCameraManager.StartCameraShake` :`self` (`GameplayStatics.GetPlayerCameraManager` 0) :`ShakeClass` "/Game/Blueprints/Boss/BP_CameraShake.BP_CameraShake_C"))))

(fn `UserConstructionScript`)
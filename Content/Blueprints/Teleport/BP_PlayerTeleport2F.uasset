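; Player teleporter Blueprint that adds transition feedback to a level change handled by its C++ parent.
; The teleport event calls the parent, then shows a fade-in widget, blocks move input and branches on IsDoor for sound.
; The door branch plays a door-open sound, while the teleport branch has no sound assigned.
; A separate event destroys the Box component, and fade-out is left to each Level Blueprint.
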(event `DestroyBox`
  (`ActorComponent.K2_DestroyComponent` (`self.Box`)))

(event `self.TeleportToOtherLevel`
  ;[1 1 1] C++에서 BlueprintNativeEvent로 레벨전환은 C++ , Fade -> Blueprint Implementation
  (`parent.TeleportToOtherLevel`) ; fadeout은 각각 levelblueprint에서 설정해야함
  (bind _returnvalue (`|CreateWidget` "/Game/UI/WBP_FadeAnimWidget.WBP_FadeAnimWidget_C"))
  (`UserWidget.AddToViewport` _returnvalue 0)
  (`/Game/UI/WBP_FadeAnimWidget.PlayFadeIn` _returnvalue)
  (`Controller.SetIgnoreMoveInput` (`GameplayStatics.GetPlayerController` 0) true)
  (if (`self.IsDoor`)
    ;[1 1 1] true: 문소리/ false: 텔포소리
    (`GameplayStatics.PlaySound2D` "/Game/Audio/SFX/SFX_DoorOpen.SFX_DoorOpen" 1.0 1.0 0.0 null null)
    (else
      (`GameplayStatics.PlaySound2D` null 1.0 1.0 0.0 null null))))

(fn `UserConstructionScript`)
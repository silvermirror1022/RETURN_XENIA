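; Player teleporter to another level (Noah after disaster) that stays in the world only if the RedCloak profile status is acquired.
; Shortly after BeginPlay it checks RXGameInstance and destroys itself when that status is missing.
; On teleport it calls the parent C++ level transition, then plays a fade-in widget, locks player input and plays a door or teleport sound based on IsDoor.
; Fade-out is left to each level Blueprint.
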(event `self.ReceiveBeginPlay`
  (`KismetSystemLibrary.Delay` 0.2)
  (bind _asrxgame_instance (cast `RXGameInstance` (`GameplayStatics.GetGameInstance`)))
  (if (not (`RXGameInstance.IsProfileStatusAcquired` _asrxgame_instance "RedCloak"))
    (`self.K2_DestroyActor`)))

(event `self.TeleportToOtherLevel`
  (bind _returnvalue (`GameplayStatics.GetPlayerController` 0))
  ;[1 1 1] C++에서 BlueprintNativeEvent로 레벨전환은 C++ , Fade -> Blueprint Implementation
  (`parent.TeleportToOtherLevel`) ; fadeout은 각각 levelblueprint에서 설정해야함
  (bind _returnvalue_2 (`|CreateWidget` "/Game/UI/WBP_FadeAnimWidget.WBP_FadeAnimWidget_C"))
  (`UserWidget.AddToViewport` _returnvalue_2 0)
  (`/Game/UI/WBP_FadeAnimWidget.PlayFadeIn` _returnvalue_2)
  (`Controller.SetIgnoreMoveInput` _returnvalue true)
  (`self.DisableInput` (`GameplayStatics.GetPlayerCharacter` 0) _returnvalue)
  (if (`self.IsDoor`)
    ;[1 1 1] true: 문소리/ false: 텔포소리
    (`GameplayStatics.PlaySound2D` "/Game/Audio/SFX/SFX_DoorOpen.SFX_DoorOpen" 1.0 1.0 0.0 null null)
    (else
      (`GameplayStatics.PlaySound2D` "/Game/Audio/SFX/SFX_Teleport.SFX_Teleport" 1.0 1.0 0.0 null null))))

(fn `UserConstructionScript`)
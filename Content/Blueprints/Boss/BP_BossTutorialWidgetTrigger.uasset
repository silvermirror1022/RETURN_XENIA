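; Boss tutorial trigger volume that shows a boss skill guide widget the first time an RXPlayer overlaps its box.
; It switches on the game instance's AcquiredBossHintNum, mapping counts one through five to fixed hint images passed to WBP_BossSkillGuide.
; Any other count calls RandomShow, which picks one of the same five hints at random, intended for players who have died five or more times.
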(event `self.Box.OnComponentBeginOverlap`
  (params (OverlappedComponent :type "PrimitiveComponent Object Reference") (OtherActor :type "Actor Object Reference") (OtherComp :type "PrimitiveComponent Object Reference") (OtherBodyIndex :type Integer) (bFromSweep :type Boolean) (SweepResult :type "HitResult Structure (by ref)"))
  (cast `RXPlayer` OtherActor)
  (`/Engine/EditorBlueprintResources/StandardMacros.DoOnce` false
    (:`Completed`
      (bind _asrxgame_instance (cast `RXGameInstance` (`GameplayStatics.GetGameInstance`)))
      (switch `int` (`RXGameInstance.AcquiredBossHintNum` _asrxgame_instance)
        (:`Default`
          (`self.RandomShow`))
        (:`1`
          (bind _returnvalue (`|CreateWidget` "/Game/UI/Tutorial/WBP_BossSkillGuide.WBP_BossSkillGuide_C"))
          (`UserWidget.AddToViewport` _returnvalue 0)
          (`/Game/UI/Tutorial/WBP_BossSkillGuide.InitBossHintImage` _returnvalue "NewEnumerator4"))
        (:`2`
          (bind _returnvalue_2 (`|CreateWidget` "/Game/UI/Tutorial/WBP_BossSkillGuide.WBP_BossSkillGuide_C"))
          (`UserWidget.AddToViewport` _returnvalue_2 0)
          (`/Game/UI/Tutorial/WBP_BossSkillGuide.InitBossHintImage` _returnvalue_2 "NewEnumerator6"))
        (:`3`
          (bind _returnvalue_3 (`|CreateWidget` "/Game/UI/Tutorial/WBP_BossSkillGuide.WBP_BossSkillGuide_C"))
          (`UserWidget.AddToViewport` _returnvalue_3 0)
          (`/Game/UI/Tutorial/WBP_BossSkillGuide.InitBossHintImage` _returnvalue_3 "NewEnumerator2"))
        (:`4`
          (bind _returnvalue_4 (`|CreateWidget` "/Game/UI/Tutorial/WBP_BossSkillGuide.WBP_BossSkillGuide_C"))
          (`UserWidget.AddToViewport` _returnvalue_4 0)
          (`/Game/UI/Tutorial/WBP_BossSkillGuide.InitBossHintImage` _returnvalue_4 "NewEnumerator0"))
        (:`5`
          (bind _returnvalue_5 (`|CreateWidget` "/Game/UI/Tutorial/WBP_BossSkillGuide.WBP_BossSkillGuide_C"))
          (`UserWidget.AddToViewport` _returnvalue_5 0)
          (`/Game/UI/Tutorial/WBP_BossSkillGuide.InitBossHintImage` _returnvalue_5 "NewEnumerator8"))))))

(event `RandomShow`
  ;[1 1 1] 5번 이상 죽었을 때 랜덤으로 보스 가이드 UI
  (switch `int` (`KismetMathLibrary.RandomIntegerInRange` 1 5)
    (:`1`
      (bind _returnvalue (`|CreateWidget` "/Game/UI/Tutorial/WBP_BossSkillGuide.WBP_BossSkillGuide_C"))
      (`UserWidget.AddToViewport` _returnvalue 0)
      (`/Game/UI/Tutorial/WBP_BossSkillGuide.InitBossHintImage` _returnvalue "NewEnumerator4"))
    (:`2`
      (bind _returnvalue_2 (`|CreateWidget` "/Game/UI/Tutorial/WBP_BossSkillGuide.WBP_BossSkillGuide_C"))
      (`UserWidget.AddToViewport` _returnvalue_2 0)
      (`/Game/UI/Tutorial/WBP_BossSkillGuide.InitBossHintImage` _returnvalue_2 "NewEnumerator6"))
    (:`3`
      (bind _returnvalue_3 (`|CreateWidget` "/Game/UI/Tutorial/WBP_BossSkillGuide.WBP_BossSkillGuide_C"))
      (`UserWidget.AddToViewport` _returnvalue_3 0)
      (`/Game/UI/Tutorial/WBP_BossSkillGuide.InitBossHintImage` _returnvalue_3 "NewEnumerator2"))
    (:`4`
      (bind _returnvalue_4 (`|CreateWidget` "/Game/UI/Tutorial/WBP_BossSkillGuide.WBP_BossSkillGuide_C"))
      (`UserWidget.AddToViewport` _returnvalue_4 0)
      (`/Game/UI/Tutorial/WBP_BossSkillGuide.InitBossHintImage` _returnvalue_4 "NewEnumerator0"))
    (:`5`
      (bind _returnvalue_5 (`|CreateWidget` "/Game/UI/Tutorial/WBP_BossSkillGuide.WBP_BossSkillGuide_C"))
      (`UserWidget.AddToViewport` _returnvalue_5 0)
      (`/Game/UI/Tutorial/WBP_BossSkillGuide.InitBossHintImage` _returnvalue_5 "NewEnumerator8"))))

(fn `UserConstructionScript`)
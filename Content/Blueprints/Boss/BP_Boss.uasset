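; BP_Boss is the boss actor that tracks and broadcasts its combat phase as Sealed Stones are released.
; On BeginPlay it binds IncreasePhase to every BP_SealedStone, caches the fireball spawn manager, and starts in Phase1.
; Each unseal increments a counter from zero, so the first stays in Phase1 and later ones advance up to Phase4.
; Per-phase event dispatchers notify subscribers, and ReturnCurrentPhase exposes the current phase.
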(event `self.ReceiveBeginPlay`
  (bind _outactors (`GameplayStatics.GetAllActorsOfClass` "/Game/Blueprints/Boss/BP_SealedStone.BP_SealedStone_C"))
  (for _array_element _outactors
    (add `/Game/Blueprints/Boss/BP_SealedStone.UnsealStone` _array_element (delegate `IncreasePhase`))
    (set `self.CurrentPhaseNum` 0)
    (set `self.CurrentPhase` "Phase1")
    (bind _returnvalue (`GameplayStatics.GetActorOfClass` "/Game/Blueprints/Boss/AttackPattern/BP_BossFBSpawnManager.BP_BossFBSpawnManager_C"))
    (set `self.FireballSpawner` _returnvalue)
    (`self.ChangedToPhase1`)))

(event `IncreasePhase`
  ;[1 1 1] 봉인석 2개 해제시 2(CurrentPhase) 페이즈2시작 / 3->3
  (bind _result (`/Engine/EditorBlueprintResources/StandardMacros.IncrementInt` (`self.CurrentPhaseNum`))
    (:`  `
      (bind _output_get (set `self.CurrentPhaseNum` _result))
      (switch `int` _output_get
        (:`1`
          ;[1 1 1] 해당 이벤트 디스페처 구독시 페이즈 변화시 바인딩 함수 각각 Call
          (set `self.CurrentPhase` "Phase1")
          (`self.ChangedToPhase1`))
        (:`2`
          (set `self.CurrentPhase` "Phase2")
          (`self.ChangedToPhase2`))
        (:`3`
          (set `self.CurrentPhase` "Phase3")
          (`self.ChangedToPhase3`))
        (:`4`
          (set `self.CurrentPhase` "Phase4")
          (`self.ChangedToPhase4`))))))

(fn `ReturnCurrentPhase`
  (returns (Phase :type Name))
  (return (`self.CurrentPhase`)))

(fn `UserConstructionScript`)
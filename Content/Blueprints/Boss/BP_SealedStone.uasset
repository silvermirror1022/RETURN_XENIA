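; BP_SealedStone is a boss-fight seal stone that the player unseals by standing inside its trigger sphere.
; Overlap presses the button and runs a looping timer that raises ActivationLevel; leaving releases it and starts decay after a cooldown.
; The level lights six cells by material swap; full charge ends interaction, activates the referenced spline, calls UnsealStone, plays effects and spawns a healing potion.
; BP_Boss's phase 4 event stops its audio.
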(event `ActiveButton`
  ;[1 1 1] 버튼 누르는 Relative Location :  Animation Timeline
  (bind (_direction _btnheight) (`Timeline|Timeline` :!via `PlayFromStart`)
    (:`Update`
      (`SceneComponent.K2_SetRelativeLocation` (`self.SM_Button`) (`KismetMathLibrary.MakeVector` 0.0 0.0 (`KismetMathLibrary.Lerp` 0.0 -15.0 _btnheight)) false false))
    (:`Sound`
      (`GameplayStatics.PlaySound2D` "/Game/Audio/SFX/Boss/SFX_StoneTrigger.SFX_StoneTrigger" 1.0 1.0 0.0 null null))))

(event `UnSealCompleted`
  (bind (_returnvalue_x _returnvalue_y _returnvalue_z) (`KismetMathLibrary.BreakVector` (`self.K2_GetActorLocation`)))
  (bind (_returnvalue_x_2 _returnvalue_y_2 _returnvalue_z_2) (`KismetMathLibrary.BreakVector` (`self.K2_GetActorLocation`)))
  (bind (_returnvalue_roll _returnvalue_pitch _returnvalue_yaw) (`KismetMathLibrary.BreakRotator` (`self.K2_GetActorRotation`)))
  ;[1 1 1] 봉인해제시 이펙트 효과 함수
  (`self.DeactiveButton`)
  (set `self.IsCompleted` true)
  (`GameplayStatics.SpawnEmitterAtLocation` "/Game/InfinityBladeEffects/Effects/FX_Cines/Ausar/P_Ausar_Resurrection.P_Ausar_Resurrection" (`KismetMathLibrary.MakeVector` _returnvalue_x_2 _returnvalue_y_2 (- _returnvalue_z_2 4.0)) (struct) (0.6 0.6 0.6))
  (`KismetSystemLibrary.Delay` 8.0)
  (`GameplayStatics.SpawnEmitterAtLocation` "/Game/InfinityBladeEffects/Effects/FX_Mobile/combat/P_Charge_Target_Beam_Ice.P_Charge_Target_Beam_Ice" (`KismetMathLibrary.MakeVector` _returnvalue_x _returnvalue_y (+ _returnvalue_z 60.0)) (`KismetMathLibrary.MakeRotator` _returnvalue_roll (+ _returnvalue_pitch 90.0) _returnvalue_yaw)))

(event `DeactiveButton`
  ;[1 1 1] 버튼 누르는 Relative Location :  Animation Timeline
  (bind (_direction _btnheight) (`Timeline|Timeline_0` :!via `PlayFromStart`)
    (:`Update`
      (`SceneComponent.K2_SetRelativeLocation` (`self.SM_Button`) (`KismetMathLibrary.MakeVector` 0.0 0.0 (`KismetMathLibrary.Lerp` -15.0 0.0 _btnheight)) false false))))

(event `self.ReceiveBeginPlay`
  (set `self.ChangedMaterial` "/Game/Designer/Materials/puzzel/MI_SealedStone_A02.MI_SealedStone_A02")
  (set `self.OriginalMaterial` "/Game/Designer/Materials/puzzel/MI_SealedStone_A01.MI_SealedStone_A01")
  ;[1 1 1] 이펙트 비활성화
  (`ActorComponent.Deactivate` (`self.PS_ActivationState`))
  (bind _returnvalue (`GameplayStatics.GetActorOfClass` "/Game/Blueprints/Boss/BP_Boss.BP_Boss_C"))
  (add `/Game/Blueprints/Boss/BP_Boss.ChangedToPhase4` _returnvalue (delegate `StopStoneSound`)))

(event `StopStoneSound`
  ;[1 1 1] 이펙트 비활성화
  (`AudioComponent.Stop` (`self.Audio`)))

(event `IncreaseAL`
  (bind _refsplineactor (`self.RefSplineActor`))
  (bind _result (`/Engine/EditorBlueprintResources/StandardMacros.IncrementFloat` (`self.ActivationLevel`))
    (:`  `
      (set `self.ActivationLevel` (`KismetMathLibrary.FClamp` _result 0.0 100.0))
      (bind _newparam (`self.CheckActivationLevel` (`self.ActivationLevel`) :!label _label))
      (switch `name` _newparam
        (:`Gauge1`
          (`PrimitiveComponent.SetMaterial` (`self.SM_Cell1`) 0 (`self.ChangedMaterial`))
          (`PrimitiveComponent.SetMaterial` (`self.SM_Cell2`) 0 (`self.OriginalMaterial`))
          (`PrimitiveComponent.SetMaterial` (`self.SM_Cell4`) 0 (`self.OriginalMaterial`))
          (`PrimitiveComponent.SetMaterial` (`self.SM_Cell6`) 0 (`self.OriginalMaterial`))
          (`PrimitiveComponent.SetMaterial` (`self.SM_Cell5`) 0 (`self.OriginalMaterial`))
          (`PrimitiveComponent.SetMaterial` (`self.SM_Cell3`) 0 (`self.OriginalMaterial`)))
        (:`Gauge2`
          (`PrimitiveComponent.SetMaterial` (`self.SM_Cell2`) 0 (`self.ChangedMaterial`))
          (`PrimitiveComponent.SetMaterial` (`self.SM_Cell1`) 0 (`self.ChangedMaterial`))
          (`PrimitiveComponent.SetMaterial` (`self.SM_Cell3`) 0 (`self.OriginalMaterial`))
          (`PrimitiveComponent.SetMaterial` (`self.SM_Cell4`) 0 (`self.OriginalMaterial`))
          (`PrimitiveComponent.SetMaterial` (`self.SM_Cell6`) 0 (`self.OriginalMaterial`))
          (`PrimitiveComponent.SetMaterial` (`self.SM_Cell5`) 0 (`self.OriginalMaterial`)))
        (:`Gauge3`
          (`PrimitiveComponent.SetMaterial` (`self.SM_Cell3`) 0 (`self.ChangedMaterial`))
          (`PrimitiveComponent.SetMaterial` (`self.SM_Cell1`) 0 (`self.ChangedMaterial`))
          (`PrimitiveComponent.SetMaterial` (`self.SM_Cell2`) 0 (`self.ChangedMaterial`))
          (`PrimitiveComponent.SetMaterial` (`self.SM_Cell5`) 0 (`self.OriginalMaterial`))
          (`PrimitiveComponent.SetMaterial` (`self.SM_Cell4`) 0 (`self.OriginalMaterial`))
          (`PrimitiveComponent.SetMaterial` (`self.SM_Cell6`) 0 (`self.OriginalMaterial`)))
        (:`Gauge4`
          (`PrimitiveComponent.SetMaterial` (`self.SM_Cell4`) 0 (`self.ChangedMaterial`))
          (`PrimitiveComponent.SetMaterial` (`self.SM_Cell3`) 0 (`self.ChangedMaterial`))
          (`PrimitiveComponent.SetMaterial` (`self.SM_Cell2`) 0 (`self.ChangedMaterial`))
          (`PrimitiveComponent.SetMaterial` (`self.SM_Cell1`) 0 (`self.ChangedMaterial`))
          (`PrimitiveComponent.SetMaterial` (`self.SM_Cell5`) 0 (`self.OriginalMaterial`))
          (`PrimitiveComponent.SetMaterial` (`self.SM_Cell6`) 0 (`self.OriginalMaterial`)))
        (:`Gauge5`
          (`PrimitiveComponent.SetMaterial` (`self.SM_Cell5`) 0 (`self.ChangedMaterial`))
          (`PrimitiveComponent.SetMaterial` (`self.SM_Cell4`) 0 (`self.ChangedMaterial`))
          (`PrimitiveComponent.SetMaterial` (`self.SM_Cell3`) 0 (`self.ChangedMaterial`))
          (`PrimitiveComponent.SetMaterial` (`self.SM_Cell2`) 0 (`self.ChangedMaterial`))
          (`PrimitiveComponent.SetMaterial` (`self.SM_Cell1`) 0 (`self.ChangedMaterial`))
          (`PrimitiveComponent.SetMaterial` (`self.SM_Cell6`) 0 (`self.OriginalMaterial`)))
        (:`Gauge6`
          ;[1 1 1] 봉인석 해제 로직 HERE
          (`PrimitiveComponent.SetMaterial` (`self.SM_Cell6`) 0 (`self.ChangedMaterial`))
          (`PrimitiveComponent.SetMaterial` (`self.SM_Cell5`) 0 (`self.ChangedMaterial`))
          (`PrimitiveComponent.SetMaterial` (`self.SM_Cell4`) 0 (`self.ChangedMaterial`))
          (`PrimitiveComponent.SetMaterial` (`self.SM_Cell3`) 0 (`self.ChangedMaterial`))
          (`PrimitiveComponent.SetMaterial` (`self.SM_Cell2`) 0 (`self.ChangedMaterial`))
          (`PrimitiveComponent.SetMaterial` (`self.SM_Cell1`) 0 (`self.ChangedMaterial`))
          (`PrimitiveComponent.SetMaterial` (`self.SM_Structure`) 0 (`self.ChangedMaterial`))
          (`PrimitiveComponent.SetMaterial` (`self.SM_Button`) 0 (`self.ChangedMaterial`))
          (`ActorComponent.K2_DestroyComponent` (`self.Sphere`))
          (`KismetSystemLibrary.K2_ClearTimer` null "DecreaseAL")
          (`KismetSystemLibrary.K2_ClearTimer` null "CalculateCooldown")
          (`KismetSystemLibrary.K2_ClearTimer` null "IncreaseAL")
          ;[1 1 1] 봉인석 하나 클리어 로직 (사운드추가)
          ;;[1 1 1] 봉인석게이지 해제시 이펙트효과후 이벤트디스페쳐 바인딩 함수 호출 (Unseal Stone BP_Boss) Bind
          (`/Engine/EditorBlueprintResources/StandardMacros.IsValid` _refsplineactor
            (:`Is Valid`
              (`/Game/Blueprints/Boss/AttackPattern/RefBP/BP_SplineVFX_ElectricLightning.ActiveSpline` _refsplineactor)
              (`self.UnsealStone`)
              (`self.UnSealCompleted`)
              (`GameplayStatics.PlaySound2D` "/Game/Audio/SFX/Boss/SFX_UnsealStone.SFX_UnsealStone" 1.0 1.0 0.0 null null)
              (`KismetSystemLibrary.Delay` 2.0)
              ;[1 1 1] 체력회복 템 스폰
              (`|SpawnActorFromClass` "/Game/Blueprints/Item/BP_HealingPotion.BP_HealingPotion_C" (`SceneComponent.K2_GetComponentToWorld` (`self.ItemSpawnPos`)) "Undefined" "MultiplyWithRoot" null null))))))))

(event `DecreaseAL`
  (bind _result (`/Engine/EditorBlueprintResources/StandardMacros.DecrementFloat` (`self.ActivationLevel`))
    (:`  `
      (set `self.ActivationLevel` (`KismetMathLibrary.FClamp` _result 0.0 100.0))
      (goto _label))))

(event `self.Sphere.OnComponentBeginOverlap`
  (params (OverlappedComponent :type "PrimitiveComponent Object Reference") (OtherActor :type "Actor Object Reference") (OtherComp :type "PrimitiveComponent Object Reference") (OtherBodyIndex :type Integer) (bFromSweep :type Boolean) (SweepResult :type "HitResult Structure (by ref)"))
  (bind _ps_activationstate (`self.PS_ActivationState`))
  (if (not (`self.IsCompleted`))
    (cast `RXPlayer` OtherActor)
    (`KismetSystemLibrary.K2_ClearTimer` null "DecreaseAL")
    (`KismetSystemLibrary.K2_ClearTimer` null "CalculateCooldown")
    (`KismetSystemLibrary.K2_SetTimer` null "IncreaseAL" 0.5 true)
    (`SceneComponent.SetHiddenInGame` _ps_activationstate false false)
    (`ActorComponent.Activate` _ps_activationstate false)
    (`self.ActiveButton`)))

(event `self.Sphere.OnComponentEndOverlap`
  (params (OverlappedComponent :type "PrimitiveComponent Object Reference") (OtherActor :type "Actor Object Reference") (OtherComp :type "PrimitiveComponent Object Reference") (OtherBodyIndex :type Integer))
  (if (not (`self.IsCompleted`))
    (cast `RXPlayer` OtherActor)
    (`KismetSystemLibrary.K2_ClearTimer` null "IncreaseAL")
    (`KismetSystemLibrary.K2_SetTimerDelegate` (delegate `CalculateCooldown`) 5.0)
    (`SceneComponent.SetHiddenInGame` (`self.PS_ActivationState`) true false)
    (`self.DeactiveButton`)))

(event `CalculateCooldown`
  (`KismetSystemLibrary.K2_SetTimer` null "DecreaseAL" 0.5 true))

(fn `CheckActivationLevel`
  (params (ActivationLevel :type "Float (double-precision)"))
  (returns (NewParam :type Name))
  (switch `int` (`KismetMathLibrary.FTrunc` (/ ActivationLevel 16.0))
    (:`1`
      (return "Gauge1"))
    (:`2`
      (return "Gauge2"))
    (:`3`
      (return "Gauge3"))
    (:`4`
      (return "Gauge4"))
    (:`5`
      (return "Gauge5"))
    (:`6`
      (return "Gauge6"))))

(fn `UserConstructionScript`)
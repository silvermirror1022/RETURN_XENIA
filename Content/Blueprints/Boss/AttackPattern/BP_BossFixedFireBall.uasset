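; BP_BossFixedFireBall is a boss attack projectile, a fixed fireball that damages the player on overlap.
; Overlapping BP_Player applies 1 damage through its RXPlayerStatComponent, spawns an explosion emitter and destroys the fireball.
; A timer started on BeginPlay destroys it after six seconds otherwise.
; Phase 2 and 3 events set the ProjectileMovement initial and max speed, currently to identical values.
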(event `SetPhase2Velocity`
  (bind _projectilemovement (`self.ProjectileMovement`))
  ;[1 1 1] 페이즈마다 속도를 변경하는 함수
  (set `ProjectileMovementComponent.InitialSpeed` 2000.0 _projectilemovement)
  (set `ProjectileMovementComponent.MaxSpeed` 2000.0 _projectilemovement))

(event `SetPhase3Velocity`
  (bind _projectilemovement (`self.ProjectileMovement`))
  ;[1 1 1] 페이즈마다 속도를 변경하는 함수
  (set `ProjectileMovementComponent.InitialSpeed` 2000.0 _projectilemovement)
  (set `ProjectileMovementComponent.MaxSpeed` 2000.0 _projectilemovement))

(event `self.ReceiveBeginPlay`
  ;[1 1 1] 고정된 파이어볼
  (`KismetSystemLibrary.K2_SetTimerDelegate` (delegate `CustomEvent`) 6.0))

(event `CustomEvent`
  (`self.K2_DestroyActor`))

(event `self.Box.OnComponentBeginOverlap`
  (params (OverlappedComponent :type "PrimitiveComponent Object Reference") (OtherActor :type "Actor Object Reference") (OtherComp :type "PrimitiveComponent Object Reference") (OtherBodyIndex :type Integer) (bFromSweep :type Boolean) (SweepResult :type "HitResult Structure (by ref)"))
  (bind _asbp_player (cast `/Game/Blueprints/Player/BP_Player` OtherActor))
  (`RXPlayerStatComponent.ApplyDamage` (`self.GetComponentByClass` _asbp_player "/Script/RETURN_XENIA.RXPlayerStatComponent") 1)
  (`GameplayStatics.SpawnEmitterAtLocation` "/Game/ImportedAsset/StarterContent/Particles/P_Explosion.P_Explosion" (`self.K2_GetActorLocation`))
  (`self.K2_DestroyActor`))

(fn `UserConstructionScript`)
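; Boss-fight fire hazard that starts dormant, with Niagara effect, collision box and audio off.
; It binds to BP_Boss phase events, apparently switching on at phase 2, and destroys itself at phase 4.
; Players overlapping the box take damage, hear a hit sound and are launched randomly left or right of the fire's arrow direction.
; A Timeline for the Niagara "Progress" growth is present but never runs.
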(event `ActivateFire`
  (`ActorComponent.Activate` (`self.Niagara`) false)
  (`PrimitiveComponent.SetCollisionEnabled` (`self.Box`) "PhysicsOnly")
  (`AudioComponent.Play` (`self.Audio`) 0.0))

(event `self.ReceiveBeginPlay`
  (`|ExecutionSequence`
    (:`then_0`
      (`ActorComponent.Deactivate` (`self.Niagara`))
      (`PrimitiveComponent.SetCollisionEnabled` (`self.Box`) "NoCollision")
      (`AudioComponent.Stop` (`self.Audio`)))
    (:`then_1`
      ;[1 1 1] 페이즈 2 활성화시 보스 이벤트 디스페처 구독 (활성화)
      (bind _returnvalue (`GameplayStatics.GetActorOfClass` "/Game/Blueprints/Boss/BP_Boss.BP_Boss_C"))
      (add `/Game/Blueprints/Boss/BP_Boss.ChangedToPhase2` _returnvalue (`|CreateDelegate` :!event `ActivateFire`)))
    (:`then_2`
      ;[1 1 1] 페이즈 4 활성화 보스 이벤트 디스페처 구독 (파괴)
      (bind _returnvalue_2 (`GameplayStatics.GetActorOfClass` "/Game/Blueprints/Boss/BP_Boss.BP_Boss_C"))
      (add `/Game/Blueprints/Boss/BP_Boss.ChangedToPhase4` _returnvalue_2 (delegate `DestroyActor`)))))

(event `DestroyActor`
  ;[1 1 1] 페이즈 4 활성화 보스 이벤트 디스페처 구독 (파괴)
  (`self.K2_DestroyActor`))

(event `self.Box.OnComponentBeginOverlap`
  (params (OverlappedComponent :type "PrimitiveComponent Object Reference") (OtherActor :type "Actor Object Reference") (OtherComp :type "PrimitiveComponent Object Reference") (OtherBodyIndex :type Integer) (bFromSweep :type Boolean) (SweepResult :type "HitResult Structure (by ref)"))
  (bind _asbp_player (cast `/Game/Blueprints/Player/BP_Player` OtherActor))
  (`RXPlayerStatComponent.ApplyDamage` (`self.GetComponentByClass` _asbp_player "/Script/RETURN_XENIA.RXPlayerStatComponent") 1)
  ;[1 1 1] 렌덤으로 불길 기준 플레이어를 좌우로 밀어냄
  (bind _newparam (`self.GetRandomDirection`))
  (`Character.LaunchCharacter` (`GameplayStatics.GetPlayerCharacter` 0) (* _newparam 1500.0) true false)
  (`GameplayStatics.PlaySound2D` "/Game/Audio/SFX/Boss/SFX_HitFire.SFX_HitFire" 1.0 1.0 0.0 null null))

(fn `GetRandomDirection`
  (returns (NewParam :type "Vector Structure"))
  ;[1 1 1] 불길에 닿았을 때 랜덤 왼쪽or오른쪽으로 방향벡터 전달
  (switch `int` (`KismetMathLibrary.RandomIntegerInRange` 0 1)
    (:`0`
      (return (`KismetMathLibrary.RotateAngleAxis` (`SceneComponent.GetForwardVector` (`self.Arrow`)) 90.0 (0.0 0.0 1.0))))
    (:`1`
      (return (`KismetMathLibrary.RotateAngleAxis` (`SceneComponent.GetForwardVector` (`self.Arrow`)) -90.0 (0.0 0.0 1.0))))))

(fn `UserConstructionScript`
  (`TimelineComponent.SetPlayRate` (`self.Timeline`) (`self.GrowSpeed`)))
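; BP_BossSplineFire_Outline is an outer fire hazard in the boss fight that destroys itself when BP_Boss changes to Phase 4.
; Overlapping its box deals damage through the player's RXPlayerStatComponent and launches the player toward the boss, overriding horizontal velocity.
; The construction script sets a timeline's play rate from GrowSpeed, but nothing in the graph plays that timeline to drive the Niagara Progress parameter.
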(event `self.ReceiveBeginPlay`
  ;[1 1 1] 페이즈 4 활성화시 보스 이벤트 디스페처 구독 (파괴)
  (bind _returnvalue (`GameplayStatics.GetActorOfClass` "/Game/Blueprints/Boss/BP_Boss.BP_Boss_C"))
  (add `/Game/Blueprints/Boss/BP_Boss.ChangedToPhase4` _returnvalue (delegate `DestroyActor`)))

(event `DestroyActor`
  ;[1 1 1] 페이즈 4 활성화시 보스 이벤트 디스페처 구독 (파괴)
  (`self.K2_DestroyActor`))

(event `self.Box.OnComponentBeginOverlap`
  (params (OverlappedComponent :type "PrimitiveComponent Object Reference") (OtherActor :type "Actor Object Reference") (OtherComp :type "PrimitiveComponent Object Reference") (OtherBodyIndex :type Integer) (bFromSweep :type Boolean) (SweepResult :type "HitResult Structure (by ref)"))
  (bind _asbp_player (cast `/Game/Blueprints/Player/BP_Player` OtherActor))
  (`RXPlayerStatComponent.ApplyDamage` (`self.GetComponentByClass` _asbp_player "/Script/RETURN_XENIA.RXPlayerStatComponent") 1)
  ;[1 1 1] 외곽 불길 피격시 보스방향으로 플레이어를 밀어냄
  (bind _returnvalue (`GameplayStatics.GetActorOfClass` "/Game/Blueprints/Boss/BP_Boss.BP_Boss_C"))
  (`Character.LaunchCharacter` (`GameplayStatics.GetPlayerCharacter` 0) (* (`KismetMathLibrary.GetDirectionUnitVector` (`self.K2_GetActorLocation` (`GameplayStatics.GetPlayerCharacter` 0)) (`self.K2_GetActorLocation` _returnvalue)) 800.0) true false))

(fn `UserConstructionScript`
  (`TimelineComponent.SetPlayRate` (`self.Timeline`) (`self.GrowSpeed`)))
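; Boss attack-pattern manager that spawns circular fireball volleys for BP_Boss.
; On BeginPlay it caches the boss actor, and ShootFireball switches on the boss's current phase.
; Each phase currently runs the same timed sequence of three ring volleys from the manager's location, alternating two circle variants with delays between them.
; The firing functions are called here but defined outside this graph.
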(event `self.ReceiveBeginPlay`
  (`parent.ReceiveBeginPlay`)
  (bind _returnvalue (`GameplayStatics.GetActorOfClass` "/Game/Blueprints/Boss/BP_Boss.BP_Boss_C"))
  (set `self.Boss` _returnvalue))

(event `ShootFireball`
  (bind _returnvalue (`self.K2_GetActorLocation`))
  (bind _returnvalue_2 (`self.K2_GetActorLocation`))
  (bind _returnvalue_3 (`self.K2_GetActorLocation`))
  (bind _phase (`/Game/Blueprints/Boss/BP_Boss.ReturnCurrentPhase` (`self.Boss`)))
  (switch `name` _phase
    (:`Phase1`
      ;[1 1 1] 발사 함수는 총 9에 걸쳐 사출
      (`self.FireInCircleAt190` _returnvalue_3)
      (`KismetSystemLibrary.Delay` 3.0)
      (`self.FireInCircleAt300` _returnvalue_3)
      (`KismetSystemLibrary.Delay` 3.0)
      (`self.FireInCircleAt190` _returnvalue_3))
    (:`Phase2`
      (`self.FireInCircleAt190` _returnvalue_2)
      (`KismetSystemLibrary.Delay` 3.0)
      (`self.FireInCircleAt300` _returnvalue_2)
      (`KismetSystemLibrary.Delay` 3.0)
      (`self.FireInCircleAt190` _returnvalue_2))
    (:`Phase3`
      (`self.FireInCircleAt190` _returnvalue)
      (`KismetSystemLibrary.Delay` 3.0)
      (`self.FireInCircleAt300` _returnvalue)
      (`KismetSystemLibrary.Delay` 3.0)
      (`self.FireInCircleAt190` _returnvalue))))

(fn `UserConstructionScript`)
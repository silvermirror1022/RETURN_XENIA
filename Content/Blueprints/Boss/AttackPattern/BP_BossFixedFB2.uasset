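; Boss fireball projectile for an attack pattern, which damages the player on contact and speeds up as the boss changes phase.
; On BeginPlay it finds BP_Boss and binds to its phase 2 and 3 change delegates, with events that raise Speed.
; A box overlap with the player applies damage through RXPlayerStatComponent, plays explosion and sound effects, then returns the fireball to its pool via C++ ResetFireball.
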(event `SetPhase2_Velocity`
  ;[1 1 1] 페이즈마다 속도를 변경하는 함수
  (set `self.Speed` 1800.0))

(event `SetPhase3_Velocity`
  ;[1 1 1] 페이즈마다 속도를 변경하는 함수
  (set `self.Speed` 2100.0))

(event `self.ReceiveBeginPlay`
  (`parent.ReceiveBeginPlay`)
  (bind _returnvalue (`GameplayStatics.GetActorOfClass` "/Game/Blueprints/Boss/BP_Boss.BP_Boss_C"))
  (`|ExecutionSequence`
    (:`then_0`
      ;[1 1 1] 페이즈변경시 델리게이트를 통해서 속도 변경 / 함수 구독
      (add `/Game/Blueprints/Boss/BP_Boss.ChangedToPhase2` _returnvalue (`|CreateDelegate` :!event `SetPhase2_Velocity`)))
    (:`then_1`
      (add `/Game/Blueprints/Boss/BP_Boss.ChangedToPhase3` _returnvalue (`|CreateDelegate` :!event `SetPhase3_Velocity`)))))

(event `self.Box.OnComponentBeginOverlap`
  (params (OverlappedComponent :type "PrimitiveComponent Object Reference") (OtherActor :type "Actor Object Reference") (OtherComp :type "PrimitiveComponent Object Reference") (OtherBodyIndex :type Integer) (bFromSweep :type Boolean) (SweepResult :type "HitResult Structure (by ref)"))
  (bind _asbp_player (cast `/Game/Blueprints/Player/BP_Player` OtherActor))
  (`RXPlayerStatComponent.ApplyDamage` (`self.GetComponentByClass` _asbp_player "/Script/RETURN_XENIA.RXPlayerStatComponent") 1)
  (`GameplayStatics.SpawnEmitterAtLocation` "/Game/ImportedAsset/StarterContent/Particles/P_Explosion.P_Explosion" (`self.K2_GetActorLocation`))
  (`GameplayStatics.PlaySound2D` "/Game/Audio/SFX/Boss/SFX_HitFire.SFX_HitFire" 1.0 1.0 0.0 null null)
  ;[1 1 1] 플레이어와 피격시 풀로 반환 (C++)
  (`self.ResetFireball`))

(fn `UserConstructionScript`)
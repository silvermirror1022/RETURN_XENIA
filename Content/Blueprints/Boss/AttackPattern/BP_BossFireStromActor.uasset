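; Boss attack actor that telegraphs a firestorm with a notify circle, then damages and knocks up players caught in it.
; After a short delay on BeginPlay, the storm particles and collision box switch on and the notify circle switches off.
; Box overlap applies damage through RXPlayerStatComponent and adds an upward movement impulse.
; A LifeSecond timer from spawn removes storm and box, then destroys the actor shortly after.
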(event `self.ReceiveBeginPlay`
  ;[1 1 1] 스폰즉시 오로라 생기고 2.5초후 스톰이 생김 6.5초후(LifeSecond-2.5) Destroy
  (`KismetSystemLibrary.K2_SetTimerDelegate` (delegate `Destroy`) (`self.LifeSecond`))
  (`PrimitiveComponent.SetCollisionEnabled` (`self.Box`) "NoCollision")
  (`ActorComponent.Deactivate` (`self.PSC_Firestorm`))
  (`KismetSystemLibrary.Delay` 2.5)
  (`ActorComponent.Activate` (`self.PSC_Firestorm`) false)
  (`PrimitiveComponent.SetCollisionEnabled` (`self.Box`) "QueryAndPhysics")
  (`ActorComponent.Deactivate` (`self.PSC_NotifyCircle`)))

(event `Destroy`
  (`ActorComponent.K2_DestroyComponent` (`self.PSC_Firestorm`))
  (`ActorComponent.K2_DestroyComponent` (`self.Box`))
  (`KismetSystemLibrary.Delay` 2.0)
  (`self.K2_DestroyActor`))

(event `self.Box.OnComponentBeginOverlap`
  (params (OverlappedComponent :type "PrimitiveComponent Object Reference") (OtherActor :type "Actor Object Reference") (OtherComp :type "PrimitiveComponent Object Reference") (OtherBodyIndex :type Integer) (bFromSweep :type Boolean) (SweepResult :type "HitResult Structure (by ref)"))
  (bind _asrxplayer (cast `RXPlayer` OtherActor))
  (`RXPlayerStatComponent.ApplyDamage` (`self.GetComponentByClass` _asrxplayer "/Script/RETURN_XENIA.RXPlayerStatComponent") 1)
  (`CharacterMovementComponent.AddImpulse` (`Character.CharacterMovement` _asrxplayer) (0.0 0.0 90000.0) false))

(fn `UserConstructionScript`)
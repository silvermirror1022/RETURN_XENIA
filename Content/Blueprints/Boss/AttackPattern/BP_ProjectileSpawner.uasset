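; Boss attack projectile spawner that fires rays and targeting fireballs through FireProjectile.
; Rays spawn at the spawner's own location, while fireballs spawn from the ShootPos of the BP_Boss found in the level.
; Three phase events each run a looping timer, then clear it after a delay, with shorter intervals and longer barrages in later phases.
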(event `self.ReceiveBeginPlay`)

(event `FireRay`
  (`self.FireProjectile` (`self.RayClass`) (`self.K2_GetActorLocation`)))

(event `FireTargetFB`
  (bind _returnvalue (`GameplayStatics.GetActorOfClass` "/Game/Blueprints/Boss/BP_Boss.BP_Boss_C"))
  (`self.FireProjectile` (`self.TargetingFireballClass`) (`SceneComponent.K2_GetComponentLocation` (`/Game/Blueprints/Boss/BP_Boss.ShootPos` _returnvalue))))

(event `FireTargetingFB_Phase1`
  (bind _returnvalue (`KismetSystemLibrary.K2_SetTimerDelegate` (`|CreateDelegate` :!event `FireTargetFB`) 1.0 true))
  (`KismetSystemLibrary.Delay` 4.0)
  (`KismetSystemLibrary.K2_ClearAndInvalidateTimerHandle` _returnvalue))

(event `FireTargetingFB_Phase2`
  (bind _returnvalue (`KismetSystemLibrary.K2_SetTimerDelegate` (`|CreateDelegate` :!event `FireTargetFB`) 0.75 true))
  (`KismetSystemLibrary.Delay` 6.0)
  (`KismetSystemLibrary.K2_ClearAndInvalidateTimerHandle` _returnvalue))

(event `FireTargetingFB_Phase3`
  (bind _returnvalue (`KismetSystemLibrary.K2_SetTimerDelegate` (`|CreateDelegate` :!event `FireTargetFB`) 0.5 true))
  (`KismetSystemLibrary.Delay` 8.0)
  (`KismetSystemLibrary.K2_ClearAndInvalidateTimerHandle` _returnvalue))

(fn `UserConstructionScript`)
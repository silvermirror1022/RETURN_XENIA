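; Phase 1 boss ray projectile that flies toward the player and damages them on contact.
; On BeginPlay it finds BP_Player, enables query collision on three boxes and destroys itself five seconds later.
; RotateToTarget aims once without homing, passing the flattened world direction times Speed to SetVelocityInLocalSpace rather than rotating the actor.
; Each box overlap with the player applies 1 damage through RXPlayerStatComponent, without destroying the ray.
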(event `self.ReceiveBeginPlay`
  ;[1 1 1] TimeLine FloatTrack Length = DelayDuration
  (bind _returnvalue (`GameplayStatics.GetActorOfClass` "/Game/Blueprints/Player/BP_Player.BP_Player_C"))
  (bind _output_get (set `self.Player` _returnvalue))
  (`/Engine/EditorBlueprintResources/StandardMacros.IsValid` _output_get
    (:`Is Valid`
      (`PrimitiveComponent.SetCollisionEnabled` (`self.Box`) "QueryOnly")
      (`PrimitiveComponent.SetCollisionEnabled` (`self.Box1`) "QueryOnly")
      (`PrimitiveComponent.SetCollisionEnabled` (`self.Box2`) "QueryOnly")
      (`self.RotateToTarget`)
      (`KismetSystemLibrary.Delay` 5.0)
      (`self.K2_DestroyActor`))))

(event `RotateToTarget`
  (bind (_returnvalue_x _returnvalue_y) (`KismetMathLibrary.BreakVector` (`KismetMathLibrary.GetDirectionUnitVector` (`self.K2_GetActorLocation`) (`self.K2_GetActorLocation` (`self.Player`)))))
  (`ProjectileMovementComponent.SetVelocityInLocalSpace` (`self.ProjectileMovement`) (* (`KismetMathLibrary.MakeVector` _returnvalue_x _returnvalue_y 0.0) (`self.Speed`))))

(event `self.Box.OnComponentBeginOverlap`
  (params (OverlappedComponent :type "PrimitiveComponent Object Reference") (OtherActor :type "Actor Object Reference") (OtherComp :type "PrimitiveComponent Object Reference") (OtherBodyIndex :type Integer) (bFromSweep :type Boolean) (SweepResult :type "HitResult Structure (by ref)"))
  (bind _asbp_player (cast `/Game/Blueprints/Player/BP_Player` OtherActor))
  (`RXPlayerStatComponent.ApplyDamage` (`self.GetComponentByClass` _asbp_player "/Script/RETURN_XENIA.RXPlayerStatComponent") 1))

(event `self.Box1.OnComponentBeginOverlap`
  (params (OverlappedComponent :type "PrimitiveComponent Object Reference") (OtherActor :type "Actor Object Reference") (OtherComp :type "PrimitiveComponent Object Reference") (OtherBodyIndex :type Integer) (bFromSweep :type Boolean) (SweepResult :type "HitResult Structure (by ref)"))
  (bind _asbp_player (cast `/Game/Blueprints/Player/BP_Player` OtherActor))
  (`RXPlayerStatComponent.ApplyDamage` (`self.GetComponentByClass` _asbp_player "/Script/RETURN_XENIA.RXPlayerStatComponent") 1))

(event `self.Box2.OnComponentBeginOverlap`
  (params (OverlappedComponent :type "PrimitiveComponent Object Reference") (OtherActor :type "Actor Object Reference") (OtherComp :type "PrimitiveComponent Object Reference") (OtherBodyIndex :type Integer) (bFromSweep :type Boolean) (SweepResult :type "HitResult Structure (by ref)"))
  (bind _asbp_player (cast `/Game/Blueprints/Player/BP_Player` OtherActor))
  (`RXPlayerStatComponent.ApplyDamage` (`self.GetComponentByClass` _asbp_player "/Script/RETURN_XENIA.RXPlayerStatComponent") 1))

(fn `UserConstructionScript`)
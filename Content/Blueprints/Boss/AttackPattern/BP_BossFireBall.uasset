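; BP_BossFireBall is a boss attack projectile that fires toward the player as soon as it spawns.
; On BeginPlay it finds BP_Player and sets a one-time velocity toward that position at Speed, with no homing.
; RotateToTarget sets only velocity, passing the world-space direction to SetVelocityInLocalSpace without rotating the actor.
; Box overlap with the player only prints placeholder text and deals no damage.
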(event `self.ReceiveBeginPlay`
  ;[1 1 1] 스폰 즉시 플레이어를 찾아서 플레이어의 위치를 기록한 후 발사함.
  (bind _returnvalue (`GameplayStatics.GetActorOfClass` "/Game/Blueprints/Player/BP_Player.BP_Player_C"))
  (bind _output_get (set `self.Player` _returnvalue))
  (`/Engine/EditorBlueprintResources/StandardMacros.IsValid` _output_get
    (:`Is Valid`
      (`self.RotateToTarget`))))

(event `RotateToTarget`
  (`ProjectileMovementComponent.SetVelocityInLocalSpace` (`self.ProjectileMovement`) (* (`KismetMathLibrary.GetDirectionUnitVector` (`self.K2_GetActorLocation`) (`self.K2_GetActorLocation` (`self.Player`))) (`self.Speed`))))

(event `self.Box.OnComponentBeginOverlap`
  (params (OverlappedComponent :type "PrimitiveComponent Object Reference") (OtherActor :type "Actor Object Reference") (OtherComp :type "PrimitiveComponent Object Reference") (OtherBodyIndex :type Integer) (bFromSweep :type Boolean) (SweepResult :type "HitResult Structure (by ref)"))
  (cast `/Game/Blueprints/Player/BP_Player` OtherActor)
  (`KismetSystemLibrary.PrintText` "Hello"))

(fn `UserConstructionScript`)
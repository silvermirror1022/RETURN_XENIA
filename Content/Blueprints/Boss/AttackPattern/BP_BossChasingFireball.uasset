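; BP_BossChasingFireball is a boss attack projectile that homes in on the player and explodes on contact.
; On BeginPlay it finds BP_Player, sets its root as the ProjectileMovement homing target, and slows Tick to once per second.
; Both a Box overlap with the player and a proximity check on Tick deal damage through RXPlayerStatComponent, spawn an explosion and destroy the fireball.
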(event `self.ReceiveTick`
  (params (DeltaSeconds :type "Float (single-precision)"))
  (if (<= (`KismetMathLibrary.Vector_Distance` (`self.K2_GetActorLocation` (`self.PlayerTarget`)) (`self.K2_GetActorLocation`)) 125.0)
    (`RXPlayerStatComponent.ApplyDamage` (`self.GetComponentByClass` (`self.PlayerTarget`) "/Script/RETURN_XENIA.RXPlayerStatComponent") 1)
    (`GameplayStatics.SpawnEmitterAtLocation` "/Game/ImportedAsset/StarterContent/Particles/P_Explosion.P_Explosion" (`self.K2_GetActorLocation`))
    (`self.K2_DestroyActor`)))

(event `self.ReceiveBeginPlay`
  ;[1 1 1] TimeLine FloatTrack Length = DelayDuration
  (bind _returnvalue (`GameplayStatics.GetActorOfClass` "/Game/Blueprints/Player/BP_Player.BP_Player_C"))
  (bind _output_get (set `self.PlayerTarget` _returnvalue))
  (`/Engine/EditorBlueprintResources/StandardMacros.IsValid` _output_get
    (:`Is Valid`
      (set `ProjectileMovementComponent.HomingTargetComponent` (`Actor.RootComponent` (`self.PlayerTarget`)) (`self.ProjectileMovement`))
      (`self.SetActorTickInterval` 1.0))))

(event `self.Box.OnComponentBeginOverlap`
  (params (OverlappedComponent :type "PrimitiveComponent Object Reference") (OtherActor :type "Actor Object Reference") (OtherComp :type "PrimitiveComponent Object Reference") (OtherBodyIndex :type Integer) (bFromSweep :type Boolean) (SweepResult :type "HitResult Structure (by ref)"))
  (bind _asbp_player (cast `/Game/Blueprints/Player/BP_Player` OtherActor))
  (`RXPlayerStatComponent.ApplyDamage` (`self.GetComponentByClass` _asbp_player "/Script/RETURN_XENIA.RXPlayerStatComponent") 1)
  (`GameplayStatics.SpawnEmitterAtLocation` "/Game/ImportedAsset/StarterContent/Particles/P_Explosion.P_Explosion" SweepResult_Location)
  (`self.K2_DestroyActor`))

(fn `UserConstructionScript`)
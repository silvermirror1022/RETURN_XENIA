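; Boss melee attack actor that plays the attack effects and damages and knocks back the player.
; MeleeAttack switches on seven particle systems, inactive from BeginPlay, for one second.
; DamagePlayer applies damage through RXPlayerStatComponent, spawns an explosion at the player and calls ImpulsePlayer.
; ImpulsePlayer launches the player along BP_Boss's forward vector, then forces Walking movement after a short delay as a bug workaround.
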(event `self.ReceiveBeginPlay`
  (`ActorComponent.Deactivate` (`self.ParticleSystem`))
  (`ActorComponent.Deactivate` (`self.ParticleSystem2`))
  (`ActorComponent.Deactivate` (`self.ParticleSystem3`))
  (`ActorComponent.Deactivate` (`self.ParticleSystem4`))
  (`ActorComponent.Deactivate` (`self.ParticleSystem5`))
  (`ActorComponent.Deactivate` (`self.ParticleSystem6`))
  (`ActorComponent.Deactivate` (`self.ParticleSystem7`)))

(event `ImpulsePlayer`
  (bind _returnvalue (`GameplayStatics.GetPlayerCharacter` 0))
  (bind _returnvalue_2 (`GameplayStatics.GetActorOfClass` "/Game/Blueprints/Boss/BP_Boss.BP_Boss_C"))
  (`Character.LaunchCharacter` _returnvalue (* (`SceneComponent.GetForwardVector` (`Actor.RootComponent` _returnvalue_2)) (`self.Force`)) true false)
  ;[1 1 1] 버그방지
  (`KismetSystemLibrary.Delay` 0.75)
  (`CharacterMovementComponent.SetMovementMode` (`Character.CharacterMovement` _returnvalue) "MOVE_Walking" 0))

(event `MeleeAttack`
  (`ActorComponent.Activate` (`self.ParticleSystem`) false)
  (`ActorComponent.Activate` (`self.ParticleSystem2`) false)
  (`ActorComponent.Activate` (`self.ParticleSystem3`) false)
  (`ActorComponent.Activate` (`self.ParticleSystem4`) false)
  (`ActorComponent.Activate` (`self.ParticleSystem5`) false)
  (`ActorComponent.Activate` (`self.ParticleSystem6`) false)
  (`ActorComponent.Activate` (`self.ParticleSystem7`) false)
  (`KismetSystemLibrary.Delay` 1.0)
  (`ActorComponent.Deactivate` (`self.ParticleSystem`))
  (`ActorComponent.Deactivate` (`self.ParticleSystem2`))
  (`ActorComponent.Deactivate` (`self.ParticleSystem3`))
  (`ActorComponent.Deactivate` (`self.ParticleSystem4`))
  (`ActorComponent.Deactivate` (`self.ParticleSystem5`))
  (`ActorComponent.Deactivate` (`self.ParticleSystem6`))
  (`ActorComponent.Deactivate` (`self.ParticleSystem7`)))

(event `DamagePlayer`
  (bind _returnvalue (`GameplayStatics.GetPlayerCharacter` 0))
  (bind _asrxplayer (cast `RXPlayer` _returnvalue))
  (`RXPlayerStatComponent.ApplyDamage` (`self.GetComponentByClass` _asrxplayer "/Script/RETURN_XENIA.RXPlayerStatComponent") 1)
  (`GameplayStatics.SpawnEmitterAtLocation` "/Game/ImportedAsset/StarterContent/Particles/P_Explosion.P_Explosion" (`self.K2_GetActorLocation` _returnvalue))
  (`self.ImpulsePlayer`))

(fn `UserConstructionScript`)
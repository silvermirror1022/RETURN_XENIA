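; Boss ray attack projectile that damages the player on contact and gets faster as the boss advances through its phases.
; BeginPlay sets the base ProjectileMovement speed, then binds to BP_Boss's phase 2 and phase 3 delegates for the speed-up events, which change initial and max speed.
; Many box colliders each repeat the same overlap logic, applying damage through the player's RXPlayerStatComponent and playing an electric sound.
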(event `SetPhase2_Velocity`
  (bind _projectilemovement (`self.ProjectileMovement`))
  ;[1 1 1] 페이즈 올라갈 때마다 속도 상승 함수
  (set `ProjectileMovementComponent.InitialSpeed` 2600.0 _projectilemovement)
  (set `ProjectileMovementComponent.MaxSpeed` 2500.0 _projectilemovement))

(event `SetPhase3_Velocity`
  (bind _projectilemovement (`self.ProjectileMovement`))
  ;[1 1 1] 페이즈 올라갈 때마다 속도 상승 함수
  (set `ProjectileMovementComponent.InitialSpeed` 3000.0 _projectilemovement)
  (set `ProjectileMovementComponent.MaxSpeed` 3000.0 _projectilemovement))

(event `self.ReceiveBeginPlay`
  (bind _projectilemovement (`self.ProjectileMovement`))
  ;[1 1 1] 속도 설정
  (set `ProjectileMovementComponent.InitialSpeed` 2200.0 _projectilemovement)
  (set `ProjectileMovementComponent.MaxSpeed` 2200.0 _projectilemovement)
  (bind _returnvalue (`GameplayStatics.GetActorOfClass` "/Game/Blueprints/Boss/BP_Boss.BP_Boss_C"))
  (`|ExecutionSequence`
    (:`then_0`
      ;[1 1 1] 페이즈변경시 델리게이트를 통해서 속도 변경 / 함수 구독
      (add `/Game/Blueprints/Boss/BP_Boss.ChangedToPhase2` _returnvalue (`|CreateDelegate` :!event `SetPhase2_Velocity`)))
    (:`then_1`
      (add `/Game/Blueprints/Boss/BP_Boss.ChangedToPhase3` _returnvalue (`|CreateDelegate` :!event `SetPhase3_Velocity`)))))

(event `self.Box.OnComponentBeginOverlap`
  (params (OverlappedComponent :type "PrimitiveComponent Object Reference") (OtherActor :type "Actor Object Reference") (OtherComp :type "PrimitiveComponent Object Reference") (OtherBodyIndex :type Integer) (bFromSweep :type Boolean) (SweepResult :type "HitResult Structure (by ref)"))
  (bind _asbp_player (cast `/Game/Blueprints/Player/BP_Player` OtherActor))
  (`RXPlayerStatComponent.ApplyDamage` (`self.GetComponentByClass` _asbp_player "/Script/RETURN_XENIA.RXPlayerStatComponent") 1)
  (`GameplayStatics.PlaySound2D` "/Game/Audio/SFX/Boss/SFX_Elec2.SFX_Elec2" 1.0 1.0 0.0 null null))

(event `self.Box1.OnComponentBeginOverlap`
  (params (OverlappedComponent :type "PrimitiveComponent Object Reference") (OtherActor :type "Actor Object Reference") (OtherComp :type "PrimitiveComponent Object Reference") (OtherBodyIndex :type Integer) (bFromSweep :type Boolean) (SweepResult :type "HitResult Structure (by ref)"))
  (bind _asbp_player (cast `/Game/Blueprints/Player/BP_Player` OtherActor))
  (`RXPlayerStatComponent.ApplyDamage` (`self.GetComponentByClass` _asbp_player "/Script/RETURN_XENIA.RXPlayerStatComponent") 1)
  (`GameplayStatics.PlaySound2D` "/Game/Audio/SFX/Boss/SFX_Elec2.SFX_Elec2" 1.0 1.0 0.0 null null))

(event `self.Box11.OnComponentBeginOverlap`
  (params (OverlappedComponent :type "PrimitiveComponent Object Reference") (OtherActor :type "Actor Object Reference") (OtherComp :type "PrimitiveComponent Object Reference") (OtherBodyIndex :type Integer) (bFromSweep :type Boolean) (SweepResult :type "HitResult Structure (by ref)"))
  (bind _asbp_player (cast `/Game/Blueprints/Player/BP_Player` OtherActor))
  (`RXPlayerStatComponent.ApplyDamage` (`self.GetComponentByClass` _asbp_player "/Script/RETURN_XENIA.RXPlayerStatComponent") 1)
  (`GameplayStatics.PlaySound2D` "/Game/Audio/SFX/Boss/SFX_Elec2.SFX_Elec2" 1.0 1.0 0.0 null null))

(event `self.Box2.OnComponentBeginOverlap`
  (params (OverlappedComponent :type "PrimitiveComponent Object Reference") (OtherActor :type "Actor Object Reference") (OtherComp :type "PrimitiveComponent Object Reference") (OtherBodyIndex :type Integer) (bFromSweep :type Boolean) (SweepResult :type "HitResult Structure (by ref)"))
  (bind _asbp_player (cast `/Game/Blueprints/Player/BP_Player` OtherActor))
  (`RXPlayerStatComponent.ApplyDamage` (`self.GetComponentByClass` _asbp_player "/Script/RETURN_XENIA.RXPlayerStatComponent") 1)
  (`GameplayStatics.PlaySound2D` "/Game/Audio/SFX/Boss/SFX_Elec2.SFX_Elec2" 1.0 1.0 0.0 null null))

(event `self.Box12.OnComponentBeginOverlap`
  (params (OverlappedComponent :type "PrimitiveComponent Object Reference") (OtherActor :type "Actor Object Reference") (OtherComp :type "PrimitiveComponent Object Reference") (OtherBodyIndex :type Integer) (bFromSweep :type Boolean) (SweepResult :type "HitResult Structure (by ref)"))
  (bind _asbp_player (cast `/Game/Blueprints/Player/BP_Player` OtherActor))
  (`RXPlayerStatComponent.ApplyDamage` (`self.GetComponentByClass` _asbp_player "/Script/RETURN_XENIA.RXPlayerStatComponent") 1)
  (`GameplayStatics.PlaySound2D` "/Game/Audio/SFX/Boss/SFX_Elec2.SFX_Elec2" 1.0 1.0 0.0 null null))

(event `self.Box4.OnComponentBeginOverlap`
  (params (OverlappedComponent :type "PrimitiveComponent Object Reference") (OtherActor :type "Actor Object Reference") (OtherComp :type "PrimitiveComponent Object Reference") (OtherBodyIndex :type Integer) (bFromSweep :type Boolean) (SweepResult :type "HitResult Structure (by ref)"))
  (bind _asbp_player (cast `/Game/Blueprints/Player/BP_Player` OtherActor))
  (`RXPlayerStatComponent.ApplyDamage` (`self.GetComponentByClass` _asbp_player "/Script/RETURN_XENIA.RXPlayerStatComponent") 1)
  (`GameplayStatics.PlaySound2D` "/Game/Audio/SFX/Boss/SFX_Elec2.SFX_Elec2" 1.0 1.0 0.0 null null))

(event `self.Box14.OnComponentBeginOverlap`
  (params (OverlappedComponent :type "PrimitiveComponent Object Reference") (OtherActor :type "Actor Object Reference") (OtherComp :type "PrimitiveComponent Object Reference") (OtherBodyIndex :type Integer) (bFromSweep :type Boolean) (SweepResult :type "HitResult Structure (by ref)"))
  (bind _asbp_player (cast `/Game/Blueprints/Player/BP_Player` OtherActor))
  (`RXPlayerStatComponent.ApplyDamage` (`self.GetComponentByClass` _asbp_player "/Script/RETURN_XENIA.RXPlayerStatComponent") 1)
  (`GameplayStatics.PlaySound2D` "/Game/Audio/SFX/Boss/SFX_Elec2.SFX_Elec2" 1.0 1.0 0.0 null null))

(event `self.Box5.OnComponentBeginOverlap`
  (params (OverlappedComponent :type "PrimitiveComponent Object Reference") (OtherActor :type "Actor Object Reference") (OtherComp :type "PrimitiveComponent Object Reference") (OtherBodyIndex :type Integer) (bFromSweep :type Boolean) (SweepResult :type "HitResult Structure (by ref)"))
  (bind _asbp_player (cast `/Game/Blueprints/Player/BP_Player` OtherActor))
  (`RXPlayerStatComponent.ApplyDamage` (`self.GetComponentByClass` _asbp_player "/Script/RETURN_XENIA.RXPlayerStatComponent") 1)
  (`GameplayStatics.PlaySound2D` "/Game/Audio/SFX/Boss/SFX_Elec2.SFX_Elec2" 1.0 1.0 0.0 null null))

(event `self.Box13.OnComponentBeginOverlap`
  (params (OverlappedComponent :type "PrimitiveComponent Object Reference") (OtherActor :type "Actor Object Reference") (OtherComp :type "PrimitiveComponent Object Reference") (OtherBodyIndex :type Integer) (bFromSweep :type Boolean) (SweepResult :type "HitResult Structure (by ref)"))
  (bind _asbp_player (cast `/Game/Blueprints/Player/BP_Player` OtherActor))
  (`RXPlayerStatComponent.ApplyDamage` (`self.GetComponentByClass` _asbp_player "/Script/RETURN_XENIA.RXPlayerStatComponent") 1)
  (`GameplayStatics.PlaySound2D` "/Game/Audio/SFX/Boss/SFX_Elec2.SFX_Elec2" 1.0 1.0 0.0 null null))

(event `self.Box6.OnComponentBeginOverlap`
  (params (OverlappedComponent :type "PrimitiveComponent Object Reference") (OtherActor :type "Actor Object Reference") (OtherComp :type "PrimitiveComponent Object Reference") (OtherBodyIndex :type Integer) (bFromSweep :type Boolean) (SweepResult :type "HitResult Structure (by ref)"))
  (bind _asbp_player (cast `/Game/Blueprints/Player/BP_Player` OtherActor))
  (`RXPlayerStatComponent.ApplyDamage` (`self.GetComponentByClass` _asbp_player "/Script/RETURN_XENIA.RXPlayerStatComponent") 1)
  (`GameplayStatics.PlaySound2D` "/Game/Audio/SFX/Boss/SFX_Elec2.SFX_Elec2" 1.0 1.0 0.0 null null))

(event `self.Box15.OnComponentBeginOverlap`
  (params (OverlappedComponent :type "PrimitiveComponent Object Reference") (OtherActor :type "Actor Object Reference") (OtherComp :type "PrimitiveComponent Object Reference") (OtherBodyIndex :type Integer) (bFromSweep :type Boolean) (SweepResult :type "HitResult Structure (by ref)"))
  (bind _asbp_player (cast `/Game/Blueprints/Player/BP_Player` OtherActor))
  (`RXPlayerStatComponent.ApplyDamage` (`self.GetComponentByClass` _asbp_player "/Script/RETURN_XENIA.RXPlayerStatComponent") 1)
  (`GameplayStatics.PlaySound2D` "/Game/Audio/SFX/Boss/SFX_Elec2.SFX_Elec2" 1.0 1.0 0.0 null null))

(event `self.Box3.OnComponentBeginOverlap`
  (params (OverlappedComponent :type "PrimitiveComponent Object Reference") (OtherActor :type "Actor Object Reference") (OtherComp :type "PrimitiveComponent Object Reference") (OtherBodyIndex :type Integer) (bFromSweep :type Boolean) (SweepResult :type "HitResult Structure (by ref)"))
  (bind _asbp_player (cast `/Game/Blueprints/Player/BP_Player` OtherActor))
  (`RXPlayerStatComponent.ApplyDamage` (`self.GetComponentByClass` _asbp_player "/Script/RETURN_XENIA.RXPlayerStatComponent") 1)
  (`GameplayStatics.PlaySound2D` "/Game/Audio/SFX/Boss/SFX_Elec2.SFX_Elec2" 1.0 1.0 0.0 null null))

(event `self.Box16.OnComponentBeginOverlap`
  (params (OverlappedComponent :type "PrimitiveComponent Object Reference") (OtherActor :type "Actor Object Reference") (OtherComp :type "PrimitiveComponent Object Reference") (OtherBodyIndex :type Integer) (bFromSweep :type Boolean) (SweepResult :type "HitResult Structure (by ref)"))
  (bind _asbp_player (cast `/Game/Blueprints/Player/BP_Player` OtherActor))
  (`RXPlayerStatComponent.ApplyDamage` (`self.GetComponentByClass` _asbp_player "/Script/RETURN_XENIA.RXPlayerStatComponent") 1)
  (`GameplayStatics.PlaySound2D` "/Game/Audio/SFX/Boss/SFX_Elec2.SFX_Elec2" 1.0 1.0 0.0 null null))

(event `self.Box10.OnComponentBeginOverlap`
  (params (OverlappedComponent :type "PrimitiveComponent Object Reference") (OtherActor :type "Actor Object Reference") (OtherComp :type "PrimitiveComponent Object Reference") (OtherBodyIndex :type Integer) (bFromSweep :type Boolean) (SweepResult :type "HitResult Structure (by ref)"))
  (bind _asbp_player (cast `/Game/Blueprints/Player/BP_Player` OtherActor))
  (`RXPlayerStatComponent.ApplyDamage` (`self.GetComponentByClass` _asbp_player "/Script/RETURN_XENIA.RXPlayerStatComponent") 1)
  (`GameplayStatics.PlaySound2D` "/Game/Audio/SFX/Boss/SFX_Elec2.SFX_Elec2" 1.0 1.0 0.0 null null))

(event `self.Box9.OnComponentBeginOverlap`
  (params (OverlappedComponent :type "PrimitiveComponent Object Reference") (OtherActor :type "Actor Object Reference") (OtherComp :type "PrimitiveComponent Object Reference") (OtherBodyIndex :type Integer) (bFromSweep :type Boolean) (SweepResult :type "HitResult Structure (by ref)"))
  (bind _asbp_player (cast `/Game/Blueprints/Player/BP_Player` OtherActor))
  (`RXPlayerStatComponent.ApplyDamage` (`self.GetComponentByClass` _asbp_player "/Script/RETURN_XENIA.RXPlayerStatComponent") 1)
  (`GameplayStatics.PlaySound2D` "/Game/Audio/SFX/Boss/SFX_Elec2.SFX_Elec2" 1.0 1.0 0.0 null null))

(event `self.Box7.OnComponentBeginOverlap`
  (params (OverlappedComponent :type "PrimitiveComponent Object Reference") (OtherActor :type "Actor Object Reference") (OtherComp :type "PrimitiveComponent Object Reference") (OtherBodyIndex :type Integer) (bFromSweep :type Boolean) (SweepResult :type "HitResult Structure (by ref)"))
  (bind _asbp_player (cast `/Game/Blueprints/Player/BP_Player` OtherActor))
  (`RXPlayerStatComponent.ApplyDamage` (`self.GetComponentByClass` _asbp_player "/Script/RETURN_XENIA.RXPlayerStatComponent") 1)
  (`GameplayStatics.PlaySound2D` "/Game/Audio/SFX/Boss/SFX_Elec2.SFX_Elec2" 1.0 1.0 0.0 null null))

(event `self.Box8.OnComponentBeginOverlap`
  (params (OverlappedComponent :type "PrimitiveComponent Object Reference") (OtherActor :type "Actor Object Reference") (OtherComp :type "PrimitiveComponent Object Reference") (OtherBodyIndex :type Integer) (bFromSweep :type Boolean) (SweepResult :type "HitResult Structure (by ref)"))
  (bind _asbp_player (cast `/Game/Blueprints/Player/BP_Player` OtherActor))
  (`RXPlayerStatComponent.ApplyDamage` (`self.GetComponentByClass` _asbp_player "/Script/RETURN_XENIA.RXPlayerStatComponent") 1)
  (`GameplayStatics.PlaySound2D` "/Game/Audio/SFX/Boss/SFX_Elec2.SFX_Elec2" 1.0 1.0 0.0 null null))

(fn `UserConstructionScript`)
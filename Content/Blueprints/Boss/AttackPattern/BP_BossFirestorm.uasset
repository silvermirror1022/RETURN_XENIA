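; BP_BossFirestorm is a boss attack hazard that damages the player and launches them upward on overlap.
; A notify circle warns for 2.5 seconds, then the storm activates, enables its hitbox and AI-moves toward a one-time snapshot of the player's position.
; A lifetime timer removes its components, then the actor after a short delay.
; Phase speed events exist, but their boss bindings are unconnected.
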(event `SetPhase2_Velocity`
  ;[1 1 1] 페이즈마다 속도를 변경하는 함수
  (set `FloatingPawnMovement.MaxSpeed` 400.0 (`self.FloatingPawnMovement`)))

(event `SetPhase3_Velocity`
  ;[1 1 1] 페이즈마다 속도를 변경하는 함수
  (set `FloatingPawnMovement.MaxSpeed` 450.0 (`self.FloatingPawnMovement`)))

(event `self.ReceiveBeginPlay`
  (bind (_returnvalue_x _returnvalue_y) (`KismetMathLibrary.BreakVector` (`self.K2_GetActorLocation` (`GameplayStatics.GetPlayerCharacter` 0))))
  ;[1 1 1] 스폰즉시 오로라 생기고 2.5초후 스톰이 생김 6.5초후(LifeSecond-2.5) Destroy
  (`KismetSystemLibrary.K2_SetTimerDelegate` (delegate `Destroy`) (`self.LifeSecond`))
  (`PrimitiveComponent.SetCollisionEnabled` (`self.HitBox`) "NoCollision")
  (`ActorComponent.Deactivate` (`self.PSC_Firestorm`))
  (`KismetSystemLibrary.Delay` 2.5)
  (`ActorComponent.Activate` (`self.PSC_Firestorm`) false)
  ;[1 1 1] 불폭풍의 플레이어 추적 기능 추가
  (`|AIMoveTo` self (`KismetMathLibrary.MakeVector` _returnvalue_x _returnvalue_y) null 1.0
    (:`then`
      (`PrimitiveComponent.SetCollisionEnabled` (`self.HitBox`) "QueryAndPhysics")
      (`ActorComponent.Deactivate` (`self.PSC_NotifyCircle`)))))

(event `Destroy`
  (`ActorComponent.K2_DestroyComponent` (`self.PSC_Firestorm`))
  (`ActorComponent.K2_DestroyComponent` (`self.Box`))
  (`ActorComponent.K2_DestroyComponent` (`self.HitBox`))
  (`KismetSystemLibrary.Delay` 2.0)
  (`self.K2_DestroyActor`))

(event `self.HitBox.OnComponentBeginOverlap`
  (params (OverlappedComponent :type "PrimitiveComponent Object Reference") (OtherActor :type "Actor Object Reference") (OtherComp :type "PrimitiveComponent Object Reference") (OtherBodyIndex :type Integer) (bFromSweep :type Boolean) (SweepResult :type "HitResult Structure (by ref)"))
  (bind _asrxplayer (cast `RXPlayer` OtherActor))
  (`RXPlayerStatComponent.ApplyDamage` (`self.GetComponentByClass` _asrxplayer "/Script/RETURN_XENIA.RXPlayerStatComponent") 1)
  (`CharacterMovementComponent.AddImpulse` (`Character.CharacterMovement` _asrxplayer) (0.0 0.0 90000.0) false))

(fn `UserConstructionScript`)
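; AI controller for the boss that starts the BT_Boss behavior tree one second after possession.
; Helper functions write the current attack type to the Blackboard, with the melee setter also storing the player Actor, and GetSenseSight reads whether an actor's sight stimulus was successfully sensed.
; The logic switching to melee when a Player-tagged actor is seen and ranged otherwise is disconnected, leaving OnPerceptionUpdated empty.
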(event `self.ReceivePossess`
  (params (PossessedPawn :type "Pawn Object Reference"))
  (`KismetSystemLibrary.Delay` 1.0)
  (`self.RunBehaviorTree` "/Game/Blueprints/Boss/BT_Boss.BT_Boss"))

(event `self.AIPerception.OnPerceptionUpdated`
  (params (UpdatedActors :type "Array of Actor Object Reference (by ref)"))
  ;[1 1 1] OnPerceptionUpdated 특정 대상의 퍼셉션이 업데이트될 때 호출됨
)

(fn `GetSenseSight`
  (params (Actor :type "Actor Object Reference"))
  (returns (`Successfully Sensed` :type Boolean))
  (bind _info (`AIPerceptionComponent.GetActorsPerception` (`self.AIPerception`) Actor))
  (for _array_element (`.LastSensedStimuli` (break `ActorPerceptionBlueprintInfo` _info))
    (bind _returnvalue (`AIPerceptionSystem.GetSenseClassForStimulus` _array_element))
    (if (== _returnvalue "/Script/AIModule.AISense_Sight")
      (return (`.bSuccessfullySensed` (break `AIStimulus` _array_element))))))

(fn `SetMeleeType`
  (params (AttackType :type "/Game/Blueprints/Boss/E_BossAttackType Enum" :default "NewEnumerator0") (Actor :type "Actor Object Reference"))
  (set `self.CurrentBossAttackType` AttackType)
  (`BlackboardComponent.SetValueAsEnum` (`self.Blackboard`) (`self.BossAttackTypeKeyName`) (`self.CurrentBossAttackType`))
  (`BlackboardComponent.SetValueAsObject` (`self.Blackboard`) (`self.PlayerKeyName`) Actor))

(fn `SetRangeType`
  (params (BossAttackType :type "/Game/Blueprints/Boss/E_BossAttackType Enum" :default "NewEnumerator0"))
  (set `self.CurrentBossAttackType` BossAttackType)
  (`BlackboardComponent.SetValueAsEnum` (`self.Blackboard`) (`self.BossAttackTypeKeyName`) (`self.CurrentBossAttackType`)))

(fn `UserConstructionScript`)
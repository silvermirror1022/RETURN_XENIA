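; Dialogue actor that runs the boss's death conversation when BP_Boss changes to phase 4.
; On BeginPlay it binds to that phase event and caches the boss mesh's ABP_Astuka anim instance.
; The trigger disables player movement, sets immortality, assigns itself as DetectedNPC to start dialogue, and stops the behaviour tree through the anim instance.
; DialoguePopupEvent then plays the death montage on that anim instance.
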(event `self.ReceiveBeginPlay`
  (bind _returnvalue (`GameplayStatics.GetActorOfClass` "/Game/Blueprints/Boss/BP_Boss.BP_Boss_C"))
  (bind _output_get (set `self.Boss` _returnvalue))
  (add `/Game/Blueprints/Boss/BP_Boss.ChangedToPhase4` _output_get (delegate `StartBossDeadTalk`))
  (bind _returnvalue_2 (`GameplayStatics.GetActorOfClass` "/Game/Blueprints/Boss/BP_Boss.BP_Boss_C"))
  (bind _asabp_astuka (cast `/Game/Animation/Astuka/ABP_Astuka` (`SkeletalMeshComponent.GetAnimInstance` (`Character.Mesh` _returnvalue_2))))
  (set `self.As ABP Astuka` _asabp_astuka))

(event `StartBossDeadTalk`
  (bind _returnvalue (`GameplayStatics.GetPlayerCharacter` 0))
  (`CharacterMovementComponent.SetMovementMode` (`Character.CharacterMovement` _returnvalue) "MOVE_None" 0)
  (bind _asrxplayer (cast `RXPlayer` _returnvalue))
  (set `RXPlayerStatComponent.bIsImmortal` true (`self.GetComponentByClass` _asrxplayer "/Script/RETURN_XENIA.RXPlayerStatComponent"))
  (bind _output_get (set `RXPlayer.DetectedNPC` self _asrxplayer))
  (`self.StartDialogue` _output_get)
  (`/Game/Animation/Astuka/ABP_Astuka.StopBehaviourTree` (`self.As ABP Astuka`)))

(event `self.DialoguePopupEvent`
  (`/Game/Animation/Astuka/ABP_Astuka.PlayMontage_Dead` (`self.As ABP Astuka`)))

(fn `UserConstructionScript`)
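; BP_BossEarthquake is a short-lived boss earthquake attack effect that punishes a grounded player.
; After a 1.5-second delay from spawn it starts a camera shake and applies damage through the player's RXPlayerStatComponent unless the character is falling, so jumping dodges it.
; The grounded check happens once, with no range test, then the shake stops and the actor destroys itself shortly afterward.
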(event `self.ReceiveBeginPlay`
  (bind _returnvalue (`GameplayStatics.GetPlayerCharacter` 0))
  (bind _returnvalue_2 (`GameplayStatics.GetPlayerCameraManager` 0))
  ;[1 1 1] 스폰즉시 1.5초 후 플레이어가 공중이면 데미지x
  (`KismetSystemLibrary.Delay` 1.5)
  (bind _returnvalue_3 (`PlayerCameraManager.StartCameraShake` :`self` _returnvalue_2 :`ShakeClass` "/Game/Blueprints/Boss/Effect/RefBP/BP_CameraShake.BP_CameraShake_C"))
  ;[1 1 1] 플레이어가 공중에있으면 =true / 랜딩=false
  (if (not (`NavMovementComponent.IsFalling` (`Character.CharacterMovement` _returnvalue)))
    (`RXPlayerStatComponent.ApplyDamage` (`self.GetComponentByClass` _returnvalue "/Script/RETURN_XENIA.RXPlayerStatComponent") 1))
  (`KismetSystemLibrary.Delay` 1.3)
  (`PlayerCameraManager.StopCameraShake` _returnvalue_2 _returnvalue_3 true)
  (`self.K2_DestroyActor`))

(fn `UserConstructionScript`)
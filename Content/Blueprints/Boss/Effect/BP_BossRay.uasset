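; Boss ray attack actor that travels from the BP_BossPlate and damages the player, then destroys itself after a fixed delay.
; On BeginPlay, a timeline lerps its location from the plate to a unit plate-to-player vector plus a fixed X offset, so the endpoint is near-constant in world space.
; Three box overlaps each deal damage to BP_Player through RXPlayerStatComponent.
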(event `self.ReceiveBeginPlay`
  (`|ExecutionSequence`
    (:`then_0`
      ;[1 1 1] TimeLine FloatTrack Length = DelayDuration
      (`KismetSystemLibrary.Delay` 5.0)
      (`self.K2_DestroyActor`))
    (:`then_1`
      (bind _returnvalue (`GameplayStatics.GetActorOfClass` "/Game/Blueprints/Boss/BP_BossPlate.BP_BossPlate_C"))
      (bind (_direction _floattrack) (`Timeline|Timeline` :!via `PlayFromStart`)
        (:`Update`
          (bind _returnvalue_2 (`self.K2_GetActorLocation` _returnvalue))
          (`self.K2_SetActorLocation` (`KismetMathLibrary.VLerp` _returnvalue_2 (+ (`KismetMathLibrary.GetDirectionUnitVector` _returnvalue_2 (`self.K2_GetActorLocation` (`GameplayStatics.GetPlayerCharacter` 0))) (4500.0 0.0 0.0)) _floattrack)))))))

(event `self.Box.OnComponentBeginOverlap`
  (params (OverlappedComponent :type "PrimitiveComponent Object Reference") (OtherActor :type "Actor Object Reference") (OtherComp :type "PrimitiveComponent Object Reference") (OtherBodyIndex :type Integer) (bFromSweep :type Boolean) (SweepResult :type "HitResult Structure (by ref)"))
  (bind _asbp_player (cast `/Game/Blueprints/Player/BP_Player` OtherActor))
  (`RXPlayerStatComponent.ApplyDamage` (`self.GetComponentByClass` _asbp_player "/Script/RETURN_XENIA.RXPlayerStatComponent") 1))

(event `self.Box1.OnComponentBeginOverlap`
  (params (OverlappedComponent :type "PrimitiveComponent Object Reference") (OtherActor :type "Actor Object Reference") (OtherComp :type "PrimitiveComponent Object Reference") (OtherBodyIndex :type Integer) (bFromSweep :type Boolean) (SweepResult :type "HitResult Structure (by ref)"))
  (bind _asbp_player (cast `/Game/Blueprints/Player/BP_Player` OtherActor))
  (`RXPlayerStatComponent.ApplyDamage` (`self.GetComponentByClass` _asbp_player "/Script/RETURN_XENIA.RXPlayerStatComponent") 1))

(event `self.Box2.OnComponentBeginOverlap`
  (params (OverlappedComponent :type "PrimitiveComponent Object Reference") (OtherActor :type "Actor Object Reference") (OtherComp :type "PrimitiveComponent Object Reference") (OtherBodyIndex :type Integer) (bFromSweep :type Boolean) (SweepResult :type "HitResult Structure (by ref)"))
  (bind _asbp_player (cast `/Game/Blueprints/Player/BP_Player` OtherActor))
  (`RXPlayerStatComponent.ApplyDamage` (`self.GetComponentByClass` _asbp_player "/Script/RETURN_XENIA.RXPlayerStatComponent") 1))

(fn `UserConstructionScript`)
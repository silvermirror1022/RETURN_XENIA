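; BP_FireStrom is a boss fire storm area effect that warns with a notify circle before striking.
; After a short delay it swaps the warning particles for the firestorm and enables the box's query and physics collision.
; Players overlapping the box take damage through RXPlayerStatComponent and are launched upward by an impulse.
; A timer set by LifeSecond removes the storm and box, then destroys the actor after a brief delay.
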(event `self.ReceiveBeginPlay`
  (`KismetSystemLibrary.K2_SetTimerDelegate` (delegate `Destroy`) (`self.LifeSecond`))
  (`PrimitiveComponent.SetCollisionEnabled` (`self.Box`) "NoCollision")
  (`ActorComponent.Deactivate` (`self.PSC_Firestorm`))
  (`KismetSystemLibrary.Delay` 2.5)
  (`ActorComponent.Activate` (`self.PSC_Firestorm`) false)
  (`PrimitiveComponent.SetCollisionEnabled` (`self.Box`) "QueryAndPhysics")
  (`ActorComponent.Deactivate` (`self.PSC_NotifyCircle`)))

(event `Destroy`
  (`ActorComponent.K2_DestroyComponent` (`self.PSC_Firestorm`))
  (`ActorComponent.K2_DestroyComponent` (`self.Box`))
  (`KismetSystemLibrary.Delay` 2.0)
  (`self.K2_DestroyActor`))

(event `self.Box.OnComponentBeginOverlap`
  (params (OverlappedComponent :type "PrimitiveComponent Object Reference") (OtherActor :type "Actor Object Reference") (OtherComp :type "PrimitiveComponent Object Reference") (OtherBodyIndex :type Integer) (bFromSweep :type Boolean) (SweepResult :type "HitResult Structure (by ref)"))
  (bind _asbp_player (cast `/Game/Blueprints/Player/BP_Player` OtherActor))
  (`RXPlayerStatComponent.ApplyDamage` (`self.GetComponentByClass` _asbp_player "/Script/RETURN_XENIA.RXPlayerStatComponent") 1)
  (`CharacterMovementComponent.AddImpulse` (`Character.CharacterMovement` _asbp_player) (0.0 0.0 90000.0) false)
  (`KismetSystemLibrary.PrintText` "Hello"))

(fn `UserConstructionScript`)
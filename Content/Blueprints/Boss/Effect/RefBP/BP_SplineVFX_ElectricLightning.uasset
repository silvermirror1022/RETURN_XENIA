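; Boss lightning VFX Blueprint that plays a Niagara effect growing along what its name indicates is a spline.
; The Niagara component is deactivated on BeginPlay and switched on by the ActiveSpline event.
; That event plays a timeline that drives the Niagara Progress float parameter, with its play rate set from GrowSpeed in the construction script.
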(event `self.ReceiveBeginPlay`
  (`ActorComponent.SetActive` (`self.Niagara`) false false))

(event `ActiveSpline`
  (`ActorComponent.SetActive` (`self.Niagara`) true false)
  (bind (_direction _newtrack_0) (`Timeline|Timeline`)
    (:`Update`
      (`NiagaraComponent.SetVariableFloat` (`self.Niagara`) "Progress" _newtrack_0))))

(fn `UserConstructionScript`
  (`TimelineComponent.SetPlayRate` (`self.Timeline`) (`self.GrowSpeed`)))
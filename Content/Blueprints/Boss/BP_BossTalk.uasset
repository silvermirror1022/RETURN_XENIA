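; BP_BossTalk handles the handoff from a boss dialogue popup to the fight with BP_Boss.
; On BeginPlay it finds and caches the boss and binds SetUI to its ChangedToPhase1 dispatcher.
; After a short delay, DialoguePopupEvent plays a fade-out, starts the battle, sets player movement to Walking and broadcasts ChangedToPhase1.
; That broadcast makes SetUI create and fade in the boss health widget.
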(event `self.ReceiveBeginPlay`
  (bind _returnvalue (`GameplayStatics.GetActorOfClass` "/Game/Blueprints/Boss/BP_Boss.BP_Boss_C"))
  (bind _output_get (set `self.Boss` _returnvalue))
  (add `/Game/Blueprints/Boss/BP_Boss.ChangedToPhase1` _output_get (delegate `SetUI`)))

(event `SetUI`
  ;[1 1 1] Boss Hp UI AddToViewport
  (bind _returnvalue (`|CreateWidget` "/Game/UI/Boss/WBP_BossHealth.WBP_BossHealth_C"))
  (`UserWidget.AddToViewport` _returnvalue 0)
  (`/Game/UI/Boss/WBP_BossHealth.FadeInBossUI` _returnvalue))

(event `self.DialoguePopupEvent`
  (bind _fadewidget (`self.FadeWidget`))
  (`KismetSystemLibrary.Delay` 1.0)
  (`UserWidget.AddToViewport` _fadewidget 0)
  (`/Game/UI/WBP_FadeAnimWidget.PlayFadeOut` _fadewidget)
  (bind _returnvalue (`GameplayStatics.GetActorOfClass` "/Game/Blueprints/Boss/BP_Boss.BP_Boss_C"))
  (`/Game/Blueprints/Boss/BP_Boss.BattleStart` _returnvalue)
  (`CharacterMovementComponent.SetMovementMode` (`Character.CharacterMovement` (`GameplayStatics.GetPlayerCharacter` 0)) "MOVE_Walking" 0)
  (`/Game/Blueprints/Boss/BP_Boss.ChangedToPhase1` (`self.Boss`)))

(fn `UserConstructionScript`)
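; Fire hazard actor that hurts a player on contact and knocks them aside.
; Box overlap applies one damage through the player's RXPlayerStatComponent, then launches player character 0.
; GetRandomDirection randomly picks left or right by rotating the Arrow's forward vector 90 degrees around Z.
; The construction script sets the Timeline rate from GrowSpeed, but the Timeline feeding Niagara's Progress parameter is never triggered in this graph.
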(event `self.Box.OnComponentBeginOverlap`
  (params (OverlappedComponent :type "PrimitiveComponent Object Reference") (OtherActor :type "Actor Object Reference") (OtherComp :type "PrimitiveComponent Object Reference") (OtherBodyIndex :type Integer) (bFromSweep :type Boolean) (SweepResult :type "HitResult Structure (by ref)"))
  (bind _asbp_player (cast `/Game/Blueprints/Player/BP_Player` OtherActor))
  (`RXPlayerStatComponent.ApplyDamage` (`self.GetComponentByClass` _asbp_player "/Script/RETURN_XENIA.RXPlayerStatComponent") 1)
  ;[1 1 1] 렌덤으로 불길 기준 플레이어를 좌우로 밀어냄
  (bind _newparam (`self.GetRandomDirection`))
  (`Character.LaunchCharacter` (`GameplayStatics.GetPlayerCharacter` 0) (* _newparam 1500.0) false false))

(fn `GetRandomDirection`
  (returns (NewParam :type "Vector Structure"))
  ;[1 1 1] 불길에 닿았을 때 랜덤 왼쪽or오른쪽으로 방향벡터 전달
  (switch `int` (`KismetMathLibrary.RandomIntegerInRange` 0 1)
    (:`0`
      (return (`KismetMathLibrary.RotateAngleAxis` (`SceneComponent.GetForwardVector` (`self.Arrow`)) 90.0 (0.0 0.0 1.0))))
    (:`1`
      (return (`KismetMathLibrary.RotateAngleAxis` (`SceneComponent.GetForwardVector` (`self.Arrow`)) -90.0 (0.0 0.0 1.0))))))

(fn `UserConstructionScript`
  (`TimelineComponent.SetPlayRate` (`self.Timeline`) (`self.GrowSpeed`)))
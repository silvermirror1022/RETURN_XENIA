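; BP_LookingPuzzleTrigger is a one-time box trigger that plays the LS_LookingCircluarPuzzle level sequence when the player walks in.
; The first RXPlayer overlap disables player input, plays the FadeWidget fade-out and starts the sequence.
; A fixed delay, rather than the sequence's finish event, times a second fade-out, and input is re-enabled shortly afterward.
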(event `self.Box.OnComponentBeginOverlap`
  (params (OverlappedComponent :type "PrimitiveComponent Object Reference") (OtherActor :type "Actor Object Reference") (OtherComp :type "PrimitiveComponent Object Reference") (OtherBodyIndex :type Integer) (bFromSweep :type Boolean) (SweepResult :type "HitResult Structure (by ref)"))
  (bind _fadewidget (`self.FadeWidget`))
  (bind _fadewidget_2 (`self.FadeWidget`))
  (cast `RXPlayer` OtherActor)
  (`/Engine/EditorBlueprintResources/StandardMacros.DoOnce` false
    (:`Completed`
      (`self.DisableInput` (`GameplayStatics.GetPlayerCharacter` 0) (`GameplayStatics.GetPlayerController` 0))
      (`UserWidget.AddToViewport` _fadewidget_2 0)
      (`/Game/UI/WBP_FadeAnimWidget.PlayFadeOut` _fadewidget_2)
      (bind _outactor (`LevelSequencePlayer.CreateLevelSequencePlayer` "/Game/Cinematics/LS_LookingCircluarPuzzle.LS_LookingCircluarPuzzle"))
      (`MovieSceneSequencePlayer.Play` (`LevelSequenceActor.SequencePlayer` _outactor))
      (`KismetSystemLibrary.Delay` 6.0)
      (`UserWidget.AddToViewport` _fadewidget 0)
      (`/Game/UI/WBP_FadeAnimWidget.PlayFadeOut` _fadewidget)
      (`KismetSystemLibrary.Delay` 0.5)
      (`self.EnableInput` (`GameplayStatics.GetPlayerCharacter` 0) (`GameplayStatics.GetPlayerController` 0)))))

(fn `UserConstructionScript`)
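; BP_AltarTrigger is a trigger that starts the Pachamama altar NPC dialogue when the player overlaps its box.
; On overlap by an RXPlayer, it sets the player character's movement mode to None and starts a camera shake.
; It then finds the BP_NPC_Pachamama_Altar actor, stores it as the player's detected NPC and starts its dialogue.
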(event `self.Box.OnComponentBeginOverlap`
  (params (OverlappedComponent :type "PrimitiveComponent Object Reference") (OtherActor :type "Actor Object Reference") (OtherComp :type "PrimitiveComponent Object Reference") (OtherBodyIndex :type Integer) (bFromSweep :type Boolean) (SweepResult :type "HitResult Structure (by ref)"))
  (cast `RXPlayer` OtherActor)
  (`CharacterMovementComponent.SetMovementMode` (`Character.CharacterMovement` (`GameplayStatics.GetPlayerCharacter` 0)) "MOVE_None" 0)
  (`PlayerCameraManager.StartCameraShake` :`self` (`GameplayStatics.GetPlayerCameraManager` 0) :`ShakeClass` "/Game/Blueprints/Boss/BP_CameraShake.BP_CameraShake_C")
  (bind _asrxplayer (cast `RXPlayer` (`GameplayStatics.GetPlayerCharacter` 0)))
  (bind _returnvalue (`GameplayStatics.GetActorOfClass` "/Game/Blueprints/Characters/BP_NPC_Pachamama_Altar.BP_NPC_Pachamama_Altar_C"))
  (set `RXPlayer.DetectedNPC` _returnvalue _asrxplayer)
  (`RXNonPlayer.StartDialogue` _returnvalue))

(fn `UserConstructionScript`)
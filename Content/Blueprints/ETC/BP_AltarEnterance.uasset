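; Altar entrance door that opens in a short cutscene when ActivateOpening is called.
; It freezes player movement, plays a widget fade and switches the view to a camera actor.
; A timeline moves the door mesh along Z, with event tracks starting rock sound and camera shake.
; After the door finishes moving and a brief delay, it fades again, restores walking and player view, and destroys the blocking box.
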(event `ActivateOpening`
  (bind _fadewidget (`self.FadeWidget`))
  (bind _fadewidget_2 (`self.FadeWidget`))
  (bind _returnvalue (`SceneComponent.GetRelativeTransform` (`self.SM_door`)))
  (`CharacterMovementComponent.SetMovementMode` (`Character.CharacterMovement` (`GameplayStatics.GetPlayerCharacter` 0)) "MOVE_None" 0)
  (`UserWidget.AddToViewport` _fadewidget 0)
  (`/Game/UI/WBP_FadeAnimWidget.PlayFadeOut` _fadewidget)
  (`PlayerController.SetViewTargetWithBlend` (`GameplayStatics.GetPlayerController` 0) (`self.CameraActor`) 0.0 "VTBlend_Linear" 0.0 false)
  (bind (_direction _vectortrack) (`Timeline|Timeline` :!via `PlayFromStart`)
    (:`Update`
      (`SceneComponent.K2_SetRelativeLocation` (`self.SM_door`) (`KismetMathLibrary.MakeVector` (.x (.location _returnvalue)) (.y (.location _returnvalue)) (.z _vectortrack)) false false))
    (:`MovingCompleted`
      (`KismetSystemLibrary.Delay` 1.0)
      (`UserWidget.AddToViewport` _fadewidget_2 0)
      (`/Game/UI/WBP_FadeAnimWidget.PlayFadeOut` _fadewidget_2)
      (`CharacterMovementComponent.SetMovementMode` (`Character.CharacterMovement` (`GameplayStatics.GetPlayerCharacter` 0)) "MOVE_Walking" 0)
      (`PlayerController.SetViewTargetWithBlend` (`GameplayStatics.GetPlayerController` 0) (`GameplayStatics.GetPlayerCharacter` 0) 0.0 "VTBlend_Linear" 0.0 false)
      (`ActorComponent.K2_DestroyComponent` (`self.BlockingBox`)))
    (:`MovingStart`
      (`GameplayStatics.PlaySound2D` "/Game/Audio/SFX/SFX_MoveRock.SFX_MoveRock" 1.0 1.0 0.0 null null)
      (`PlayerCameraManager.StartCameraShake` :`self` (`GameplayStatics.GetPlayerCameraManager` 0) :`ShakeClass` "/Game/Blueprints/Boss/BP_CameraShake.BP_CameraShake_C"))))

(fn `UserConstructionScript`)
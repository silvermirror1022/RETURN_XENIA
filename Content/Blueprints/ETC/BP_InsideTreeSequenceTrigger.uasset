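; Trigger actor that starts the cutscene for entering the inside of a tree when the player overlaps its box.
; On the first RXPlayer overlap only, it shows a fade widget playing its fade-out and plays the LS_EnterTreeInside level sequence.
; Fixed delays then time a jump-assist sound and a second fade-out from a newly created widget, independent of the sequence's finish event.
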(event `self.Box.OnComponentBeginOverlap`
  (params (OverlappedComponent :type "PrimitiveComponent Object Reference") (OtherActor :type "Actor Object Reference") (OtherComp :type "PrimitiveComponent Object Reference") (OtherBodyIndex :type Integer) (bFromSweep :type Boolean) (SweepResult :type "HitResult Structure (by ref)"))
  (cast `RXPlayer` OtherActor)
  (`/Engine/EditorBlueprintResources/StandardMacros.DoOnce` false
    (:`Completed`
      (bind _returnvalue (`|CreateWidget` "/Game/UI/WBP_FadeAnimWidget.WBP_FadeAnimWidget_C"))
      (`UserWidget.AddToViewport` _returnvalue 0)
      (`/Game/UI/WBP_FadeAnimWidget.PlayFadeOut` _returnvalue)
      (bind _outactor (`LevelSequencePlayer.CreateLevelSequencePlayer` "/Game/Cinematics/LS_EnterTreeInside.LS_EnterTreeInside"))
      (`MovieSceneSequencePlayer.Play` (`LevelSequenceActor.SequencePlayer` _outactor))
      (`KismetSystemLibrary.Delay` 3.5)
      (`GameplayStatics.PlaySound2D` "/Game/Audio/SFX/Player/SFX_JumpAssist.SFX_JumpAssist" 1.0 1.0 0.0 null null)
      (`KismetSystemLibrary.Delay` 1.2)
      (bind _returnvalue_2 (`|CreateWidget` "/Game/UI/WBP_FadeAnimWidget.WBP_FadeAnimWidget_C"))
      (`UserWidget.AddToViewport` _returnvalue_2 0)
      (`/Game/UI/WBP_FadeAnimWidget.PlayFadeOut` _returnvalue_2))))

(fn `UserConstructionScript`)
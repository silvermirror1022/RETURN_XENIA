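; Small avalanche rock Blueprint, built to travel along the spline of a referenced rock trail.
; A timeline with play rate set from a completion time lerps distance along the spline, setting world location and rotation at a fixed half scale.
; This movement logic is disconnected: ActivateRockFalling and BeginPlay are empty, so nothing in this graph runs it.
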(event `ActivateRockFalling`)

(event `self.ReceiveBeginPlay`)

(fn `UserConstructionScript`)
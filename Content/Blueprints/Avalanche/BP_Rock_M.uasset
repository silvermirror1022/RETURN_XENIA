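; BP_Rock_M is an avalanche rock actor that can be launched along the direction of its Arrow component.
; Its AddImpulse event applies a velocity-change impulse to the static mesh, scaled by the Force variable, and prints a debug message.
; Nothing in the graph calls that event; BeginPlay and Tick are empty, and alternative delayed-impulse and AddForce nodes are left disconnected.
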(event `AddImpulse`
  (`PrimitiveComponent.AddImpulse` (`self.StaticMesh`) (* (`SceneComponent.GetForwardVector` (`self.Arrow`)) (`self.Force`)) "None" true)
  (`KismetSystemLibrary.PrintText` "Impulsed!!"))

(event `self.ReceiveBeginPlay`)

(event `self.ReceiveTick`
  (params (DeltaSeconds :type "Float (single-precision)")))

(fn `UserConstructionScript`)
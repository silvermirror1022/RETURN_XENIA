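; Moving island platform that travels along a referenced spline and launches the player upward with a jump sound on box overlap.
; On BeginPlay it binds its activate and return events to the level's BP_MI_EventManager.
; Activation plays a Timeline, rate-scaled to the travel time, that lerps distance along the spline to set position.
; Return reverses the Timeline, with IsMoving gating both events, though only activation sets it true.
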(event `self.ReceiveBeginPlay`
  (bind _returnvalue (`GameplayStatics.GetActorOfClass` "/Game/Blueprints/Platformer/MovingIsland/BP_MI_EventManager.BP_MI_EventManager_C"))
  (add `/Game/Blueprints/Platformer/MovingIsland/BP_MI_EventManager.ActivateIsland` _returnvalue (`|CreateDelegate` :!event `ActivateMovingPlatform`))
  (add `/Game/Blueprints/Platformer/MovingIsland/BP_MI_EventManager.ReturnIsland` _returnvalue (`|CreateDelegate` :!event `ReturnMovingPlatform`)))

(event `ActivateMovingPlatform`
  (if (not (`self.bIsMoving`))
    (set `self.bIsMoving` true)
    (`/Engine/EditorBlueprintResources/StandardMacros.IsValid` (`self.SpineRef`)
      (:`Is Valid`
        (`TimelineComponent.SetPlayRate` (`self.Timeline`) (/ 1.0 (`self.TimeToComplete(Sec)`)))
        (bind (_direction _move) (`Timeline|Timeline`)
          (:`Update`
            (`self.K2_SetActorTransform` (`KismetMathLibrary.MakeTransform` (`SplineComponent.GetLocationAtDistanceAlongSpline` (`/Game/Blueprints/Platformer/BP_SplineActor.Spline` (`self.SpineRef`)) (`KismetMathLibrary.Lerp` 0.0 (`SplineComponent.GetSplineLength` (`/Game/Blueprints/Platformer/BP_SplineActor.Spline` (`self.SpineRef`))) _move) "World") (struct) (`self.GetActorScale3D`))))
          (:`Finished`
            (set `self.bIsMoving` false)))))))

(event `ReturnMovingPlatform`
  (if (not (`self.bIsMoving`))
    (`TimelineComponent.Reverse` (`self.Timeline`))
    (`KismetSystemLibrary.Delay` (`self.TimetoComplete(Sec)`))
    (set `self.bIsMoving` false)))

(event `self.Box.OnComponentBeginOverlap`
  (params (OverlappedComponent :type "PrimitiveComponent Object Reference") (OtherActor :type "Actor Object Reference") (OtherComp :type "PrimitiveComponent Object Reference") (OtherBodyIndex :type Integer) (bFromSweep :type Boolean) (SweepResult :type "HitResult Structure (by ref)"))
  (bind _asrxplayer (cast `RXPlayer` OtherActor))
  (`Character.LaunchCharacter` _asrxplayer (0.0 0.0 1850.0) true true)
  (`GameplayStatics.PlaySound2D` "/Game/Audio/SFX/Player/SC_Jump.SC_Jump" 1.0 1.0 0.0 null null))

(fn `UserConstructionScript`)
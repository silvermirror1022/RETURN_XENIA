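; Moving platform that travels back and forth along a referenced spline in a continuous loop.
; A Timeline, rate-scaled by TimeToCompleteSec, drives its location along the spline length; on finishing it reverses, waits that duration and reactivates.
; It starts on BeginPlay, destroying its trigger box, or, with IsDelayMovingObject set, after StartDelay once an RXPlayer overlaps the box.
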(event `self.ReceiveBeginPlay`
  (if (not (`self.IsDelayMovingObject`))
    (`self.ActivateMovingPlatform`)
    (`ActorComponent.K2_DestroyComponent` (`self.Box`))))

(event `ActivateMovingPlatform`
  (`/Engine/EditorBlueprintResources/StandardMacros.IsValid` (`self.SplineRef`)
    (:`Is Valid`
      (`TimelineComponent.SetPlayRate` (`self.Timeline`) (/ 1.0 (`self.TimeToComplete(Sec)`)))
      (bind (_direction _move) (`Timeline|Timeline`)
        (:`Update`
          (`self.K2_SetActorTransform` (`KismetMathLibrary.MakeTransform` (`SplineComponent.GetLocationAtDistanceAlongSpline` (`/Game/Blueprints/Platformer/BP_SplineActor.Spline` (`self.SplineRef`)) (`KismetMathLibrary.Lerp` 0.0 (`SplineComponent.GetSplineLength` (`/Game/Blueprints/Platformer/BP_SplineActor.Spline` (`self.SplineRef`))) _move) "World") (struct) (`self.GetActorScale3D`))))
        (:`Finished`
          (`TimelineComponent.ReverseFromEnd` (`self.Timeline`))
          (`KismetSystemLibrary.Delay` (`self.TimeToComplete(Sec)`))
          (`self.ActivateMovingPlatform`))))))

(event `DeactivateMovingPlatform`
  (`TimelineComponent.Stop` (`self.Timeline`)))

(event `self.Box.OnComponentBeginOverlap`
  (params (OverlappedComponent :type "PrimitiveComponent Object Reference") (OtherActor :type "Actor Object Reference") (OtherComp :type "PrimitiveComponent Object Reference") (OtherBodyIndex :type Integer) (bFromSweep :type Boolean) (SweepResult :type "HitResult Structure (by ref)"))
  (cast `RXPlayer` OtherActor)
  (`KismetSystemLibrary.Delay` (`self.StartDelay`))
  (`self.ActivateMovingPlatform`))

(fn `UserConstructionScript`)
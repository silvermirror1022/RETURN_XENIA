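; Platformer trap that periodically activates and stuns the RXPlayer standing inside its box trigger.
; A looping timer shows the particle effect and runs a fast check timer for half of each interval.
; A check that finds the player overlapping plays a hit montage and lock sound once per cycle and disables movement.
; When the active window ends, the effect hides, the check timer clears and walking movement is restored.
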(event `self.ReceiveBeginPlay`
  (`KismetSystemLibrary.K2_SetTimerDelegate` (delegate `ActivateVisualEffect`) (`self.Interval`) true)
  (`SceneComponent.SetVisibility` (`self.ParticleSystem`) false false))

(event `ActivateVisualEffect`
  (`SceneComponent.SetVisibility` (`self.ParticleSystem`) true false)
  (bind _returnvalue (`KismetSystemLibrary.K2_SetTimerDelegate` (delegate `ActivateTrap`) 0.2 true))
  (`KismetSystemLibrary.Delay` (/ (`self.Interval`) 2.0))
  (`SceneComponent.SetVisibility` (`self.ParticleSystem`) false false)
  (`KismetSystemLibrary.K2_ClearAndInvalidateTimerHandle` _returnvalue)
  (set `self.IsPlayedMontage` false)
  (bind _asrxplayer (cast `RXPlayer` (`GameplayStatics.GetPlayerCharacter` 0)))
  (`CharacterMovementComponent.SetMovementMode` (`Character.CharacterMovement` _asrxplayer) "MOVE_Walking" 0))

(event `ActivateTrap`
  (if (`self.IsOverlappedPlayer`)
    (bind _asrxplayer (cast `RXPlayer` (`GameplayStatics.GetPlayerCharacter` 0)))
    (if (not (`self.IsPlayedMontage`))
      (`AnimInstance.Montage_Play` (`SkeletalMeshComponent.GetAnimInstance` (`Character.Mesh` _asrxplayer)) "/Game/Animation/Player/AM_Hit.AM_Hit" 1.0 "MontageLength" 0.0 false)
      (set `self.IsPlayedMontage` true)
      (`CharacterMovementComponent.SetMovementMode` (`Character.CharacterMovement` _asrxplayer) "MOVE_None" 0)
      (`GameplayStatics.SpawnSoundAtLocation` "/Game/Audio/SFX/SFX_TrapLock.SFX_TrapLock" (`self.K2_GetActorLocation`) (struct) 1.0 1.0 0.0 null null))))

(event `self.Box.OnComponentBeginOverlap`
  (params (OverlappedComponent :type "PrimitiveComponent Object Reference") (OtherActor :type "Actor Object Reference") (OtherComp :type "PrimitiveComponent Object Reference") (OtherBodyIndex :type Integer) (bFromSweep :type Boolean) (SweepResult :type "HitResult Structure (by ref)"))
  (cast `RXPlayer` OtherActor)
  (set `self.IsOverlappedPlayer` true))

(event `self.Box.OnComponentEndOverlap`
  (params (OverlappedComponent :type "PrimitiveComponent Object Reference") (OtherActor :type "Actor Object Reference") (OtherComp :type "PrimitiveComponent Object Reference") (OtherBodyIndex :type Integer))
  (cast `RXPlayer` OtherActor)
  (set `self.IsOverlappedPlayer` false))

(fn `UserConstructionScript`)
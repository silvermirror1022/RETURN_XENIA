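; Platformer moving platform that travels back and forth along a referenced spline actor, starting at BeginPlay.
; A Timeline, with play rate scaled to the travel time, lerps distance along the spline and sets the actor's location and rotation each update.
; On finish it reverses, then a Delay of the travel time calls activation again to loop.
; A deactivate event stops the Timeline.
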(event `self.ReceiveBeginPlay`
  (`self.ActivateMovingPlatform`))

(event `ActivateMovingPlatform`
  (bind _spline (`/Game/Blueprints/Platformer/BP_SplineActor.Spline` (`self.SplineRef`)))
  (`/Engine/EditorBlueprintResources/StandardMacros.IsValid` (`self.SplineRef`)
    (:`Is Valid`
      (`TimelineComponent.SetPlayRate` (`self.Timeline`) (/ 1.0 (`self.TimeToComplete(Sec)`)))
      (bind (_direction _move) (`Timeline|Timeline`)
        (:`Update`
          (bind _returnvalue (`KismetMathLibrary.Lerp` 0.0 (`SplineComponent.GetSplineLength` (`/Game/Blueprints/Platformer/BP_SplineActor.Spline` (`self.SplineRef`))) _move))
          (`self.K2_SetActorTransform` (`KismetMathLibrary.MakeTransform` (`SplineComponent.GetLocationAtDistanceAlongSpline` _spline _returnvalue "World") (`SplineComponent.GetRotationAtDistanceAlongSpline` _spline _returnvalue "World"))))
        (:`Finished`
          (`TimelineComponent.Reverse` (`self.Timeline`))
          (`KismetSystemLibrary.Delay` (`self.TimeToComplete(Sec)`))
          (`self.ActivateMovingPlatform`))))))

(event `DeactivateMovingPlatform`
  (`TimelineComponent.Stop` (`self.Timeline`)))

(fn `UserConstructionScript`)
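; Periodic wind trap for the platformer that slows the player inside its box while active.
; A looping timer turns on particles and plays a wind sound, then shuts the effect off after half the interval.
; During that window, a fast polling timer reads the box overlap flag and sets walk speed to slowed or normal.
; Speed is not restored when the window closes, so a slowdown can persist until the next active phase.
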(event `self.ReceiveBeginPlay`
  (`KismetSystemLibrary.K2_SetTimerDelegate` (delegate `ActivateVisualEffect`) (`self.Interval`) true))

(event `ActivateVisualEffect`
  (`ActorComponent.Activate` (`self.ParticleSystem`) true)
  (`GameplayStatics.SpawnSoundAtLocation` "/Game/Audio/SFX/SFX_TrapWind.SFX_TrapWind" (`self.K2_GetActorLocation`) (struct) 1.0 1.0 0.0 "/Game/Audio/SFX/PlayerExperience/SA_RockSpot.SA_RockSpot" null)
  (bind _returnvalue (`KismetSystemLibrary.K2_SetTimerDelegate` (delegate `ActivateTrap`) 0.2 true))
  (`KismetSystemLibrary.Delay` (/ (`self.Interval`) 2.0))
  (`ActorComponent.Deactivate` (`self.ParticleSystem`))
  (`KismetSystemLibrary.K2_ClearAndInvalidateTimerHandle` _returnvalue))

(event `ActivateTrap`
  (bind _returnvalue (`GameplayStatics.GetPlayerCharacter` 0))
  (if (`self.IsOverlappedPlayer`)
    (bind _asrxplayer (cast `RXPlayer` _returnvalue))
    (set `CharacterMovementComponent.MaxWalkSpeed` 75.0 (`Character.CharacterMovement` _asrxplayer))
    (else
      (bind _asrxplayer_2 (cast `RXPlayer` _returnvalue))
      (set `CharacterMovementComponent.MaxWalkSpeed` 350.0 (`Character.CharacterMovement` _asrxplayer_2)))))

(event `self.Box.OnComponentBeginOverlap`
  (params (OverlappedComponent :type "PrimitiveComponent Object Reference") (OtherActor :type "Actor Object Reference") (OtherComp :type "PrimitiveComponent Object Reference") (OtherBodyIndex :type Integer) (bFromSweep :type Boolean) (SweepResult :type "HitResult Structure (by ref)"))
  (cast `RXPlayer` OtherActor)
  (set `self.IsOverlappedPlayer` true))

(event `self.Box.OnComponentEndOverlap`
  (params (OverlappedComponent :type "PrimitiveComponent Object Reference") (OtherActor :type "Actor Object Reference") (OtherComp :type "PrimitiveComponent Object Reference") (OtherBodyIndex :type Integer))
  (cast `RXPlayer` OtherActor)
  (set `self.IsOverlappedPlayer` false))

(fn `UserConstructionScript`)
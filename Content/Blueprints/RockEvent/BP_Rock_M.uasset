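; BP_Rock_M is a rock hazard for the rock event that damages and knocks back the player on contact.
; On BeginPlay it looks up the BP_RockPlayerImpulseDir actor as a direction target.
; When its mesh hits BP_Player, it applies damage through RXPlayerStatComponent and launches the character along the rock-to-target direction, scaled by ImpulseForce.
; It also prints a debug message on each player hit.
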(event `self.ReceiveBeginPlay`
  (bind _returnvalue (`GameplayStatics.GetActorOfClass` "/Game/Blueprints/RockEvent/BP_RockPlayerImpulseDir.BP_RockPlayerImpulseDir_C")))

(event `self.StaticMesh.OnComponentHit`
  (params (HitComponent :type "PrimitiveComponent Object Reference") (OtherActor :type "Actor Object Reference") (OtherComp :type "PrimitiveComponent Object Reference") (NormalImpulse :type "Vector Structure") (Hit :type "HitResult Structure (by ref)"))
  (bind _asbp_player (cast `/Game/Blueprints/Player/BP_Player` OtherActor))
  (`RXPlayerStatComponent.ApplyDamage` (`self.GetComponentByClass` _asbp_player "/Script/RETURN_XENIA.RXPlayerStatComponent") 1)
  (`Character.LaunchCharacter` _asbp_player (* (`KismetMathLibrary.GetDirectionUnitVector` (`self.K2_GetActorLocation`) (`self.K2_GetActorLocation` (stale `self.ReceiveBeginPlay` _returnvalue))) (`self.ImpulseForce`)) false false)
  (`KismetSystemLibrary.PrintText` "Rock Damaged!"))

(fn `UserConstructionScript`)
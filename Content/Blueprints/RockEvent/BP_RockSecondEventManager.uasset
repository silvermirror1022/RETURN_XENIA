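; Manager actor for the second rock event, a one-shot trigger box that plays a cutscene when the RXPlayer enters.
; On overlap it fades the screen, disables input, starts a level sequence and runs a delayed rock camera shake, then restores input and fades again.
; BeginPlay caches three tagged groups of Level 4 rock spawners, but nothing here uses them and ActivateFallingRock is empty.
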(event `self.ReceiveBeginPlay`
  (`|ExecutionSequence`
    (:`then_0`
      (bind _outactors (`GameplayStatics.GetAllActorsOfClassWithTag` "/Game/Blueprints/RockEvent/BP_RockSpawner.BP_RockSpawner_C" "RockLevel4_0"))
      (set `self.RockSpawner0` _outactors))
    (:`then_1`
      (bind _outactors_2 (`GameplayStatics.GetAllActorsOfClassWithTag` "/Game/Blueprints/RockEvent/BP_RockSpawner.BP_RockSpawner_C" "RockLevel4_1"))
      (set `self.RockSpawner1` _outactors_2))
    (:`then_2`
      (bind _outactors_3 (`GameplayStatics.GetAllActorsOfClassWithTag` "/Game/Blueprints/RockEvent/BP_RockSpawner.BP_RockSpawner_C" "RockLevel4_2"))
      (set `self.RockSpawner2` _outactors_3))))

(event `ActivateFallingRock`)

(event `self.Box.OnComponentBeginOverlap`
  (params (OverlappedComponent :type "PrimitiveComponent Object Reference") (OtherActor :type "Actor Object Reference") (OtherComp :type "PrimitiveComponent Object Reference") (OtherBodyIndex :type Integer) (bFromSweep :type Boolean) (SweepResult :type "HitResult Structure (by ref)"))
  (bind _fadewidget (`self.FadeWidget`))
  (bind _fadewidget_2 (`self.FadeWidget`))
  (if (not (`self.bIsTriggered`))
    (cast `RXPlayer` OtherActor)
    (set `self.bIsTriggered` true)
    (`UserWidget.AddToViewport` _fadewidget_2 0)
    (`/Game/UI/WBP_FadeAnimWidget.PlayFadeOut` _fadewidget_2)
    (`self.DisableInput` (`GameplayStatics.GetPlayerCharacter` 0) (`GameplayStatics.GetPlayerController` 0))
    (bind _outactor (`LevelSequencePlayer.CreateLevelSequencePlayer` null))
    (`MovieSceneSequencePlayer.Play` (`LevelSequenceActor.SequencePlayer` _outactor))
    (`KismetSystemLibrary.Delay` 4.0)
    (bind _returnvalue (`PlayerCameraManager.StartCameraShake` :`self` (`GameplayStatics.GetPlayerCameraManager` 0) :`ShakeClass` "/Game/Blueprints/RockEvent/BP_CameraShake_Rock.BP_CameraShake_Rock_C" :`Scale` 2.0))
    (`KismetSystemLibrary.Delay` 3.0)
    (`PlayerCameraManager.StopCameraShake` (`GameplayStatics.GetPlayerCameraManager` 0) _returnvalue false)
    (`self.EnableInput` (`GameplayStatics.GetPlayerCharacter` 0) (`GameplayStatics.GetPlayerController` 0))
    (`UserWidget.AddToViewport` _fadewidget 0)
    (`/Game/UI/WBP_FadeAnimWidget.PlayFadeOut` _fadewidget)))

(fn `UserConstructionScript`)
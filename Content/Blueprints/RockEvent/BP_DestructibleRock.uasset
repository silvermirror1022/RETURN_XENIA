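; BP_DestructibleRock is a falling-rock hazard built on a geometry collection that damages the player on contact.
; Physics stays off at BeginPlay until ActivateFallingRock enables simulation, then clears the IsActive flag after a delay.
; While IsActive is set, component hits on BP_Player apply damage through its RXPlayerStatComponent.
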(event `self.ReceiveBeginPlay`
  (`PrimitiveComponent.SetSimulatePhysics` (`self.GeometryCollection`) false))

(event `ActivateFallingRock`
  (`PrimitiveComponent.SetSimulatePhysics` (`self.GeometryCollection`) true)
  (`KismetSystemLibrary.Delay` 10.0)
  (set `self.bIsActive` false))

(event `self.GeometryCollection.OnComponentHit`
  (params (HitComponent :type "PrimitiveComponent Object Reference") (OtherActor :type "Actor Object Reference") (OtherComp :type "PrimitiveComponent Object Reference") (NormalImpulse :type "Vector Structure") (Hit :type "HitResult Structure (by ref)"))
  (if (`self.bIsActive`)
    (bind _asbp_player (cast `/Game/Blueprints/Player/BP_Player` OtherActor))
    (`RXPlayerStatComponent.ApplyDamage` (`self.GetComponentByClass` _asbp_player "/Script/RETURN_XENIA.RXPlayerStatComponent") 1)))

(fn `UserConstructionScript`)
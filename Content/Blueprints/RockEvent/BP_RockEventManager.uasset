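; Rock-fall event manager that starts a cutscene and repeating rock spawn patterns when the player first enters its trigger box.
; BeginPlay groups BP_RockSpawner actors by tag, and four pattern events spawn from these groups in delayed waves, with pattern 2 chaining into pattern 1.
; The trigger starts four looping timers and plays LS_RockEvent with fades, camera shake and locked input.
; StopAllRockEvent clears the timers and calls deactivation for all rocks.
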(event `OnPattern1`
  (`|ExecutionSequence`
    (:`then_0`
      (for _array_element (`self.Level0_1`)
        (`RXRockSpawner.SpawnRock` _array_element)))
    (:`then_1`
      ;[1 1 1] 페턴1시작시 각각 스폰 딜레이
      (`KismetSystemLibrary.Delay` 0.4)
      (for _array_element_2 (`self.Level0_4`)
        (`RXRockSpawner.SpawnRock` _array_element_2)))
    (:`then_2`
      (`KismetSystemLibrary.Delay` 0.6)
      (for _array_element_3 (`self.Level0_3`)
        (`RXRockSpawner.SpawnRock` _array_element_3)))
    (:`then_3`
      (`KismetSystemLibrary.Delay` 0.8)
      (for _array_element_4 (`self.Level0_2`)
        (`RXRockSpawner.SpawnRock` _array_element_4)))))

(event `OnPattern2`
  (for _array_element (`self.Level1`)
    (`RXRockSpawner.SpawnRock` _array_element)
    ;[1 1 1] 패턴2,3,4 딜레이
    (`KismetSystemLibrary.Delay` 2.0)
    (`self.OnPattern1`)))

(event `self.ReceiveBeginPlay`
  (`|ExecutionSequence`
    (:`then_0`
      ;[1 1 1] 해당월드에 배치한 태그를 여기서의 Level 액터로 기록.이를바탕으로 이 레벨 변수를 통해서 돌을 스폰함.
      (bind _outactors (`GameplayStatics.GetAllActorsOfClassWithTag` "/Game/Blueprints/RockEvent/BP_RockSpawner.BP_RockSpawner_C" "RockLevel0_1"))
      (set `self.Level0_1` _outactors))
    (:`then_1`
      (bind _outactors_2 (`GameplayStatics.GetAllActorsOfClassWithTag` "/Game/Blueprints/RockEvent/BP_RockSpawner.BP_RockSpawner_C" "RockLevel0_2"))
      (set `self.Level0_2` _outactors_2))
    (:`then_2`
      (bind _outactors_3 (`GameplayStatics.GetAllActorsOfClassWithTag` "/Game/Blueprints/RockEvent/BP_RockSpawner.BP_RockSpawner_C" "RockLevel0_3"))
      (set `self.Level0_3` _outactors_3))
    (:`then_3`
      (bind _outactors_4 (`GameplayStatics.GetAllActorsOfClassWithTag` "/Game/Blueprints/RockEvent/BP_RockSpawner.BP_RockSpawner_C" "RockLevel0_4"))
      (set `self.Level0_4` _outactors_4))
    (:`then_4`
      (bind _outactors_5 (`GameplayStatics.GetAllActorsOfClassWithTag` "/Game/Blueprints/RockEvent/BP_RockSpawner.BP_RockSpawner_C" "RockLevel1"))
      (set `self.Level1` _outactors_5))
    (:`then_5`
      (bind _outactors_6 (`GameplayStatics.GetAllActorsOfClassWithTag` "/Game/Blueprints/RockEvent/BP_RockSpawner.BP_RockSpawner_C" "RockLevel2"))
      (set `self.Level2` _outactors_6))
    (:`then_6`
      (bind _outactors_7 (`GameplayStatics.GetAllActorsOfClassWithTag` "/Game/Blueprints/RockEvent/BP_RockSpawner.BP_RockSpawner_C" "RockLevel3"))
      (set `self.Level3` _outactors_7))
    (:`then_7`
      (bind _outactors_8 (`GameplayStatics.GetAllActorsOfClassWithTag` "/Game/Blueprints/RockEvent/BP_RockSpawner.BP_RockSpawner_C" "RockLevel4_0"))
      (set `self.Level4_0` _outactors_8))
    (:`then_8`
      (bind _outactors_9 (`GameplayStatics.GetAllActorsOfClassWithTag` "/Game/Blueprints/RockEvent/BP_RockSpawner.BP_RockSpawner_C" "RockLevel4_1"))
      (set `self.Level4_1` _outactors_9))
    (:`then_9`
      (bind _outactors_10 (`GameplayStatics.GetAllActorsOfClassWithTag` "/Game/Blueprints/RockEvent/BP_RockSpawner.BP_RockSpawner_C" "RockLevel4_2"))
      (set `self.Level4_2` _outactors_10))))

(event `OnPattern3`
  (for _array_element (`self.Level3`)
    (`RXRockSpawner.SpawnRock` _array_element)
    ;[1 1 1] 패턴2,3,4 딜레이
    (`KismetSystemLibrary.Delay` 0.75)
    (for _array_element_2 (`self.Level2`)
      (`RXRockSpawner.SpawnRock` _array_element_2))))

(event `OnPattern4`
  (for _array_element (`self.Level4_0`)
    (`RXRockSpawner.SpawnRock` _array_element)
    ;[1 1 1] 패턴2,3,4 딜레이
    (`KismetSystemLibrary.Delay` 0.75)
    (for _array_element_2 (`self.Level4_1`)
      (`RXRockSpawner.SpawnRock` _array_element_2)
      (`KismetSystemLibrary.Delay` 1.0)
      (for _array_element_3 (`self.Level4_2`)
        (`RXRockSpawner.SpawnRock` _array_element_3)))))

(event `StopAllRockEvent`
  ;[1 1 1] 모든 락 이벤트를 초기화하는 함수 로직
  (`KismetSystemLibrary.K2_ClearAndInvalidateTimerHandle` (stale `self.Box.OnComponentBeginOverlap` _returnvalue))
  (`KismetSystemLibrary.K2_ClearAndInvalidateTimerHandle` (stale `self.Box.OnComponentBeginOverlap` _returnvalue_2))
  (`KismetSystemLibrary.K2_ClearAndInvalidateTimerHandle` (stale `self.Box.OnComponentBeginOverlap` _returnvalue_3))
  (`KismetSystemLibrary.K2_ClearAndInvalidateTimerHandle` (stale `self.Box.OnComponentBeginOverlap` _returnvalue_4))
  ;;[1 0.03854 0.03854] 스포너에게 델리게이트
  (`self.DeactivateAllRocks`))

(event `self.Box.OnComponentBeginOverlap`
  (params (OverlappedComponent :type "PrimitiveComponent Object Reference") (OtherActor :type "Actor Object Reference") (OtherComp :type "PrimitiveComponent Object Reference") (OtherBodyIndex :type Integer) (bFromSweep :type Boolean) (SweepResult :type "HitResult Structure (by ref)"))
  (if (not (`self.bIsTriggered`))
    (cast `RXPlayer` OtherActor)
    (`self.PlayLevelSequence`)
    (set `self.bIsTriggered` true)
    (`self.StopAllRockEvent`)
    ;[1 1 1] Looping 체크가 되어있어야 계쏙 이벤트동안 스폰을함. 이니셜스타티딜레이는 이벤트시작후 스폰되기시작하는애들 아래 createEvent를 통해 패턴이 시작되는거임
    (bind _returnvalue (`KismetSystemLibrary.K2_SetTimerDelegate` (`|CreateDelegate` :!event `OnPattern1`) 5.0 true))
    (bind _returnvalue_2 (`KismetSystemLibrary.K2_SetTimerDelegate` (`|CreateDelegate` :!event `OnPattern2`) 4.5 true false 1.0))
    (bind _returnvalue_3 (`KismetSystemLibrary.K2_SetTimerDelegate` (`|CreateDelegate` :!event `OnPattern3`) 7.0 true false 5.0))
    (bind _returnvalue_4 (`KismetSystemLibrary.K2_SetTimerDelegate` (`|CreateDelegate` :!event `OnPattern4`) 5.0 true false 1.0))))

(event `PlayLevelSequence`
  (bind _fadewidget (`self.FadeWidget`))
  (bind _fadewidget_2 (`self.FadeWidget`))
  (`UserWidget.AddToViewport` _fadewidget_2 0)
  (`/Game/UI/WBP_FadeAnimWidget.PlayFadeOut` _fadewidget_2)
  (`self.DisableInput` (`GameplayStatics.GetPlayerCharacter` 0) (`GameplayStatics.GetPlayerController` 0))
  (bind _outactor (`LevelSequencePlayer.CreateLevelSequencePlayer` "/Game/Cinematics/LS_RockEvent.LS_RockEvent"))
  (`MovieSceneSequencePlayer.Play` (`LevelSequenceActor.SequencePlayer` _outactor))
  (`KismetSystemLibrary.Delay` 4.0)
  (bind _returnvalue (`PlayerCameraManager.StartCameraShake` :`self` (`GameplayStatics.GetPlayerCameraManager` 0) :`ShakeClass` "/Game/Blueprints/RockEvent/BP_CameraShake_Rock.BP_CameraShake_Rock_C" :`Scale` 2.0))
  (`KismetSystemLibrary.Delay` 5.0)
  (`PlayerCameraManager.StopCameraShake` (`GameplayStatics.GetPlayerCameraManager` 0) _returnvalue false)
  (`self.EnableInput` (`GameplayStatics.GetPlayerCharacter` 0) (`GameplayStatics.GetPlayerController` 0))
  (`UserWidget.AddToViewport` _fadewidget 0)
  (`/Game/UI/WBP_FadeAnimWidget.PlayFadeOut` _fadewidget))

(fn `UserConstructionScript`)
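; Manager for a rock-fall event that triggers tagged BP_RockSpawner actors in timed patterns.
; BeginPlay caches spawners into per-tag arrays and starts two looping timers to drive the patterns.
; Pattern 1 fires the Level0 groups in a staggered order; pattern 2 fires Level1, then chains into pattern 1 after a delay.
; Level2 is cached but unused, and the box-overlap shutdown logic is disconnected.
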(event `OnPattern1`
  (`|ExecutionSequence`
    (:`then_0`
      (for _array_element (`self.Level0_1`)
        (`RXRockSpawner.SpawnRock` _array_element)))
    (:`then_1`
      ;[1 1 1] 페턴1시작시 각각 스폰 딜레이
      (`KismetSystemLibrary.Delay` 0.4)
      (for _array_element_2 (`self.Level0_4`)
        (`RXRockSpawner.SpawnRock` _array_element_2)))
    (:`then_2`
      (`KismetSystemLibrary.Delay` 0.6)
      (for _array_element_3 (`self.Level0_3`)
        (`RXRockSpawner.SpawnRock` _array_element_3)))
    (:`then_3`
      (`KismetSystemLibrary.Delay` 0.8)
      (for _array_element_4 (`self.Level0_2`)
        (`RXRockSpawner.SpawnRock` _array_element_4)))))

(event `OnPattern2`
  (for _array_element (`self.Level1`)
    (`RXRockSpawner.SpawnRock` _array_element)
    (`KismetSystemLibrary.Delay` 2.0)
    (`self.OnPattern1`)))

(event `self.ReceiveBeginPlay`
  (`|ExecutionSequence`
    (:`then_0`
      ;[1 1 1] 해당월드에 배치한 태그를 여기서의 Level 액터로 기록.이를바탕으로 이 레벨 변수를 통해서 돌을 스폰함.
      (bind _outactors (`GameplayStatics.GetAllActorsOfClassWithTag` "/Game/Blueprints/RockEvent/BP_RockSpawner.BP_RockSpawner_C" "RockLevel0_1"))
      (set `self.Level0_1` _outactors))
    (:`then_1`
      (bind _outactors_2 (`GameplayStatics.GetAllActorsOfClassWithTag` "/Game/Blueprints/RockEvent/BP_RockSpawner.BP_RockSpawner_C" "RockLevel0_2"))
      (set `self.Level0_2` _outactors_2))
    (:`then_2`
      (bind _outactors_3 (`GameplayStatics.GetAllActorsOfClassWithTag` "/Game/Blueprints/RockEvent/BP_RockSpawner.BP_RockSpawner_C" "RockLevel0_3"))
      (set `self.Level0_3` _outactors_3))
    (:`then_3`
      (bind _outactors_4 (`GameplayStatics.GetAllActorsOfClassWithTag` "/Game/Blueprints/RockEvent/BP_RockSpawner.BP_RockSpawner_C" "RockLevel0_4"))
      (set `self.Level0_4` _outactors_4))
    (:`then_4`
      (bind _outactors_5 (`GameplayStatics.GetAllActorsOfClassWithTag` "/Game/Blueprints/RockEvent/BP_RockSpawner.BP_RockSpawner_C" "RockLevel1"))
      (set `self.Level1` _outactors_5))
    (:`then_5`
      (bind _outactors_6 (`GameplayStatics.GetAllActorsOfClassWithTag` "/Game/Blueprints/RockEvent/BP_RockSpawner.BP_RockSpawner_C" "RockLevel2"))
      (set `self.Level2` _outactors_6))
    (:`then_6`
      ;[1 1 1] Looping 체크가 되어있어야 계쏙 이벤트동안 스폰을함. 이니셜스타티딜레이는 이벤트시작후 스폰되기시작하는애들 아래 createEvent를 통해 패턴이 시작되는거임
      (bind _returnvalue (`KismetSystemLibrary.K2_SetTimerDelegate` (`|CreateDelegate` :!event `OnPattern1`) 5.0 true))
      (bind _returnvalue_2 (`KismetSystemLibrary.K2_SetTimerDelegate` (`|CreateDelegate` :!event `OnPattern2`) 4.5 true false 1.0)))))

(event `StopAllRockEvent`
  ;[1 1 1] 모든 락 이벤트를 초기화하는 함수 로직
  (`KismetSystemLibrary.K2_ClearAndInvalidateTimerHandle` (stale `self.ReceiveBeginPlay` _returnvalue))
  (`KismetSystemLibrary.K2_ClearAndInvalidateTimerHandle` (stale `self.ReceiveBeginPlay` _returnvalue_2)))

(event `self.Box.OnComponentBeginOverlap`
  (params (OverlappedComponent :type "PrimitiveComponent Object Reference") (OtherActor :type "Actor Object Reference") (OtherComp :type "PrimitiveComponent Object Reference") (OtherBodyIndex :type Integer) (bFromSweep :type Boolean) (SweepResult :type "HitResult Structure (by ref)")))

(fn `UserConstructionScript`)
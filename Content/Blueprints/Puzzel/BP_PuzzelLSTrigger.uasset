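; BP_PuzzelLSTrigger is a box trigger that plays a submap's intro level sequence when the player enters, if that submap's puzzle is not yet acquired.
; A DoOnce-gated overlap uses PuzzelMapType to select which puzzle status to query in RXGameInstance.
; PlayLevelSequence runs a fade-out, disables player input and plays the matching sequence.
; After a fixed delay, rather than a finished callback, it restores input and runs the fade-out again.
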(event `self.ReceiveBeginPlay`
  (bind _asrxgame_instance (cast `RXGameInstance` (`GameplayStatics.GetGameInstance`)))
  (set `self.RXGame Instance` _asrxgame_instance))

(event `PlayLevelSequence`
  (bind _fadewidget (`self.FadeWidget`))
  (bind _fadewidget_2 (`self.FadeWidget`))
  (`UserWidget.AddToViewport` _fadewidget 0)
  (`/Game/UI/WBP_FadeAnimWidget.PlayFadeOut` _fadewidget)
  (`self.DisableInput` (`GameplayStatics.GetPlayerCharacter` 0) (`GameplayStatics.GetPlayerController` 0))
  (switch `name` (`self.PuzzelMapType`)
    (:`submap1`
      (bind _outactor (`LevelSequencePlayer.CreateLevelSequencePlayer` "/Game/Cinematics/LS_submap1.LS_submap1"))
      (`MovieSceneSequencePlayer.Play` (`LevelSequenceActor.SequencePlayer` _outactor))
      (`KismetSystemLibrary.Delay` 5.0))
    (:`submap2`
      (bind _outactor_2 (`LevelSequencePlayer.CreateLevelSequencePlayer` "/Game/Cinematics/LS_submap2.LS_submap2"))
      (`MovieSceneSequencePlayer.Play` (`LevelSequenceActor.SequencePlayer` _outactor_2))
      (`KismetSystemLibrary.Delay` 5.0))
    (:`submap3`
      (bind _outactor_3 (`LevelSequencePlayer.CreateLevelSequencePlayer` "/Game/Cinematics/LS_submap3.LS_submap3"))
      (`MovieSceneSequencePlayer.Play` (`LevelSequenceActor.SequencePlayer` _outactor_3))
      (`KismetSystemLibrary.Delay` 5.0))
    (:`submap4`
      (bind _outactor_4 (`LevelSequencePlayer.CreateLevelSequencePlayer` "/Game/Cinematics/LS_submap4.LS_submap4"))
      (`MovieSceneSequencePlayer.Play` (`LevelSequenceActor.SequencePlayer` _outactor_4))
      (`KismetSystemLibrary.Delay` 5.0))
    (:`submap5`
      (bind _outactor_5 (`LevelSequencePlayer.CreateLevelSequencePlayer` "/Game/Cinematics/LS_submap5.LS_submap5"))
      (`MovieSceneSequencePlayer.Play` (`LevelSequenceActor.SequencePlayer` _outactor_5))
      (`KismetSystemLibrary.Delay` 5.0)))
  (`self.EnableInput` (`GameplayStatics.GetPlayerCharacter` 0) (`GameplayStatics.GetPlayerController` 0))
  (`UserWidget.AddToViewport` _fadewidget_2 0)
  (`/Game/UI/WBP_FadeAnimWidget.PlayFadeOut` _fadewidget_2))

(event `self.Box.OnComponentBeginOverlap`
  (params (OverlappedComponent :type "PrimitiveComponent Object Reference") (OtherActor :type "Actor Object Reference") (OtherComp :type "PrimitiveComponent Object Reference") (OtherBodyIndex :type Integer) (bFromSweep :type Boolean) (SweepResult :type "HitResult Structure (by ref)"))
  (cast `RXPlayer` OtherActor)
  (`/Engine/EditorBlueprintResources/StandardMacros.DoOnce` false
    (:`Completed`
      (switch `name` (`self.PuzzelMapType`)
        (:`submap1`
          (if (not (`RXGameInstance.IsPuzzelStatusAcquired` (`self.RXGame Instance`) "PushablePuzzel"))
            (`self.PlayLevelSequence` :!label _label)))
        (:`submap2`
          (if (not (`RXGameInstance.IsPuzzelStatusAcquired` (`self.RXGame Instance`) "BlindPuzzel"))
            (goto _label)))
        (:`submap3`
          (if (not (`RXGameInstance.IsPuzzelStatusAcquired` (`self.RXGame Instance`) "PatternPuzzel"))
            (goto _label)))
        (:`submap4`
          (if (not (`RXGameInstance.IsPuzzelStatusAcquired` (`self.RXGame Instance`) "TimingPuzzel"))
            (goto _label)))
        (:`submap5`
          (if (not (`RXGameInstance.IsPuzzelStatusAcquired` (`self.RXGame Instance`) "EulerPuzzel"))
            (goto _label)))))))

(fn `UserConstructionScript`)
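; Puzzle start component that switches the player into and out of puzzle mode.
; StartPuzzelMode and EndPuzzelMode override C++ BlueprintNativeEvents, swapping the RXPlayerController's Enhanced Input context between IMC_Default and IMC_Puzzel.
; Each then calls its parent implementation (noted as handling camera and shadow setup on start) and plays a fade-out on a newly created WBP_FadeAnimWidget.
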(event `self.StartPuzzelMode`
  ;[1 1 1] 퍼즐모드 시작 : BlueprintNativeEvent
  (bind _asrxplayer_controller (cast `RXPlayerController` (`GameplayStatics.GetPlayerController` 0)))
  (bind _returnvalue (pcsubsystem `EnhancedInputLocalPlayerSubsystem` _asrxplayer_controller))
  (`EnhancedInputSubsystemInterface.RemoveMappingContext` _returnvalue "/Game/Input/IMC_Default.IMC_Default" (struct))
  (`EnhancedInputSubsystemInterface.AddMappingContext` _returnvalue "/Game/Input/IMC_Puzzel.IMC_Puzzel" 0 (struct))
  (`parent.StartPuzzelMode`) ; 블루프린트네이티브이벤트로 C++에서 카메라 셋팅, 그림자 셋팅 호출
  (bind _returnvalue_2 (`|CreateWidget` "/Game/UI/WBP_FadeAnimWidget.WBP_FadeAnimWidget_C"))
  (`UserWidget.AddToViewport` _returnvalue_2 0)
  (`/Game/UI/WBP_FadeAnimWidget.PlayFadeOut` _returnvalue_2))

(event `self.EndPuzzelMode`
  ;[1 1 1] 퍼즐모드 해제 : BlueprintNativeEvent
  (bind _asrxplayer_controller (cast `RXPlayerController` (`GameplayStatics.GetPlayerController` 0)))
  (bind _returnvalue (pcsubsystem `EnhancedInputLocalPlayerSubsystem` _asrxplayer_controller))
  (`EnhancedInputSubsystemInterface.RemoveMappingContext` _returnvalue "/Game/Input/IMC_Puzzel.IMC_Puzzel" (struct))
  (`EnhancedInputSubsystemInterface.AddMappingContext` _returnvalue "/Game/Input/IMC_Default.IMC_Default" 0 (struct))
  (`parent.EndPuzzelMode`)
  (bind _returnvalue_2 (`|CreateWidget` "/Game/UI/WBP_FadeAnimWidget.WBP_FadeAnimWidget_C"))
  (`UserWidget.AddToViewport` _returnvalue_2 0)
  (`/Game/UI/WBP_FadeAnimWidget.PlayFadeOut` _returnvalue_2))
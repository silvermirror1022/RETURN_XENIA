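; BP_TemplePuzzel is the temple puzzle event actor, which activates level 1 of its spawn manager component when the event starts.
; On finish it removes its puzzle, wall and interaction components, moves the player to BP_PuzzelClearPos, then after a delay plays a rock sound and triggers BP_PachaStatue.
; On BeginPlay, a TemplePuzzel status already acquired in RXGameInstance removes those components and both block actors, so a solved puzzle stays cleared.
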(event `self.ReceiveBeginPlay`
  ;[1 1 1] 템플퍼즐 푼후 다시들어올 때 익셉션  디스트로이처리
  (bind _asrxgame_instance (cast `RXGameInstance` (`GameplayStatics.GetGameInstance`)))
  (if (`RXGameInstance.IsPuzzelStatusAcquired` _asrxgame_instance "TemplePuzzel")
    (`ActorComponent.K2_DestroyComponent` (`self.BP_PuzzelEventManageComponent`))
    (`ActorComponent.K2_DestroyComponent` (`self.SM_InvisibleWall`))
    (`ActorComponent.K2_DestroyComponent` (`self.SM_InvisibleEdge`))
    (`ActorComponent.K2_DestroyComponent` (`self.BP_TempleSpawnManageComponent`))
    (`ActorComponent.K2_DestroyComponent` (`self.SM_Interaction`))
    (`self.K2_DestroyActor` (`self.Blocks1`))
    (`self.K2_DestroyActor` (`self.Blocks2`))))

(event `self.PuzzelEventStart`
  ;[1 1 1] 템플퍼즐이벤트 시작
  (`parent.PuzzelEventStart`)
  (`RXPuzzelSpawnManageComponent.ActivateLevel` (`self.BP_TempleSpawnManageComponent`) 1))

(event `self.PuzzelEventFinish`
  ;[1 1 1] 퍼즐클리어시 관련 기능 컴포넌트 모두 삭제
  (`parent.PuzzelEventFinish`)
  (`ActorComponent.K2_DestroyComponent` (`self.BP_PuzzelEventManageComponent`))
  (`ActorComponent.K2_DestroyComponent` (`self.SM_InvisibleWall`))
  (`ActorComponent.K2_DestroyComponent` (`self.SM_InvisibleEdge`))
  (`ActorComponent.K2_DestroyComponent` (`self.BP_TempleSpawnManageComponent`))
  (`ActorComponent.K2_DestroyComponent` (`self.SM_Interaction`))
  (bind _returnvalue (`GameplayStatics.GetActorOfClass` "/Game/Blueprints/Puzzel/BP_PuzzelClearPos.BP_PuzzelClearPos_C"))
  (`self.K2_SetActorTransform` (`GameplayStatics.GetPlayerCharacter` 0) (`self.GetTransform` _returnvalue) false false)
  (`KismetSystemLibrary.Delay` 1.5)
  (`GameplayStatics.PlaySound2D` "/Game/Audio/SFX/SFX_MoveRock.SFX_MoveRock" 1.0 1.0 0.0 null null)
  (bind _returnvalue_2 (`GameplayStatics.GetActorOfClass` "/Game/Blueprints/ETC/BP_PachaStatue.BP_PachaStatue_C"))
  (`/Game/Blueprints/ETC/BP_PachaStatue.StartEvent` _returnvalue_2))

(fn `UserConstructionScript`)
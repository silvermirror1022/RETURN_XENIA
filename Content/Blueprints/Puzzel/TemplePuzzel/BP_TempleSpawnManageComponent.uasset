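; Temple puzzle level manager component that tracks the current trigger color and advances the player through four color-based levels, extending parent reset and startup logic.
; BeginPlay binds to five colored trigger actors' pass-color dispatchers to follow the active color.
; Helper events activate tagged green triggers and changing tiles.
; GoNextLevel checks the cleared-color count, then activates the next level or ends puzzle mode and records completion in the GameInstance.
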(event `SetActiveToAllTriggerActor`
  (bind _outactors (`GameplayStatics.GetAllActorsOfClassWithTag` "/Game/Blueprints/Puzzel/TemplePuzzel/BP_Puzzel_TempleGreenTrigger.BP_Puzzel_TempleGreenTrigger_C" "UnderwayPuzzel"))
  (for _array_element _outactors
    (set `/Game/Blueprints/Puzzel/TemplePuzzel/BP_Puzzel_TempleGreenTrigger.bIsActive` true _array_element)))

(event `SetActiveToChangingTile`
  (bind _outactors (`GameplayStatics.GetAllActorsOfClass` "/Game/Blueprints/Puzzel/TemplePuzzel/BP_Puzzel_Temple_ChangingTile.BP_Puzzel_Temple_ChangingTile_C"))
  (for _array_element _outactors
    (set `/Game/Blueprints/Puzzel/TemplePuzzel/BP_Puzzel_Temple_ChangingTile.bIsTileTriggerActive` true _array_element)))

(event `GoNextLevel`
  ;[1 1 1] 클리어조건이 아니면 False : Nothing
  (bind _isclear (`self.CheckClearCondition` (`self.CurrentLevelID`)))
  (if _isclear
    ;[1 1 1] 레벨1~3(false)면 다음 레벨로 레벨 1증가 후 ActivatelLevel , 레벨4(true)면 이벤트 종료
    (if (== (`self.CurrentLevelID`) 4)
      (`RXPuzzelEventManageComponent.EndPuzzelMode` (`Actor.GetComponentByClass` (`self.GetOwner`) "/Game/Blueprints/Puzzel/BP_PuzzelEventManageComponent.BP_PuzzelEventManageComponent_C"))
      ;[1 1 1] 게임 인스턴스에 클리어 조건 상태 전달
      (bind _asrxgame_instance (cast `RXGameInstance` (`GameplayStatics.GetGameInstance`)))
      (`RXGameInstance.SetPuzzelStatusAcquired` _asrxgame_instance "TemplePuzzel")
      (else
        (bind _result (`/Engine/EditorBlueprintResources/StandardMacros.IncrementInt` (`self.CurrentLevelID`))
          (:`  `
            (`self.ActivateLevel` _result)))))))

(event `self.ResetCurrentLevel`
  (`parent.ResetCurrentLevel`)
  (set `self.ClearColorNum` 0)
  (set `self.CurrentTriggerColor` "None"))

(event `SetTriggerColor`
  (params (CurrentColor :type Name))
  (set `self.CurrentTriggerColor` CurrentColor))

(event `self.ReceiveBeginPlay`
  (`parent.ReceiveBeginPlay`)
  (`|ExecutionSequence`
    (:`then_0`
      ;[1 1 1] 현재 진행중인 플레이어의 색을 바인딩 하는 로직
      (bind _returnvalue (`GameplayStatics.GetActorOfClass` "/Game/Blueprints/Puzzel/TemplePuzzel/BP_Puzzel_TempleRedTrigger.BP_Puzzel_TempleRedTrigger_C"))
      (`/Engine/EditorBlueprintResources/StandardMacros.IsValid` _returnvalue
        (:`Is Valid`
          (add `/Game/Blueprints/Puzzel/TemplePuzzel/BP_Puzzel_TempleRedTrigger.PassTriggerRedColor` _returnvalue (`|CreateDelegate` :!event `SetTriggerColor`)))))
    (:`then_1`
      (bind _returnvalue_2 (`GameplayStatics.GetActorOfClass` "/Game/Blueprints/Puzzel/TemplePuzzel/BP_Puzzel_TempleBlueTrigger.BP_Puzzel_TempleBlueTrigger_C"))
      (`/Engine/EditorBlueprintResources/StandardMacros.IsValid` _returnvalue_2
        (:`Is Valid`
          (add `/Game/Blueprints/Puzzel/TemplePuzzel/BP_Puzzel_TempleBlueTrigger.PassTriggerBlueColor` _returnvalue_2 (`|CreateDelegate` :!event `SetTriggerColor`)))))
    (:`then_2`
      (bind _returnvalue_3 (`GameplayStatics.GetActorOfClass` "/Game/Blueprints/Puzzel/TemplePuzzel/BP_Puzzel_TempleGreenTrigger.BP_Puzzel_TempleGreenTrigger_C"))
      (`/Engine/EditorBlueprintResources/StandardMacros.IsValid` _returnvalue_3
        (:`Is Valid`
          (add `/Game/Blueprints/Puzzel/TemplePuzzel/BP_Puzzel_TempleGreenTrigger.PassTriggerGreenColor` _returnvalue_3 (`|CreateDelegate` :!event `SetTriggerColor`)))))
    (:`then_3`
      (bind _returnvalue_4 (`GameplayStatics.GetActorOfClass` "/Game/Blueprints/Puzzel/TemplePuzzel/BP_Puzzel_TemplePurpleTrigger.BP_Puzzel_TemplePurpleTrigger_C"))
      (`/Engine/EditorBlueprintResources/StandardMacros.IsValid` _returnvalue_4
        (:`Is Valid`
          (add `/Game/Blueprints/Puzzel/TemplePuzzel/BP_Puzzel_TemplePurpleTrigger.PassTriggerPurpleColor` _returnvalue_4 (`|CreateDelegate` :!event `SetTriggerColor`)))))
    (:`then_4`
      (bind _returnvalue_5 (`GameplayStatics.GetActorOfClass` "/Game/Blueprints/Puzzel/TemplePuzzel/BP_Puzzel_TempleYellowTrigger.BP_Puzzel_TempleYellowTrigger_C"))
      (`/Engine/EditorBlueprintResources/StandardMacros.IsValid` _returnvalue_5
        (:`Is Valid`
          (add `/Game/Blueprints/Puzzel/TemplePuzzel/BP_Puzzel_TempleYellowTrigger.PassTriggerYellowColor` _returnvalue_5 (`|CreateDelegate` :!event `SetTriggerColor`)))))))

(fn `CheckClearCondition`
  (params (CurrentLevelNum :type Integer))
  (returns (IsClear :type Boolean))
  ;[1 1 1] 클리어 조건 레벨 1,2 ->4 ,  2,3->5
  (switch `int` CurrentLevelNum
    (:`1`
      _)
    (:`2`
      _)
    (:`3`
      (if (== (`self.ClearColorNum`) 5) :!label _label
        (return true)
        (else
          (return false))))
    (:`4`
      (goto _label)))
  (if (== (`self.ClearColorNum`) 4)
    (return true)
    (else
      (return false))))
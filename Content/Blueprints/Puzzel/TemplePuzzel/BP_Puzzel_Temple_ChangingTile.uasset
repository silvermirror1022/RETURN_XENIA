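; Color-changing floor tile for the temple puzzle, painted when the player steps on it.
; While the tile is trigger-active, overlap reads CurrentTriggerColor from BP_TemplePuzzel's spawn manage component, stores it as an actor tag and swaps the mesh material to match.
; Stepping on a tile already flagged color-completed also resets the current level.
; ResetObjectState extends the parent reset, restoring the default material and clearing flags and color tags.
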(event `PlayerTriggerColor`
  (bind _sm_tile (`self.SM_Tile`))
  (bind _sm_tile_2 (`self.SM_Tile`))
  ;[1 1 1] 현재 플레이어의 트리거색으로 색을 바꿔줌 + current trigger color -> actor tag add
  (bind _returnvalue (`GameplayStatics.GetActorOfClass` "/Game/Blueprints/Puzzel/TemplePuzzel/BP_TemplePuzzel.BP_TemplePuzzel_C"))
  (bind _currenttriggercolor (`/Game/Blueprints/Puzzel/TemplePuzzel/BP_TempleSpawnManageComponent.CurrentTriggerColor` (`self.GetComponentByClass` _returnvalue "/Game/Blueprints/Puzzel/TemplePuzzel/BP_TempleSpawnManageComponent.BP_TempleSpawnManageComponent_C")))
  (`KismetArrayLibrary.Array_Add` (`self.Tags`) _currenttriggercolor)
  (switch `name` _currenttriggercolor
    (:`Default`
      (`KismetSystemLibrary.PrintText` "Player didn't trigger colorTrigger"))
    (:`Red`
      (`PrimitiveComponent.SetMaterial` _sm_tile 0 "/Game/Designer/Materials/MI_TemplePuzzel_A04.MI_TemplePuzzel_A04"))
    (:`Green`
      (`PrimitiveComponent.SetMaterial` _sm_tile 0 "/Game/Designer/Materials/MI_TemplePuzzel_A01.MI_TemplePuzzel_A01"))
    (:`Blue`
      (`PrimitiveComponent.SetMaterial` _sm_tile_2 0 "/Game/Designer/Materials/MI_TemplePuzzel_A02.MI_TemplePuzzel_A02"))
    (:`Yellow`
      (`PrimitiveComponent.SetMaterial` _sm_tile_2 0 "/Game/Designer/Materials/MI_TemplePuzzel_A05.MI_TemplePuzzel_A05"))
    (:`Purple`
      (`PrimitiveComponent.SetMaterial` (`self.SM_Tile`) 0 "/Game/Designer/Materials/MI_TemplePuzzel_A03.MI_TemplePuzzel_A03"))))

(event `ResetAllState`
  (bind _tags (`self.Tags`))
  ;[1 1 1] 속성 값들을 초기화하는 함수 -> 색을 원래의 색으로 변경, 완성된 색 타일이 있다면 변수 초기화, 태그에 추가된 색 초기화, 머터리얼 색 복구
  (`PrimitiveComponent.SetMaterial` (`self.SM_Tile`) 0 "/Game/Designer/Modeling/puzzel/WorldGridMaterial.WorldGridMaterial")
  (set `self.bIsTileTriggerActive` false)
  (set `self.bIsTileColorCompleted` false)
  (for _array_element (`self.AllColorRefer`)
    (if (`KismetArrayLibrary.Array_Contains` _tags _array_element)
      (`KismetArrayLibrary.Array_RemoveItem` _tags _array_element))))

(event `self.ResetObjectState`
  (`parent.ResetObjectState`)
  (`self.ResetAllState`))

(event `self.Box.OnComponentBeginOverlap`
  (params (OverlappedComponent :type "PrimitiveComponent Object Reference") (OtherActor :type "Actor Object Reference") (OtherComp :type "PrimitiveComponent Object Reference") (OtherBodyIndex :type Integer) (bFromSweep :type Boolean) (SweepResult :type "HitResult Structure (by ref)"))
  (cast `RXPlayer` OtherActor)
  ;[1 1 1 1 15] Trigger를 밟으면 모든 IsTileTriggerActive가 true가 됨. false인 경우는 Nothing 상태임
  (if (`self.bIsTileTriggerActive`)
    (`self.PlayerTriggerColor`)
    (if (`self.bIsTileColorCompleted`)
      (bind _returnvalue (`GameplayStatics.GetActorOfClass` "/Game/Blueprints/Puzzel/TemplePuzzel/BP_TemplePuzzel.BP_TemplePuzzel_C"))
      (`RXPuzzelSpawnManageComponent.ResetCurrentLevel` (`self.GetComponentByClass` _returnvalue "/Game/Blueprints/Puzzel/TemplePuzzel/BP_TempleSpawnManageComponent.BP_TempleSpawnManageComponent_C")))))

(fn `UserConstructionScript`)
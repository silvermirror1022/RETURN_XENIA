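; Yellow endpoint trigger for the temple line-drawing puzzle, where the player connects two triggers of the same color.
; The first player overlap passes Yellow on and activates all triggers and tiles through BP_TempleSpawnManageComponent.
; A later overlap at the other Yellow endpoint completes Yellow-tagged tiles and calls GoNextLevel, while a wrong color or the starting trigger resets the level.
; The color is hard-coded, with comments marking what other color variants must change.
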(event `self.ResetObjectState`
  (`parent.ResetObjectState`)
  ;[1 1 1 1 15] IsActive: 플레이어가 아무 트리거도 안밟은 상태인지? / IsTriggeredAgain: this 트리거를 밟은 상태로 다시 같은 this 트리거를 밟았는지? / IsCompleted: 한줄긋기를 완료한 trigger인지?
  (set `self.bIsActive` false)
  (set `self.bIsTriggeredAgain` true)
  (set `self.bIsCompleted` false))

(event `self.Box.OnComponentBeginOverlap`
  (params (OverlappedComponent :type "PrimitiveComponent Object Reference") (OtherActor :type "Actor Object Reference") (OtherComp :type "PrimitiveComponent Object Reference") (OtherBodyIndex :type Integer) (bFromSweep :type Boolean) (SweepResult :type "HitResult Structure (by ref)"))
  ;[1 1 1 1 15] IsCompleted -> true : nothing / IsActive -> False : 플레이어가 처음으로 트리거->활성화상태 True: 플레이어가 이미 경로를 긋고 있는상황
  (cast `RXPlayer` OtherActor)
  (if (`self.bIsCompleted`)
    _
    (elif (`self.bIsActive`)
      ;[1 1 1 1 15] 같은색으로 들어온경우-> 서로 잇기 종료, 다른색 -> 초기화
      (bind _newparam (`self.IsSameColor`))
      (if _newparam
        ;[1 1 1] 같은색? this 트리거와 다른 객체인지 확인
        (if (`self.bIsTriggeredAgain`)
          (bind _returnvalue (`GameplayStatics.GetActorOfClass` "/Game/Blueprints/Puzzel/TemplePuzzel/BP_TemplePuzzel.BP_TemplePuzzel_C"))
          (bind _returnvalue_2 (`self.GetComponentByClass` _returnvalue "/Game/Blueprints/Puzzel/TemplePuzzel/BP_TempleSpawnManageComponent.BP_TempleSpawnManageComponent_C"))
          (`/Engine/EditorBlueprintResources/StandardMacros.IncrementInt` (`/Game/Blueprints/Puzzel/TemplePuzzel/BP_TempleSpawnManageComponent.ClearColorNum` _returnvalue_2)
            (:`  `
              (`/Engine/EditorBlueprintResources/StandardMacros.IsValid` (`self.Box`)
                (:`Is Valid`
                  (for _array_element (`PrimitiveComponent.GetOverlappingActors` (`self.Box`) "/Game/Blueprints/Puzzel/TemplePuzzel/BP_Puzzel_Temple_ChangingTile.BP_Puzzel_Temple_ChangingTile_C")
                    (`/Engine/EditorBlueprintResources/StandardMacros.IsValid` _array_element
                      (:`Is Valid`
                        (bind _asbp_puzzel_temple_changing_tile (cast `/Game/Blueprints/Puzzel/TemplePuzzel/BP_Puzzel_Temple_ChangingTile` _array_element))
                        (`/Game/Blueprints/Puzzel/TemplePuzzel/BP_Puzzel_Temple_ChangingTile.PlayerTriggerColor` _asbp_puzzel_temple_changing_tile)
                        (`GameplayStatics.PlaySound2D` "/Game/Audio/SFX/SFX_Itemheal.SFX_Itemheal" 1.0 1.0 0.0 null null)
                        (set `/Game/Blueprints/Puzzel/TemplePuzzel/BP_Puzzel_Temple_ChangingTile.bIsTileColorCompleted` true _asbp_puzzel_temple_changing_tile)
                        (`/Game/Blueprints/Puzzel/TemplePuzzel/BP_TempleSpawnManageComponent.GoNextLevel` _returnvalue_2)
                        ;[1 0.101 0.101] 다른 색 트리거에서 변수 변경 필수!
                        (bind _outactors (`GameplayStatics.GetAllActorsOfClassWithTag` "/Game/Blueprints/Puzzel/TemplePuzzel/BP_Puzzel_Temple_ChangingTile.BP_Puzzel_Temple_ChangingTile_C" "Yellow"))
                        (for _array_element_2 _outactors
                          (set `/Game/Blueprints/Puzzel/TemplePuzzel/BP_Puzzel_Temple_ChangingTile.bIsTileColorCompleted` true _array_element_2)))))))))
          (else
            (bind _returnvalue_3 (`GameplayStatics.GetActorOfClass` "/Game/Blueprints/Puzzel/TemplePuzzel/BP_TemplePuzzel.BP_TemplePuzzel_C" :!label _label))
            (`RXPuzzelSpawnManageComponent.ResetCurrentLevel` (`self.GetComponentByClass` _returnvalue_3 "/Game/Blueprints/Puzzel/TemplePuzzel/BP_TempleSpawnManageComponent.BP_TempleSpawnManageComponent_C"))
            (`GameplayStatics.PlaySound2D` "/Game/Audio/SFX/Puzzel/SFX_CannotIneract.SFX_CannotIneract" 1.0 1.0 0.0 null null)))
        (else
          (goto _label)))
      (else
        (`GameplayStatics.PlaySound2D` "/Game/Audio/SFX/SFX_Itemheal.SFX_Itemheal" 1.0 1.0 0.0 null null)
        ;[1 0.101 0.101 1 13] 다른 색 트리거에서 변수 변경 필수!
        (`self.PassTriggerYellowColor` "Yellow")
        (bind _returnvalue_4 (`GameplayStatics.GetActorOfClass` "/Game/Blueprints/Puzzel/TemplePuzzel/BP_TemplePuzzel.BP_TemplePuzzel_C"))
        (bind _returnvalue_5 (`self.GetComponentByClass` _returnvalue_4 "/Game/Blueprints/Puzzel/TemplePuzzel/BP_TempleSpawnManageComponent.BP_TempleSpawnManageComponent_C"))
        ;[1 1 1] 모든 다른 트리거에게 IsActive 변수를 true 만들어줌
        (`/Game/Blueprints/Puzzel/TemplePuzzel/BP_TempleSpawnManageComponent.SetActiveToAllTriggerActor` _returnvalue_5)
        (`/Game/Blueprints/Puzzel/TemplePuzzel/BP_TempleSpawnManageComponent.SetActiveToChangingTile` _returnvalue_5)
        (set `self.bIsTriggeredAgain` false)))))

(fn `IsSameColor`
  (returns (NewParam :type Boolean))
  (bind _returncolor (`self.ReturnTriggerColor`))
  (return (== _returncolor "Yellow")))

(fn `ReturnTriggerColor`
  (returns (ReturnColor :type Name))
  (bind _returnvalue (`GameplayStatics.GetActorOfClass` "/Game/Blueprints/Puzzel/TemplePuzzel/BP_TemplePuzzel.BP_TemplePuzzel_C"))
  (return (`/Game/Blueprints/Puzzel/TemplePuzzel/BP_TempleSpawnManageComponent.CurrentTriggerColor` (`self.GetComponentByClass` _returnvalue "/Game/Blueprints/Puzzel/TemplePuzzel/BP_TempleSpawnManageComponent.BP_TempleSpawnManageComponent_C"))))

(fn `UserConstructionScript`)
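; Component on BP_PatternPuzzel that runs a four-level puzzle of stepping on colored tiles in a repeating order.
; Each level's hint plays the color sequence on timed delays with player input disabled, then fades out.
; BeginPlay binds tile step events; CheckTileColor compares colors against the level's rule, resetting and replaying the hint on mistakes.
; GoNextLevel advances levels, finally ending puzzle mode and recording completion in RXGameInstance.
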(event `ShowLevel1_Hint`
  (`self.DisablePlayerInput`)
  (`|ExecutionSequence`
    (:`then_0`
      ;[1 1 1] Level 1 : Red->Yellow->Green (3색)
      (`/Game/Blueprints/Puzzel/PatternPuzzel/BP_PatternPuzzel.MakeHintTileColor` (`self.Pattern Puzzel`) "Red")
      (`KismetSystemLibrary.Delay` 3.0)
      (`/Game/Blueprints/Puzzel/PatternPuzzel/BP_PatternPuzzel.MakeHintTileColor` (`self.Pattern Puzzel`) "Yellow")
      (`KismetSystemLibrary.Delay` 2.0)
      (`/Game/Blueprints/Puzzel/PatternPuzzel/BP_PatternPuzzel.MakeHintTileColor` (`self.Pattern Puzzel`) "Green")
      (`KismetSystemLibrary.Delay` 2.0 :!label _label)
      (`self.FadeFunction`)
      (`/Game/Blueprints/Puzzel/PatternPuzzel/BP_PatternPuzzel.ResetHintTileColor` (`self.Pattern Puzzel`))
      (`self.OnVisibleColor`)
      (`self.EnablePlayerInput`))
    (:`then_1`
      (`KismetSystemLibrary.Delay` 1.5)
      (`self.DisablePlayerInput`))))

(event `ShowLevel2_Hint`
  (`self.DisablePlayerInput`)
  (`|ExecutionSequence`
    (:`then_0`
      ;[1 1 1] Level 2 : Red->Yellow->Green->Blue (4색)
      (`/Game/Blueprints/Puzzel/PatternPuzzel/BP_PatternPuzzel.MakeHintTileColor` (`self.Pattern Puzzel`) "Red")
      (`KismetSystemLibrary.Delay` 3.0)
      (`/Game/Blueprints/Puzzel/PatternPuzzel/BP_PatternPuzzel.MakeHintTileColor` (`self.Pattern Puzzel`) "Yellow")
      (`KismetSystemLibrary.Delay` 2.0)
      (`/Game/Blueprints/Puzzel/PatternPuzzel/BP_PatternPuzzel.MakeHintTileColor` (`self.Pattern Puzzel`) "Green")
      (`KismetSystemLibrary.Delay` 2.0)
      (`/Game/Blueprints/Puzzel/PatternPuzzel/BP_PatternPuzzel.MakeHintTileColor` (`self.Pattern Puzzel`) "Blue")
      (goto _label))
    (:`then_1`
      (`KismetSystemLibrary.Delay` 1.5)
      (`self.DisablePlayerInput`))))

(event `EnablePlayerInput`
  (`Actor.EnableInput` (`GameplayStatics.GetPlayerPawn` 0) (`GameplayStatics.GetPlayerController` 0)))

(event `ShowLevel3_Hint`
  (`self.DisablePlayerInput`)
  (`|ExecutionSequence`
    (:`then_0`
      ;[1 1 1] Level 3 : Red->Yellow->Green->Blue->Purple (5색)
      (`/Game/Blueprints/Puzzel/PatternPuzzel/BP_PatternPuzzel.MakeHintTileColor` (`self.Pattern Puzzel`) "Red")
      (`KismetSystemLibrary.Delay` 3.0)
      (`/Game/Blueprints/Puzzel/PatternPuzzel/BP_PatternPuzzel.MakeHintTileColor` (`self.Pattern Puzzel`) "Yellow")
      (`KismetSystemLibrary.Delay` 2.0)
      (`/Game/Blueprints/Puzzel/PatternPuzzel/BP_PatternPuzzel.MakeHintTileColor` (`self.Pattern Puzzel`) "Green")
      (`KismetSystemLibrary.Delay` 2.0)
      (`/Game/Blueprints/Puzzel/PatternPuzzel/BP_PatternPuzzel.MakeHintTileColor` (`self.Pattern Puzzel`) "Blue")
      (`KismetSystemLibrary.Delay` 2.0)
      (`/Game/Blueprints/Puzzel/PatternPuzzel/BP_PatternPuzzel.MakeHintTileColor` (`self.Pattern Puzzel`) "Purple")
      (goto _label))
    (:`then_1`
      (`KismetSystemLibrary.Delay` 1.5)
      (`self.DisablePlayerInput`))))

(event `DisablePlayerInput`
  (`Actor.DisableInput` (`GameplayStatics.GetPlayerPawn` 0) (`GameplayStatics.GetPlayerController` 0)))

(event `ShowLevel4_Hint`
  (`self.DisablePlayerInput`)
  (`|ExecutionSequence`
    (:`then_0`
      ;[1 1 1] Level 4 :  Red->Yellow->Green->Blue->Purple->Pink (6색)
      (`/Game/Blueprints/Puzzel/PatternPuzzel/BP_PatternPuzzel.MakeHintTileColor` (`self.Pattern Puzzel`) "Red")
      (`KismetSystemLibrary.Delay` 3.0)
      (`/Game/Blueprints/Puzzel/PatternPuzzel/BP_PatternPuzzel.MakeHintTileColor` (`self.Pattern Puzzel`) "Yellow")
      (`KismetSystemLibrary.Delay` 2.0)
      (`/Game/Blueprints/Puzzel/PatternPuzzel/BP_PatternPuzzel.MakeHintTileColor` (`self.Pattern Puzzel`) "Green")
      (`KismetSystemLibrary.Delay` 2.0)
      (`/Game/Blueprints/Puzzel/PatternPuzzel/BP_PatternPuzzel.MakeHintTileColor` (`self.Pattern Puzzel`) "Blue")
      (`KismetSystemLibrary.Delay` 2.0)
      (`/Game/Blueprints/Puzzel/PatternPuzzel/BP_PatternPuzzel.MakeHintTileColor` (`self.Pattern Puzzel`) "Purple")
      (`KismetSystemLibrary.Delay` 2.0)
      (`/Game/Blueprints/Puzzel/PatternPuzzel/BP_PatternPuzzel.MakeHintTileColor` (`self.Pattern Puzzel`) "Pink")
      (goto _label))
    (:`then_1`
      (`KismetSystemLibrary.Delay` 1.5)
      (`self.DisablePlayerInput`))))

(event `FadeFunction`
  (bind _fadewidget (`self.FadeWidget`))
  ;[1 1 1] 노드 단축 편의를 위해 만든 컴포넌트 내 페이드 함수
  (`UserWidget.AddToViewport` _fadewidget 0)
  (`/Game/UI/WBP_FadeAnimWidget.PlayFadeOut` _fadewidget))

(event `CheckTileColor`
  (params (TileColor :type String))
  ;[1 1 1] 레벨의 색 순서와 현재 밟은 타일 색을 체크하는 함수
  (switch `int` (`self.CurrentLevelID`)
    (:`1`
      (if (`KismetStringLibrary.EqualEqual_StrStr` TileColor (`|GetArrayItem` (`self.Level1ColorRule`) (`self.CurrentColorIdx`)))
        ;[1 1 1 1 15] 같으면 인덱스 1증가
        (bind _result (`/Engine/EditorBlueprintResources/StandardMacros.IncrementInt` (`self.CurrentColorIdx`))
          (:`  `
            ;[1 1 1] 인덱스와 배열길이 같으면 인덱스를 0으로 Set해서 다시 돌 수 있도록 함
            (if (== (`KismetArrayLibrary.Array_Length` (`self.Level1ColorRule`)) _result)
              (set `self.CurrentColorIdx` 0))))
        (else
          (`self.ResetCurrentLevel` :!label _label_2)
          (`GameplayStatics.PlaySound2D` "/Game/Audio/SFX/Puzzel/SFX_CannotIneract.SFX_CannotIneract" 1.0 1.0 0.0 null null))))
    (:`2`
      (if (`KismetStringLibrary.EqualEqual_StrStr` TileColor (`|GetArrayItem` (`self.Level2ColorRule`) (`self.CurrentColorIdx`)))
        (bind _result_2 (`/Engine/EditorBlueprintResources/StandardMacros.IncrementInt` (`self.CurrentColorIdx`))
          (:`  `
            (if (== (`KismetArrayLibrary.Array_Length` (`self.Level2ColorRule`)) _result_2)
              (set `self.CurrentColorIdx` 0))))
        (else
          (goto _label_2))))
    (:`3`
      (if (`KismetStringLibrary.EqualEqual_StrStr` TileColor (`|GetArrayItem` (`self.Level3ColorRule`) (`self.CurrentColorIdx`)))
        (bind _result_3 (`/Engine/EditorBlueprintResources/StandardMacros.IncrementInt` (`self.CurrentColorIdx`))
          (:`  `
            (if (== (`KismetArrayLibrary.Array_Length` (`self.Level3ColorRule`)) _result_3)
              (set `self.CurrentColorIdx` 0))))
        (else
          (goto _label_2))))
    (:`4`
      (if (`KismetStringLibrary.EqualEqual_StrStr` TileColor (`|GetArrayItem` (`self.Level4ColorRule`) (`self.CurrentColorIdx`)))
        (bind _result_4 (`/Engine/EditorBlueprintResources/StandardMacros.IncrementInt` (`self.CurrentColorIdx`))
          (:`  `
            (if (== (`KismetArrayLibrary.Array_Length` (`self.Level4ColorRule`)) _result_4)
              (set `self.CurrentColorIdx` 0))))
        (else
          (goto _label_2))))))

(event `GoNextLevel`
  (bind _result (`/Engine/EditorBlueprintResources/StandardMacros.IncrementInt` (`self.CurrentLevelID`))
    (:`  `
      (if (== _result 5)
        ;[1 1 1] 레벨이 5라면 퍼즐이벤트종료
        (`RXPuzzelEventManageComponent.EndPuzzelMode` (`Actor.GetComponentByClass` (`self.GetOwner`) "/Game/Blueprints/Puzzel/BP_PuzzelEventManageComponent.BP_PuzzelEventManageComponent_C"))
        ;[1 1 1] 게임 인스턴스에 클리어 조건 상태 전달
        (bind _asrxgame_instance (cast `RXGameInstance` (`GameplayStatics.GetGameInstance`)))
        (`RXGameInstance.SetPuzzelStatusAcquired` _asrxgame_instance "PatternPuzzel")
        (else
          ;[1 1 1] 레벨이 1~3이면 다음레벨로 활성화함
          (`self.ActivateLevel` _result)
          (`self.ResetCurrentLevel`)
          (`GameplayStatics.PlaySound2D` "/Game/Audio/SFX/Boss/SFX_StoneTrigger.SFX_StoneTrigger" 1.0 1.0 0.0 null null))))))

(event `self.ReceiveBeginPlay`
  (`parent.ReceiveBeginPlay`)
  (bind _asbp_pattern_puzzel (cast `/Game/Blueprints/Puzzel/PatternPuzzel/BP_PatternPuzzel` (`self.GetOwner`)))
  (set `self.Pattern Puzzel` _asbp_pattern_puzzel)
  (`|ExecutionSequence`
    (:`then_0`
      ;[1 1 1] Blue Tile Event Dispatcher Binding
      (bind _outactors (`GameplayStatics.GetAllActorsOfClass` "/Game/Blueprints/Puzzel/PatternPuzzel/BP_Puzzel_PatternPurpleTile.BP_Puzzel_PatternPurpleTile_C"))
      (add `/Game/Blueprints/Puzzel/PatternPuzzel/BP_Puzzel_PatternPurpleTile.OnTileStepped` _outactors (`|CreateDelegate` :!event `CheckTileColor`)))
    (:`then_1`
      ;[1 1 1] Gray Tile Event Dispatcher Binding
      (bind _outactors_2 (`GameplayStatics.GetAllActorsOfClass` "/Game/Blueprints/Puzzel/PatternPuzzel/BP_Puzzel_PatternGrayTile.BP_Puzzel_PatternGrayTile_C"))
      (add `/Game/Blueprints/Puzzel/PatternPuzzel/BP_Puzzel_PatternGrayTile.OnTileStepped` _outactors_2 (`|CreateDelegate` :!event `CheckTileColor`)))
    (:`then_2`
      ;[1 1 1] Orange Tile Event Dispatcher Binding
      (bind _outactors_3 (`GameplayStatics.GetAllActorsOfClass` "/Game/Blueprints/Puzzel/PatternPuzzel/BP_Puzzel_PatternYellowTile.BP_Puzzel_PatternYellowTile_C"))
      (add `/Game/Blueprints/Puzzel/PatternPuzzel/BP_Puzzel_PatternYellowTile.OnTileStepped` _outactors_3 (`|CreateDelegate` :!event `CheckTileColor`)))
    (:`then_3`
      ;[1 1 1] Pink Tile Event Dispatcher Binding
      (bind _outactors_4 (`GameplayStatics.GetAllActorsOfClass` "/Game/Blueprints/Puzzel/PatternPuzzel/BP_Puzzel_PatternPinkTile.BP_Puzzel_PatternPinkTile_C"))
      (add `/Game/Blueprints/Puzzel/PatternPuzzel/BP_Puzzel_PatternPinkTile.OnTileStepped` _outactors_4 (`|CreateDelegate` :!event `CheckTileColor`)))
    (:`then_4`
      ;[1 1 1] Red Tile Event Dispatcher Binding
      (bind _outactors_5 (`GameplayStatics.GetAllActorsOfClass` "/Game/Blueprints/Puzzel/PatternPuzzel/BP_Puzzel_PatternRedTile.BP_Puzzel_PatternRedTile_C"))
      (add `/Game/Blueprints/Puzzel/PatternPuzzel/BP_Puzzel_PatternRedTile.OnTileStepped` _outactors_5 (`|CreateDelegate` :!event `CheckTileColor`)))
    (:`then_5`
      ;[1 1 1] Sky Tile Event Dispatcher Binding
      (bind _outactors_6 (`GameplayStatics.GetAllActorsOfClass` "/Game/Blueprints/Puzzel/PatternPuzzel/BP_Puzzel_PatternBlueTile.BP_Puzzel_PatternBlueTile_C"))
      (add `/Game/Blueprints/Puzzel/PatternPuzzel/BP_Puzzel_PatternBlueTile.OnTileStepped` _outactors_6 (`|CreateDelegate` :!event `CheckTileColor`)))
    (:`then_6`
      ;[1 1 1] Green Tile Event Dispatcher Binding
      (bind _outactors_7 (`GameplayStatics.GetAllActorsOfClass` "/Game/Blueprints/Puzzel/PatternPuzzel/BP_Puzzel_PatternGreenTile.BP_Puzzel_PatternGreenTile_C"))
      (add `/Game/Blueprints/Puzzel/PatternPuzzel/BP_Puzzel_PatternGreenTile.OnTileStepped` _outactors_7 (`|CreateDelegate` :!event `CheckTileColor`)))))

(event `self.ResetCurrentLevel`
  ;[1 1 1] CPP : 각각 모든 PuzzelObject에게 Resetobjectstate 를 호출함. / Deactive Color Function In Each Tile BP
  (`parent.ResetCurrentLevel`)
  (switch `int` (`self.CurrentLevelID`)
    (:`1`
      (`self.ShowLevel1_Hint`))
    (:`2`
      (`self.ShowLevel2_Hint`))
    (:`3`
      (`self.ShowLevel3_Hint`))
    (:`4`
      (`self.ShowLevel4_Hint`)))
  (set `self.CurrentColorIdx` 0))
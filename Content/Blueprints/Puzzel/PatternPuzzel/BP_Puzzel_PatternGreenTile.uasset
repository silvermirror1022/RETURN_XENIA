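; Green tile of the pattern puzzle, which shows or hides its colour mesh and reports when the player steps on it.
; On BeginPlay it finds BP_PatternPuzzel and binds to its spawn-manage component's OnVisibleColor dispatcher.
; An RXPlayer overlapping the box fires OnTileStepped with "Green" for bound listeners, noted as the spawn manager component.
; Resetting the object state hides the colour mesh.
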(event `ActiveColor`
  ;[1 1 1] 색 활성화/비활성화 함수
  (`SceneComponent.SetVisibility` (`self.SM_This`) true false))

(event `DeActiveColor`
  ;[1 1 1] 색 활성화/비활성화 함수
  (`SceneComponent.SetVisibility` (`self.SM_This`) false false))

(event `self.ResetObjectState`
  (`self.DeActiveColor`))

(event `self.ReceiveBeginPlay`
  ;[1 1 1] 스폰컴포넌트의 함수 구독
  (bind _returnvalue (`GameplayStatics.GetActorOfClass` "/Game/Blueprints/Puzzel/PatternPuzzel/BP_PatternPuzzel.BP_PatternPuzzel_C"))
  (add `/Game/Blueprints/Puzzel/PatternPuzzel/BP_PatternPuzzelSpawnManageComponent.OnVisibleColor` (`self.GetComponentByClass` _returnvalue "/Game/Blueprints/Puzzel/PatternPuzzel/BP_PatternPuzzelSpawnManageComponent.BP_PatternPuzzelSpawnManageComponent_C") (`|CreateDelegate` :!event `ActiveColor`)))

(event `self.Box.OnComponentBeginOverlap`
  (params (OverlappedComponent :type "PrimitiveComponent Object Reference") (OtherActor :type "Actor Object Reference") (OtherComp :type "PrimitiveComponent Object Reference") (OtherBodyIndex :type Integer) (bFromSweep :type Boolean) (SweepResult :type "HitResult Structure (by ref)"))
  ;[1 1 1] 플레이어가 Tile을 오버랩 하는 경우, 스폰매니저컴포넌트에게 해당 색을 파라미터로 바인딩된 함수 호출
  (cast `RXPlayer` OtherActor)
  (`self.OnTileStepped` "Green"))

(fn `UserConstructionScript`)
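; Pattern puzzle actor that shows color hints on a flat tile mesh as part of a leveled temple puzzle.
; Hint events swap the tile's material to one of seven colors or restore the default.
; On start it calls the parent event, then has the spawn manager component activate and reset the first level.
; On finish it destroys its invisible walls, event manager, interaction visibility component and hint tile.
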(event `MakeHintTileColor`
  (params (Color :type Name))
  ;[1 1 1] 색은 총 레벨1부터 4까지 : 총 7 색
  (switch `name` Color
    (:`Red`
      (`PrimitiveComponent.SetMaterial` (`self.SM_PatternFlat`) 0 "/Game/Designer/Materials/MI_TemplePuzzel_A04.MI_TemplePuzzel_A04"))
    (:`Orange`
      (`PrimitiveComponent.SetMaterial` (`self.SM_PatternFlat`) 0 "/Game/Designer/Materials/puzzel/MI_TemplePuzzel_A08.MI_TemplePuzzel_A08"))
    (:`Blue`
      (`PrimitiveComponent.SetMaterial` (`self.SM_PatternFlat`) 0 "/Game/Designer/Materials/MI_TemplePuzzel_A06.MI_TemplePuzzel_A06"))
    (:`Sky`
      (`PrimitiveComponent.SetMaterial` (`self.SM_PatternFlat`) 0 "/Game/Designer/Materials/MI_TemplePuzzel_A02.MI_TemplePuzzel_A02"))
    (:`Gray`
      (`PrimitiveComponent.SetMaterial` (`self.SM_PatternFlat`) 0 "/Game/Designer/Materials/MI_TemplePuzzel_A07.MI_TemplePuzzel_A07"))
    (:`Pink`
      (`PrimitiveComponent.SetMaterial` (`self.SM_PatternFlat`) 0 "/Game/Designer/Materials/MI_TemplePuzzel_A03.MI_TemplePuzzel_A03"))
    (:`Green`
      (`PrimitiveComponent.SetMaterial` (`self.SM_PatternFlat`) 0 "/Game/Designer/Materials/MI_TemplePuzzel_A01.MI_TemplePuzzel_A01"))))

(event `ResetHintTileColor`
  (`PrimitiveComponent.SetMaterial` (`self.SM_PatternFlat`) 0 "/Game/Designer/Materials/puzzel/MI_PuzzelSet_A02.MI_PuzzelSet_A02"))

(event `self.PuzzelEventStart`
  (bind _bp_patternpuzzelspawnmanagecomponent (`self.BP_PatternPuzzelSpawnManageComponent`))
  ;[1 1 1] 패턴퍼즐 이벤트 시작
  (`parent.PuzzelEventStart`)
  (`RXPuzzelSpawnManageComponent.ActivateLevel` _bp_patternpuzzelspawnmanagecomponent 1)
  (`RXPuzzelSpawnManageComponent.ResetCurrentLevel` _bp_patternpuzzelspawnmanagecomponent))

(event `self.PuzzelEventFinish`
  ;[1 1 1] 퍼즐클리어시 관련 기능 컴포넌트 모두 삭제
  (`ActorComponent.K2_DestroyComponent` (`self.SM_puzzel_InvisibleEdgeWall`))
  (`ActorComponent.K2_DestroyComponent` (`self.SM_puzzel_InvisibleWall`))
  (`ActorComponent.K2_DestroyComponent` (`self.BP_PuzzelEventManageComponent`))
  (`ActorComponent.K2_DestroyComponent` (`self.RXInteractionVisibility`))
  (`ActorComponent.K2_DestroyComponent` (`self.SM_PatternFlat`)))

(fn `UserConstructionScript`
  (`parent.UserConstructionScript`))
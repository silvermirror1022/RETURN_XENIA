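; End tile of the blind puzzle that sends the puzzle to its next level when the player reaches it.
; It starts with a translucent inactive material, and its SetActiveColor and SetDeActiveColor events swap between that and the highlighted end-tile material.
; When RXPlayer overlaps its box, it finds BP_BlindPuzzel and calls GoNextLevel on that actor's spawn-manage component.
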(event `self.ReceiveBeginPlay`
  ;[1 1 1] DeActive->배경타일(보라색), Active->노란색
  (`self.SetDeActiveColor`))

(event `SetActiveColor`
  ;[1 1 1] DeActive->배경타일(보라색), Active->노란색
  (`PrimitiveComponent.SetMaterial` (`self.SM_This`) 0 "/Game/Designer/Materials/puzzel/MI_EndTile_A01.MI_EndTile_A01"))

(event `SetDeActiveColor`
  ;[1 1 1] DeActive->배경타일(보라색), Active->노란색
  (`PrimitiveComponent.SetMaterial` (`self.SM_This`) 0 "/Game/Designer/Materials/MI_PuzzelTranslucent.MI_PuzzelTranslucent"))

(event `self.Box.OnComponentBeginOverlap`
  (params (OverlappedComponent :type "PrimitiveComponent Object Reference") (OtherActor :type "Actor Object Reference") (OtherComp :type "PrimitiveComponent Object Reference") (OtherBodyIndex :type Integer) (bFromSweep :type Boolean) (SweepResult :type "HitResult Structure (by ref)"))
  ;[1 1 1] 플레이어가 EndTile을 오버랩 하는 경우, 해당 레벨에서 컴포넌트를 통해서 함수 호출해줌
  (cast `RXPlayer` OtherActor)
  (bind _returnvalue (`GameplayStatics.GetActorOfClass` "/Game/Blueprints/Puzzel/BlindPuzzel/BP_BlindPuzzel.BP_BlindPuzzel_C"))
  (bind _returnvalue_2 (`self.GetComponentByClass` _returnvalue "/Game/Blueprints/Puzzel/BlindPuzzel/BP_BlindPuzzelSpawnManageComponent.BP_BlindPuzzelSpawnManageComponent_C"))
  (`/Engine/EditorBlueprintResources/StandardMacros.IsValid` _returnvalue_2
    (:`Is Valid`
      (`/Game/Blueprints/Puzzel/BlindPuzzel/BP_BlindPuzzelSpawnManageComponent.GoNextLevel` _returnvalue_2))))

(fn `UserConstructionScript`)
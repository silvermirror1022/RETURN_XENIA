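; BP_BlindPuzzel is the blind puzzle actor, a child of a puzzle parent that supplies the start event.
; On start it calls the parent, then has its spawn manage component activate and reset the first level.
; Separate events hide or show its plane mesh.
; On finish it destroys its puzzle components, including the invisible walls, plane, spawn and event managers, and interaction visibility.
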(event `self.PuzzelEventStart`
  (bind _bp_blindpuzzelspawnmanagecomponent (`self.BP_BlindPuzzelSpawnManageComponent`))
  ;[1 1 1] 블라인드퍼즐 이벤트 시작
  (`parent.PuzzelEventStart`)
  (`RXPuzzelSpawnManageComponent.ActivateLevel` _bp_blindpuzzelspawnmanagecomponent 1)
  (`RXPuzzelSpawnManageComponent.ResetCurrentLevel` _bp_blindpuzzelspawnmanagecomponent))

(event `SetPlaneHidden`
  ;[1 1 1] Plane Component 활성화/비활성화 함수
  (`SceneComponent.SetHiddenInGame` (`self.SM_Plane`) true false))

(event `self.PuzzelEventFinish`
  ;[1 1 1] 퍼즐클리어시 관련 기능 컴포넌트 모두 삭제
  (`ActorComponent.K2_DestroyComponent` (`self.SM_puzzel_InvisibleEdgeWall`))
  (`ActorComponent.K2_DestroyComponent` (`self.SM_puzzel_InvisibleWall`))
  (`ActorComponent.K2_DestroyComponent` (`self.SM_Plane`))
  (`ActorComponent.K2_DestroyComponent` (`self.BP_BlindPuzzelSpawnManageComponent`))
  (`ActorComponent.K2_DestroyComponent` (`self.BP_PuzzelEventManageComponent`))
  (`ActorComponent.K2_DestroyComponent` (`self.RXInteractionVisibility`)))

(event `SetPlaneVisible`
  ;[1 1 1] Plane Component 활성화/비활성화 함수
  (`SceneComponent.SetHiddenInGame` (`self.SM_Plane`) false false))

(fn `UserConstructionScript`
  (`parent.UserConstructionScript`))
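; Level manager component for BP_BlindPuzzel, driving a memory-style puzzle where hint tiles show briefly before play.
; GoNextLevel activates and resets each next level, or at level five ends puzzle mode and records the clear in RXGameInstance.
; ResetCurrentLevel extends its C++ parent, fading, disabling input, hiding the plane and playing the hint Level Sequence.
; After a five-second delay it fades again, restoring input and the plane.
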(event `ShowHintTile`
  ;[1 1 1] Hint Tile 보여주기 함수 :  레벨 시퀀스를 통해서 활용
  (bind _outactor (`LevelSequencePlayer.CreateLevelSequencePlayer` "/Game/Cinematics/LS_BlindPuzzelHint.LS_BlindPuzzelHint"))
  (`MovieSceneSequencePlayer.Play` (`LevelSequenceActor.SequencePlayer` _outactor)))

(event `GoNextLevel`
  (bind _result (`/Engine/EditorBlueprintResources/StandardMacros.IncrementInt` (`self.CurrentLevelID`))
    (:`  `
      (if (== _result 5)
        ;[1 1 1] 레벨이 5라면 퍼즐이벤트종료
        (`RXPuzzelEventManageComponent.EndPuzzelMode` (`Actor.GetComponentByClass` (`self.GetOwner`) "/Game/Blueprints/Puzzel/BP_PuzzelEventManageComponent.BP_PuzzelEventManageComponent_C"))
        ;[1 1 1] 게임 인스턴스에 클리어 조건 상태 전달
        (bind _asrxgame_instance (cast `RXGameInstance` (`GameplayStatics.GetGameInstance`)))
        (`RXGameInstance.SetPuzzelStatusAcquired` _asrxgame_instance "BlindPuzzel")
        (else
          ;[1 1 1] 레벨이 1~3이면 다음레벨로 활성화함
          (`self.ActivateLevel` _result)
          (`self.ResetCurrentLevel`))))))

(event `self.ResetCurrentLevel`
  (bind _fadewidget (`self.FadeWidget`))
  (bind _fadewidget_2 (`self.FadeWidget`))
  ;[1 1 1] CPP : BlindHintTile을 잠시게 보이게하는 로직 -> 각각 모든 엑터들에게 resetobjectstate 를 호출함.
  (`parent.ResetCurrentLevel`)
  (`UserWidget.AddToViewport` _fadewidget 0)
  (`/Game/UI/WBP_FadeAnimWidget.PlayFadeOut` _fadewidget)
  ;[1 1 1] 플레이어 인풋 비활성화, Plane 안보이게 지정
  (`Actor.DisableInput` (`self.GamePlayer`) (`self.PlayerController`))
  (`/Game/Blueprints/Puzzel/BlindPuzzel/BP_BlindPuzzel.SetPlaneHidden` (`self.BlindPuzzel`))
  (`self.ShowHintTile`)
  ;[1 1 1] 5초 뒤 Fade Event 후, 플레이어 인풋 활성화, 다시 플레인을 보이게 지정
  (`KismetSystemLibrary.Delay` 5.0)
  (`UserWidget.AddToViewport` _fadewidget_2 0)
  (`/Game/UI/WBP_FadeAnimWidget.PlayFadeOut` _fadewidget_2)
  (`Actor.EnableInput` (`self.GamePlayer`) (`self.PlayerController`))
  (`/Game/Blueprints/Puzzel/BlindPuzzel/BP_BlindPuzzel.SetPlaneVisible` (`self.BlindPuzzel`)))

(event `self.ReceiveBeginPlay`
  (`parent.ReceiveBeginPlay`)
  (set `self.PlayerController` (`GameplayStatics.GetPlayerController` 0))
  (set `self.GamePlayer` (`GameplayStatics.GetPlayerCharacter` 0))
  (bind _asbp_blind_puzzel (cast `/Game/Blueprints/Puzzel/BlindPuzzel/BP_BlindPuzzel` (`self.GetOwner`)))
  (bind _output_get (set `self.BlindPuzzel` _asbp_blind_puzzel))
  (`/Game/Blueprints/Puzzel/BlindPuzzel/BP_BlindPuzzel.SetPlaneHidden` _output_get))
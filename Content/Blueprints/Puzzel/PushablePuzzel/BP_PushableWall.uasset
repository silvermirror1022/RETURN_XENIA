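; BP_PushableWall is a puzzle wall the player pushes along the X or Y axis, with a reset to its starting location.
; Box overlap toggles the player AnimBP's pushing flag and snaps the player's forward vector to its dominant axis.
; If an angle check rejects sideways pushes and a sphere trace finds that direction clear, a Timeline slides the wall incrementally with sound.
; An IsMoving flag blocks new pushes mid-move.
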(event `self.ReceiveBeginPlay`
  (set `self.IsMoving` false)
  (set `self.FirstTransform` (`self.K2_GetActorLocation`)))

(event `self.ResetObjectState`
  (`self.K2_SetActorLocation` (`self.FirstTransform`)))

(event `self.Box.OnComponentBeginOverlap`
  (params (OverlappedComponent :type "PrimitiveComponent Object Reference") (OtherActor :type "Actor Object Reference") (OtherComp :type "PrimitiveComponent Object Reference") (OtherBodyIndex :type Integer) (bFromSweep :type Boolean) (SweepResult :type "HitResult Structure (by ref)"))
  (bind _returnvalue (`SceneComponent.K2_GetComponentLocation` (`self.Box`)))
  (bind _asrxplayer (cast `RXPlayer` OtherActor))
  (bind _asabp_player (cast `/Game/Animation/Player/ABP_Player` (`SkeletalMeshComponent.GetAnimInstance` (`Character.Mesh` _asrxplayer))))
  (set `/Game/Animation/Player/ABP_Player.IsPushing` true _asabp_player)
  ;[1 1 1] Abs로 두 벡터 중 더 큰수를 비교, Sign을 통해 부호를 기억해서 가져옴 => MoveDirection Set
  (if (not (`self.IsMoving`))
    (bind (_returnvalue_x _returnvalue_y) (`KismetMathLibrary.BreakVector` (`SceneComponent.GetForwardVector` (`Actor.RootComponent` _asrxplayer))))
    (if (> (`KismetMathLibrary.Abs` _returnvalue_x) (`KismetMathLibrary.Abs` _returnvalue_y))
      (set `self.MoveDirection` (`KismetMathLibrary.MakeVector2D` (`KismetMathLibrary.SignOfFloat` _returnvalue_x)))
      (else
        (set `self.MoveDirection` (`KismetMathLibrary.MakeVector2D` 0.0 (`KismetMathLibrary.SignOfFloat` _returnvalue_y)))))
    (bind (_outhit _returnvalue_2) (`KismetSystemLibrary.SphereTraceSingleForObjects` :`Start` _returnvalue :`End` (+ _returnvalue (* (`self.MoveDirection`) (100.0 100.0))) :`Radius` 30.0 :`ObjectTypes` (`|MakeArray` "ObjectTypeQuery2" :!type "EObjectTypeQuery Enum") :`DrawDebugType` "ForDuration"))
    (bind _output_get (set `self.NotMovePos` (>= (`KismetMathLibrary.Acos` (`KismetMathLibrary.DotProduct2D` (`self.MoveDirection`) (`KismetMathLibrary.Conv_VectorToVector2D` (`KismetMathLibrary.GetDirectionUnitVector` (`self.K2_GetActorLocation` (`GameplayStatics.GetPlayerPawn` 0)) (`self.K2_GetActorLocation`))))) 0.707)))
    ;[1 1 1] NotMovePos(45도차이가나는지)->(false)  Hit(되었는지 false여야 이동 가능) ->false  NOR => true, true
    (if (`KismetMathLibrary.BooleanNOR` _output_get _returnvalue_2)
      (if (not (`self.IsMoving`))
        ;[1 1 1] Timeline을 통해서 벽을 2.5초에 걸쳐서 자연스럽게 이동시킴
        (bind (_direction _vectortrack) (`Timeline|Timeline` :!via `PlayFromStart`)
          (:`Update`
            (`self.K2_SetActorLocation` (`KismetMathLibrary.VLerp` (`self.K2_GetActorLocation`) (+ (`self.K2_GetActorLocation`) (* (`self.MoveDirection`) (3.3 3.3))) _vectortrack)))
          (:`Finished`
            (set `self.IsMoving` false))
          (:`EventTrack`
            (set `self.IsMoving` true)
            (`GameplayStatics.PlaySound2D` "/Game/Audio/SFX/Puzzel/SFX_PuzzleBoxMove.SFX_PuzzleBoxMove" 1.0 1.0 0.0 null null)))))))

(event `self.Box.OnComponentEndOverlap`
  (params (OverlappedComponent :type "PrimitiveComponent Object Reference") (OtherActor :type "Actor Object Reference") (OtherComp :type "PrimitiveComponent Object Reference") (OtherBodyIndex :type Integer))
  (bind _asrxplayer (cast `RXPlayer` OtherActor))
  (bind _asabp_player (cast `/Game/Animation/Player/ABP_Player` (`SkeletalMeshComponent.GetAnimInstance` (`Character.Mesh` _asrxplayer))))
  (set `/Game/Animation/Player/ABP_Player.IsPushing` false _asabp_player))

(fn `UserConstructionScript`)
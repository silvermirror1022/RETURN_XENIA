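; Spawn-manager component for the pushable puzzle that handles advancing through and resetting its levels.
; GoNextLevel plays a fade widget, increments the level ID, then activates that level with a trigger sound through logic not defined here.
; After the final level it ends puzzle mode via the owner's BP_PuzzelEventManageComponent and records completion in RXGameInstance.
; Level changes and resets, which extend the parent's, briefly disable player input.
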(event `DisablePlayerInput`
  (bind _returnvalue (`GameplayStatics.GetPlayerPawn` 0))
  (bind _returnvalue_2 (`GameplayStatics.GetPlayerController` 0))
  (`Actor.DisableInput` _returnvalue _returnvalue_2)
  (`KismetSystemLibrary.Delay` 1.5)
  (`Actor.EnableInput` _returnvalue _returnvalue_2))

(event `self.ReceiveBeginPlay`
  (`parent.ReceiveBeginPlay`))

(event `GoNextLevel`
  (bind _fadewidget (`self.FadeWidget`))
  (`UserWidget.AddToViewport` _fadewidget 0)
  (`/Game/UI/WBP_FadeAnimWidget.PlayFadeOut` _fadewidget)
  (bind _result (`/Engine/EditorBlueprintResources/StandardMacros.IncrementInt` (`self.CurrentLevelID`))
    (:`  `
      (if (== _result 5)
        ;[1 1 1] 레벨이 5라면 퍼즐이벤트종료
        (`RXPuzzelEventManageComponent.EndPuzzelMode` (`Actor.GetComponentByClass` (`self.GetOwner`) "/Game/Blueprints/Puzzel/BP_PuzzelEventManageComponent.BP_PuzzelEventManageComponent_C"))
        ;[1 1 1] 게임 인스턴스에 클리어 조건 상태 전달
        (bind _asrxgame_instance (cast `RXGameInstance` (`GameplayStatics.GetGameInstance`)))
        (`RXGameInstance.SetPuzzelStatusAcquired` _asrxgame_instance "PushablePuzzel")
        (else
          ;[1 1 1] 레벨이 1~3이면 다음레벨로 활성화함
          (`self.ActivateLevel` _result)
          (`self.DisablePlayerInput`)
          (`GameplayStatics.PlaySound2D` "/Game/Audio/SFX/Boss/SFX_StoneTrigger.SFX_StoneTrigger" 1.0 1.0 0.0 null null))))))

(event `self.ResetCurrentLevel`
  (`parent.ResetCurrentLevel`)
  (`self.DisablePlayerInput`))
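; BP_PushablePuzzel is the actor that runs the push-block puzzle's lifecycle on top of its parent puzzle events.
; On start it activates level 1 through the spawn-manage component and hides the ceiling ice and ice wall so they don't block the camera.
; On finish it destroys the invisible walls and puzzle components and unhides the ice.
; BeginPlay strips the same components when the game instance reports the puzzle already acquired.
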(event `self.ReceiveBeginPlay`
  (`parent.ReceiveBeginPlay`)
  (bind _asrxgame_instance (cast `RXGameInstance` (`GameplayStatics.GetGameInstance`)))
  (if (`RXGameInstance.IsPuzzelStatusAcquired` _asrxgame_instance "PushablePuzzel")
    (`ActorComponent.K2_DestroyComponent` (`self.SM_puzzel_InvisibleEdgeWall`))
    (`ActorComponent.K2_DestroyComponent` (`self.SM_puzzel_InvisibleWall`))
    (`ActorComponent.K2_DestroyComponent` (`self.BP_PuzzelEventManageComponent`))
    (`ActorComponent.K2_DestroyComponent` (`self.RXInteractionVisibility`))
    (`ActorComponent.K2_DestroyComponent` (`self.BP_PushablePuzzelSpawnManageComponent`))))

(event `self.PuzzelEventStart`
  ;[1 1 1] 블라인드퍼즐 이벤트 시작
  (`parent.PuzzelEventStart`)
  (`RXPuzzelSpawnManageComponent.ActivateLevel` (`self.BP_PushablePuzzelSpawnManageComponent`) 1)
  ;[1 1 1] 천장 ICE 안보이게 처리 -> 카메라 뷰 안겹치게(Only 밀기퍼즐)
  (bind _returnvalue (`GameplayStatics.GetActorOfClass` "/Game/Blueprints/Puzzel/PushablePuzzel/BP_CelingIce.BP_CelingIce_C"))
  (`/Engine/EditorBlueprintResources/StandardMacros.IsValid` _returnvalue
    (:`Is Valid`
      (`SceneComponent.SetHiddenInGame` (`/Game/Blueprints/Puzzel/PushablePuzzel/BP_CelingIce.StaticMesh` _returnvalue) true false)
      (bind _returnvalue_2 (`GameplayStatics.GetActorOfClass` "/Game/Blueprints/Puzzel/PushablePuzzel/BP_IceWall.BP_IceWall_C"))
      (`/Engine/EditorBlueprintResources/StandardMacros.IsValid` _returnvalue_2
        (:`Is Valid`
          (`SceneComponent.SetHiddenInGame` (`/Game/Blueprints/Puzzel/PushablePuzzel/BP_IceWall.StaticMesh` _returnvalue_2) true false))))))

(event `self.PuzzelEventFinish`
  ;[1 1 1] 퍼즐클리어시 관련 기능 컴포넌트 모두 삭제
  (`ActorComponent.K2_DestroyComponent` (`self.SM_puzzel_InvisibleEdgeWall`))
  (`ActorComponent.K2_DestroyComponent` (`self.SM_puzzel_InvisibleWall`))
  (`ActorComponent.K2_DestroyComponent` (`self.BP_PuzzelEventManageComponent`))
  (`ActorComponent.K2_DestroyComponent` (`self.RXInteractionVisibility`))
  (`ActorComponent.K2_DestroyComponent` (`self.BP_PushablePuzzelSpawnManageComponent`))
  ;[1 1 1] 천장 ICE 보이게 처리 -> (Only 밀기퍼즐)
  (`|ExecutionSequence`
    (:`then_0`
      (bind _returnvalue (`GameplayStatics.GetActorOfClass` "/Game/Blueprints/Puzzel/PushablePuzzel/BP_IceWall.BP_IceWall_C")))
    (:`then_1`
      (bind _returnvalue_2 (`GameplayStatics.GetActorOfClass` "/Game/Blueprints/Puzzel/PushablePuzzel/BP_CelingIce.BP_CelingIce_C"))))
  (`SceneComponent.SetHiddenInGame` (`/Game/Blueprints/Puzzel/PushablePuzzel/BP_CelingIce.StaticMesh` _returnvalue_2) false false)
  (`SceneComponent.SetHiddenInGame` (`/Game/Blueprints/Puzzel/PushablePuzzel/BP_IceWall.StaticMesh` _returnvalue) false false))

(fn `UserConstructionScript`
  (`parent.UserConstructionScript`))
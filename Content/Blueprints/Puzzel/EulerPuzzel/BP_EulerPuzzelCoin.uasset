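; A collectible coin for the Euler puzzle that the player picks up by running into its mesh.
; On a player hit it increments the coin count on the puzzle actor's spawn-manager component, found through an actor-class lookup.
; It then disables collision, hides itself and plays a pickup sound instead of being destroyed.
; A reset event restores visibility and collision so the coin can be collected again.
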(event `self.ResetObjectState`
  (`self.SetActorEnableCollision` true)
  (`self.SetActorHiddenInGame` false))

(event `self.StaticMesh.OnComponentHit`
  (params (HitComponent :type "PrimitiveComponent Object Reference") (OtherActor :type "Actor Object Reference") (OtherComp :type "PrimitiveComponent Object Reference") (NormalImpulse :type "Vector Structure") (Hit :type "HitResult Structure (by ref)"))
  (cast `RXPlayer` OtherActor)
  (bind _returnvalue (`GameplayStatics.GetActorOfClass` "/Game/Blueprints/Puzzel/EulerPuzzel/BP_EulerPuzzel.BP_EulerPuzzel_C"))
  (`/Engine/EditorBlueprintResources/StandardMacros.IncrementInt` (`/Game/Blueprints/Puzzel/EulerPuzzel/BP_EulerPuzzelSpawnManageComponent.CurrentCoinNum` (`self.GetComponentByClass` _returnvalue "/Game/Blueprints/Puzzel/EulerPuzzel/BP_EulerPuzzelSpawnManageComponent.BP_EulerPuzzelSpawnManageComponent_C"))
    (:`  `
      (`self.SetActorEnableCollision` false)
      (`self.SetActorHiddenInGame` true)
      (`GameplayStatics.PlaySound2D` "/Game/Audio/SFX/SFX_GetCoin.SFX_GetCoin" 1.0 1.0 0.0 null null))))

(fn `UserConstructionScript`)
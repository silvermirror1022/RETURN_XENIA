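; BP_EulerPuzzel_NormalTile is a step-once floor tile for the Euler path puzzle.
; The first player overlap with its box marks it triggered and swaps its material; overlapping a triggered tile resets the level through BP_EulerPuzzel's spawn manager component and plays an error sound.
; ResetObjectState restores the untriggered, translucent state.
; The IsNotAvailable flag, true when ready despite its name, blocks repeat overlaps until the next tick.
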(event `self.ResetObjectState`
  (set `self.bIsTriggered` false)
  (`PrimitiveComponent.SetMaterial` (`self.SM_This`) 0 "/Game/Designer/Materials/MI_PuzzelTranslucent.MI_PuzzelTranslucent"))

(event `self.ReceiveBeginPlay`
  (set `self.bIsTriggered` false))

(event `self.Box.OnComponentBeginOverlap`
  (params (OverlappedComponent :type "PrimitiveComponent Object Reference") (OtherActor :type "Actor Object Reference") (OtherComp :type "PrimitiveComponent Object Reference") (OtherBodyIndex :type Integer) (bFromSweep :type Boolean) (SweepResult :type "HitResult Structure (by ref)"))
  (if (`self.bIsNotAvailable`)
    (`|ExecutionSequence`
      (:`then_0`
        (set `self.bIsNotAvailable` false)
        (`KismetSystemLibrary.PrintText` "Begin Overap occured!")
        (if (`self.bIsTriggered`)
          (bind _returnvalue (`GameplayStatics.GetActorOfClass` "/Game/Blueprints/Puzzel/EulerPuzzel/BP_EulerPuzzel.BP_EulerPuzzel_C"))
          ;[1 1 1] ResetCurrentLevel 함수는 모든 해당 레벨의 타일을 Initialize
          (`RXPuzzelSpawnManageComponent.ResetCurrentLevel` (`self.GetComponentByClass` _returnvalue "/Game/Blueprints/Puzzel/EulerPuzzel/BP_EulerPuzzelSpawnManageComponent.BP_EulerPuzzelSpawnManageComponent_C"))
          (`GameplayStatics.PlaySound2D` "/Game/Audio/SFX/Puzzel/SFX_CannotIneract.SFX_CannotIneract" 1.0 1.0 0.0 null null)
          (else
            (cast `RXPlayer` OtherActor)
            (`PrimitiveComponent.SetMaterial` (`self.SM_This`) 0 "/Game/Designer/Materials/MI_TemplePuzzel_A02.MI_TemplePuzzel_A02")
            (set `self.bIsTriggered` true))))
      (:`then_1`
        (`KismetSystemLibrary.DelayUntilNextTick`)
        (set `self.bIsNotAvailable` true)))))

(fn `UserConstructionScript`)
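; BP_EulerPuzzel is the Euler puzzle actor, handling the puzzle's start and finish events on top of a parent Blueprint.
; On start it runs the parent logic, then has its spawn-manage component activate level 1.
; On finish it destroys the event and spawn managers, the interaction visibility component and the invisible wall meshes, removing the puzzle's machinery once cleared.
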(event `self.PuzzelEventStart`
  ;[1 1 1] 오일러퍼즐이벤트 시작
  (`parent.PuzzelEventStart`)
  (`RXPuzzelSpawnManageComponent.ActivateLevel` (`self.BP_EulerPuzzelSpawnManageComponent`) 1))

(event `self.PuzzelEventFinish`
  ;[1 1 1] 퍼즐클리어시 관련 기능 컴포넌트 모두 삭제
  (`ActorComponent.K2_DestroyComponent` (`self.BP_PuzzelEventManageComponent`))
  (`ActorComponent.K2_DestroyComponent` (`self.BP_EulerPuzzelSpawnManageComponent`))
  (`ActorComponent.K2_DestroyComponent` (`self.RXInteractionVisibility`))
  (`ActorComponent.K2_DestroyComponent` (`self.SM_puzzel_InvisibleEdgeWall`))
  (`ActorComponent.K2_DestroyComponent` (`self.SM_puzzel_InvisibleWall`)))

(fn `UserConstructionScript`
  (`parent.UserConstructionScript`))
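; BP_Puzzel_NormalTile is a standard floor tile for the Euler puzzle that must not be stepped on twice.
; The first RXPlayer overlap of its Box marks it triggered and swaps the mesh material from translucent to navy.
; Any overlap while triggered, without a player check, calls ResetCurrentLevel on BP_EulerPuzzel's spawn manager component.
; ResetObjectState restores the untriggered flag and translucent material.
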(event `self.ReceiveBeginPlay`
  (set `self.IsTriggered` false))

(event `self.ResetObjectState`
  (set `self.IsTriggered` false)
  (`PrimitiveComponent.SetMaterial` (`self.SM_This`) 0 "/Game/Designer/Materials/MI_PuzzelTranslucent.MI_PuzzelTranslucent"))

(event `self.Box.OnComponentBeginOverlap`
  (params (OverlappedComponent :type "PrimitiveComponent Object Reference") (OtherActor :type "Actor Object Reference") (OtherComp :type "PrimitiveComponent Object Reference") (OtherBodyIndex :type Integer) (bFromSweep :type Boolean) (SweepResult :type "HitResult Structure (by ref)"))
  (if (`self.IsTriggered`)
    (bind _returnvalue (`GameplayStatics.GetActorOfClass` "/Game/Blueprints/Puzzel/EulerPuzzel/BP_EulerPuzzel.BP_EulerPuzzel_C"))
    ;[1 1 1] ResetCurrentLevel 함수는 모든 해당 레벨의 타일을 Initialize
    (`RXPuzzelSpawnManageComponent.ResetCurrentLevel` (`self.GetComponentByClass` _returnvalue "/Game/Blueprints/Puzzel/EulerPuzzel/BP_EulerPuzzelSpawnManageComponent.BP_EulerPuzzelSpawnManageComponent_C"))
    (else
      (cast `RXPlayer` OtherActor)
      (`PrimitiveComponent.SetMaterial` (`self.SM_This`) 0 "/Game/Designer/Materials/MI_Puzzel_Navy.MI_Puzzel_Navy")
      (set `self.IsTriggered` true))))

(fn `UserConstructionScript`)
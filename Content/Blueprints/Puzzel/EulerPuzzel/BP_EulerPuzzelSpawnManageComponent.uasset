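; Level manager component for the Euler puzzle, advancing through four levels as the coins in each are collected.
; IsGetAllCoins compares the coin count to the level's target set at BeginPlay, then activates the next level, resets the count and plays a fade-out widget.
; Completing level four ends puzzle mode through BP_EulerPuzzel's event component and records the clear in RXGameInstance.
; Targets are hardcoded and must match the coins placed per level.
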(event `IsGetAllCoins`
  (params (CurrentLevelID_Param :type Integer))
  (bind _fadewidget (`self.FadeWidget`))
  (bind _currentcoinnum (`self.CurrentCoinNum`))
  ;[1 1 1] 해당 레벨 코인을 다 획득했는지? 클리어조건
  (switch `int` CurrentLevelID_Param
    (:`1`
      (if (== (`self.Level1_TargetCoinNum`) _currentcoinnum)
        ;[1 1 1] 다음레벨로 이동
        (`self.ActivateLevel` 2)
        (set `self.CurrentCoinNum` 0 :!label _label)
        (`UserWidget.AddToViewport` _fadewidget 0)
        (`/Game/UI/WBP_FadeAnimWidget.PlayFadeOut` _fadewidget)))
    (:`2`
      (if (== (`self.Level2_TargetCoinNum`) _currentcoinnum)
        (`self.ActivateLevel` 3)
        (goto _label)))
    (:`3`
      (if (== (`self.Level3_TargetCoinNum`) _currentcoinnum)
        (`self.ActivateLevel` 4)
        (goto _label)))
    (:`4`
      (if (== (`self.Level4_TargetCoinNum`) _currentcoinnum)
        ;[1 1 1] 해당 퍼즐 레벨1~4 모두 완료 퍼즐 이벤트 종료
        (bind _returnvalue (`GameplayStatics.GetActorOfClass` "/Game/Blueprints/Puzzel/EulerPuzzel/BP_EulerPuzzel.BP_EulerPuzzel_C"))
        (`RXPuzzelEventManageComponent.EndPuzzelMode` (`Actor.GetComponentByClass` _returnvalue "/Game/Blueprints/Puzzel/BP_PuzzelEventManageComponent.BP_PuzzelEventManageComponent_C"))
        ;[1 1 1] 게임 인스턴스에 클리어 조건 상태 전달
        (bind _asrxgame_instance (cast `RXGameInstance` (`GameplayStatics.GetGameInstance`)))
        (`RXGameInstance.SetPuzzelStatusAcquired` _asrxgame_instance "EulerPuzzel")))))

(event `self.ReceiveBeginPlay`
  (set `self.CurrentLevelID` 1)
  (set `self.CurrentCoinNum` 0)
  ;[1 1 1] 해당 레벨의 목표 코인 갯수 설정 , 이 갯수와 동일하게 코인오브젝트를 배치해야함!
  (`|ExecutionSequence`
    (:`then_0`
      (set `self.Level1_TargetCoinNum` 1))
    (:`then_1`
      (set `self.Level2_TargetCoinNum` 2))
    (:`then_2`
      (set `self.Level3_TargetCoinNum` 3))
    (:`then_3`
      (set `self.Level4_TargetCoinNum` 4))))

(event `self.ResetCurrentLevel`
  (set `self.CurrentCoinNum` 0)
  (`parent.ResetCurrentLevel`))
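; Spawn manager that places the Nowiniq NPC variant matching a given puzzle at its own transform, cached on BeginPlay.
; SpawnNowiniq switches on the puzzle name, spawns that submap's NPC, destroys the matching referenced actor, then turns the new NPC toward the player.
; The Temple puzzle instead spawns the Pachamama temple NPC, without destroying anything or adjusting its facing.
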(event `LookPlayer`
  (params (Actor :type "Actor Object Reference"))
  (`self.K2_SetActorRotation` Actor (`KismetMathLibrary.FindLookAtRotation` (`self.K2_GetActorLocation`) (`self.K2_GetActorLocation` (`GameplayStatics.GetPlayerCharacter` 0))) false))

(event `self.ReceiveBeginPlay`
  (set `self.SpawnTransform` (`self.GetTransform`)))

(event `SpawnNowiniq`
  (params (PuzzelName :type Name))
  (switch `name` PuzzelName
    (:`PushablePuzzel`
      (bind _returnvalue (`|SpawnActorFromClass` "/Game/Blueprints/Characters/Nowiniq/BP_NPC_Nowiniq_Submap1.BP_NPC_Nowiniq_Submap1_C" (`self.SpawnTransform`) "AdjustIfPossibleButAlwaysSpawn" "MultiplyWithRoot" null null))
      (`self.K2_DestroyActor` (`self.RefSub1`))
      (`self.LookPlayer` _returnvalue))
    (:`BlindPuzzel`
      (bind _returnvalue_2 (`|SpawnActorFromClass` "/Game/Blueprints/Characters/Nowiniq/BP_NPC_Nowiniq_Submap2.BP_NPC_Nowiniq_Submap2_C" (`self.SpawnTransform`) "AdjustIfPossibleButAlwaysSpawn" "MultiplyWithRoot" null null))
      (`self.K2_DestroyActor` (`self.RefSub2`))
      (`self.LookPlayer` _returnvalue_2))
    (:`PatternPuzzel`
      (bind _returnvalue_3 (`|SpawnActorFromClass` "/Game/Blueprints/Characters/Nowiniq/BP_NPC_Nowiniq_Submap3.BP_NPC_Nowiniq_Submap3_C" (`self.SpawnTransform`) "AdjustIfPossibleButAlwaysSpawn" "MultiplyWithRoot" null null))
      (`self.K2_DestroyActor` (`self.RefSub3`))
      (`self.LookPlayer` _returnvalue_3))
    (:`TimingPuzzel`
      (bind _returnvalue_4 (`|SpawnActorFromClass` "/Game/Blueprints/Characters/Nowiniq/BP_NPC_Nowiniq_Submap4.BP_NPC_Nowiniq_Submap4_C" (`self.SpawnTransform`) "AdjustIfPossibleButAlwaysSpawn" "MultiplyWithRoot" null null))
      (`self.K2_DestroyActor` (`self.RefSub4`))
      (`self.LookPlayer` _returnvalue_4))
    (:`EulerPuzzel`
      (bind _returnvalue_5 (`|SpawnActorFromClass` "/Game/Blueprints/Characters/Nowiniq/BP_NPC_Nowiniq_Submap5.BP_NPC_Nowiniq_Submap5_C" (`self.SpawnTransform`) "AdjustIfPossibleButAlwaysSpawn" "MultiplyWithRoot" null null))
      (`self.K2_DestroyActor` (`self.RefSub5`))
      (`self.LookPlayer` _returnvalue_5))
    (:`TemplePuzzel`
      (`|SpawnActorFromClass` "/Game/Blueprints/Characters/BP_NPC_Pachamama_Temple.BP_NPC_Pachamama_Temple_C" (`self.SpawnTransform`) "AlwaysSpawn" "MultiplyWithRoot" null null))))

(fn `UserConstructionScript`)
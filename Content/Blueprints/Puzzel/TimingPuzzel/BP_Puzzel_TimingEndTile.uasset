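; BP_Puzzel_TimingEndTile is the end tile of the timing puzzle, checking for level completion when the player steps on it.
; It starts with a purple material and exposes events to switch between yellow (active) and purple (inactive).
; On box overlap by RXPlayer, it finds the BP_TimingPuzzel actor and asks its spawn-manager component whether all coins in the current level are collected, leaving the outcome to that component.
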(event `self.ReceiveBeginPlay`
  ;[1 1 1] DeActive->배경타일(보라색), Active->노란색
  (`self.SetDeActiveColor`))

(event `SetActiveColor`
  ;[1 1 1] DeActive->배경타일(보라색), Active->노란색
  (`PrimitiveComponent.SetMaterial` (`self.SM_This`) 0 "/Game/Designer/Materials/puzzel/MI_Puzzel_Yellow.MI_Puzzel_Yellow"))

(event `SetDeActiveColor`
  ;[1 1 1] DeActive->배경타일(보라색), Active->노란색
  (`PrimitiveComponent.SetMaterial` (`self.SM_This`) 0 "/Game/Designer/Materials/puzzel/MI_PuzzelPurple.MI_PuzzelPurple"))

(event `self.Box.OnComponentBeginOverlap`
  (params (OverlappedComponent :type "PrimitiveComponent Object Reference") (OtherActor :type "Actor Object Reference") (OtherComp :type "PrimitiveComponent Object Reference") (OtherBodyIndex :type Integer) (bFromSweep :type Boolean) (SweepResult :type "HitResult Structure (by ref)"))
  ;[1 1 1] 플레이어가 EndTile을 오버랩 하는 경우, 해당 레벨에서 모든코인을 획득한 경우에 컴포넌트를 통해서 함수 호출해줌
  (cast `RXPlayer` OtherActor)
  (bind _returnvalue (`GameplayStatics.GetActorOfClass` "/Game/Blueprints/Puzzel/TimingPuzzel/BP_TimingPuzzel.BP_TimingPuzzel_C"))
  (bind _returnvalue_2 (`self.GetComponentByClass` _returnvalue "/Game/Blueprints/Puzzel/TimingPuzzel/BP_TimingPuzzelSpawnManageComponent.BP_TimingPuzzelSpawnManageComponent_C"))
  (`/Engine/EditorBlueprintResources/StandardMacros.IsValid` _returnvalue_2
    (:`Is Valid`
      (`/Game/Blueprints/Puzzel/TimingPuzzel/BP_TimingPuzzelSpawnManageComponent.IsGetAllCoins` _returnvalue_2 (`RXPuzzelSpawnManageComponent.CurrentLevelID` _returnvalue_2)))))

(fn `UserConstructionScript`)
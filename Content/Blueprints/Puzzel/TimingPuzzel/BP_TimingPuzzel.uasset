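; BP_TimingPuzzel is the timing puzzle actor, handling the start, completion and saved-clear state of the puzzle.
; On BeginPlay it asks RXGameInstance whether "TimingPuzzel" is already acquired and, if so, destroys its invisible walls, event manager, interaction visibility and spawn manager components.
; Puzzle start activates level 1 on the spawn manager component and resets the current level.
; Puzzle finish destroys the same set of components.
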(event `self.ReceiveBeginPlay`
  (`parent.ReceiveBeginPlay`)
  (bind _asrxgame_instance (cast `RXGameInstance` (`GameplayStatics.GetGameInstance`)))
  (if (`RXGameInstance.IsPuzzelStatusAcquired` _asrxgame_instance "TimingPuzzel")
    (`ActorComponent.K2_DestroyComponent` (`self.SM_puzzel_InvisibleEdgeWall`))
    (`ActorComponent.K2_DestroyComponent` (`self.SM_puzzel_InvisibleWall`))
    (`ActorComponent.K2_DestroyComponent` (`self.BP_PuzzelEventManageComponent`))
    (`ActorComponent.K2_DestroyComponent` (`self.RXInteractionVisibility`))
    (`ActorComponent.K2_DestroyComponent` (`self.BP_TimingPuzzelSpawnManageComponent`))))

(event `self.PuzzelEventStart`
  (bind _bp_timingpuzzelspawnmanagecomponent (`self.BP_TimingPuzzelSpawnManageComponent`))
  ;[1 1 1] 블라인드퍼즐 이벤트 시작
  (`parent.PuzzelEventStart`)
  (`RXPuzzelSpawnManageComponent.ActivateLevel` _bp_timingpuzzelspawnmanagecomponent 1)
  (`RXPuzzelSpawnManageComponent.ResetCurrentLevel` _bp_timingpuzzelspawnmanagecomponent))

(event `self.PuzzelEventFinish`
  ;[1 1 1] 퍼즐클리어시 관련 기능 컴포넌트 모두 삭제
  (`ActorComponent.K2_DestroyComponent` (`self.SM_puzzel_InvisibleEdgeWall`))
  (`ActorComponent.K2_DestroyComponent` (`self.SM_puzzel_InvisibleWall`))
  (`ActorComponent.K2_DestroyComponent` (`self.BP_PuzzelEventManageComponent`))
  (`ActorComponent.K2_DestroyComponent` (`self.RXInteractionVisibility`))
  (`ActorComponent.K2_DestroyComponent` (`self.BP_TimingPuzzelSpawnManageComponent`)))

(fn `UserConstructionScript`
  (`parent.UserConstructionScript`))
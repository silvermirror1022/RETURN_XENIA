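; Timing-puzzle bomb tile that flips between a red bomb state and a purple safe state, resetting the current level when the player touches it while red.
; ResetObjectState starts a looping timer, intended to drive the toggle, if the level has not started.
; Begin-overlap resets through the spawn-manage component on BP_TimingPuzzel.
; Each state change rechecks overlapping players, but that path skips the bomb-state check, so switching to purple also resets.
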(event `self.ResetObjectState`
  (if (not (`self.bIsLevelStarted`))
    (`KismetSystemLibrary.K2_SetTimerDelegate` (`|CreateDelegate` :!event `ToggleEvent`) (`self.TickIntervalSec`) true)))

(event `self.ReceiveBeginPlay`
  (`self.SetDeActiveColor`))

(event `SetActiveColor`
  ;[1 1 1] Active-> 폭탄타일(빨강색),BombState On   /   DeActive-> 배경타일(보라색), BombState Non
  (`PrimitiveComponent.SetMaterial` (`self.SM_This`) 0 "/Game/Designer/Materials/MI_Puzzel_Red.MI_Puzzel_Red")
  (set `self.bIsBombState` true)
  (`self.CheckPlayerOverlapAgain`))

(event `SetDeActiveColor`
  ;[1 1 1] Active-> 폭탄타일(빨강색),BombState On   /   DeActive-> 배경타일(보라색), BombState Non
  (`PrimitiveComponent.SetMaterial` (`self.SM_This`) 0 "/Game/Designer/Materials/MI_PuzzelPurple.MI_PuzzelPurple")
  (set `self.bIsBombState` false)
  (`self.CheckPlayerOverlapAgain`))

(event `ToggleEvent`
  ;[1 1 1] TickIntervalSec마다 Tick될 ToggleEvent Fuction
  (if (`self.bIsBombState`)
    (`self.SetDeActiveColor`)
    (else
      (`self.SetActiveColor`))))

(event `self.Box.OnComponentBeginOverlap`
  (params (OverlappedComponent :type "PrimitiveComponent Object Reference") (OtherActor :type "Actor Object Reference") (OtherComp :type "PrimitiveComponent Object Reference") (OtherBodyIndex :type Integer) (bFromSweep :type Boolean) (SweepResult :type "HitResult Structure (by ref)"))
  ;[1 1 1] 플레이어가 Bomb상태의 타일을 오버랩 하는 경우, 해당 레벨에 해당하게 플레이어 Reset
  (cast `RXPlayer` OtherActor)
  (if (`self.bIsBombState`)
    (bind _returnvalue (`GameplayStatics.GetActorOfClass` "/Game/Blueprints/Puzzel/TimingPuzzel/BP_TimingPuzzel.BP_TimingPuzzel_C" :!label _label))
    (`RXPuzzelSpawnManageComponent.ResetCurrentLevel` (`self.GetComponentByClass` _returnvalue "/Game/Blueprints/Puzzel/TimingPuzzel/BP_TimingPuzzelSpawnManageComponent.BP_TimingPuzzelSpawnManageComponent_C"))))

(event `CheckPlayerOverlapAgain`
  ;[1 1 1] 플레이어가 오버랩되어 이미 타일을 밝는 예외 상황 처리 함수
  (for _array_element (`PrimitiveComponent.GetOverlappingActors` (`self.Box`) "/Game/Blueprints/Player/BP_Player.BP_Player_C")
    (cast `RXPlayer` _array_element)
    (goto _label)))

(fn `UserConstructionScript`)
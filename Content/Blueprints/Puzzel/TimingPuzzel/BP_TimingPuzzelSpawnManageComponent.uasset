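; Level manager component for the four-stage timing puzzle, where collecting each level's target coin count advances the player.
; Clearing a level activates the next, fades the screen, then resets via the parent logic with a brief input lock.
; Reset also arms the current level's bomb tiles, found by actor tag.
; Clearing the last level ends puzzle mode and records "TimingPuzzel" completion in RXGameInstance.
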(event `DisablePlayerInput`
  (bind _returnvalue (`GameplayStatics.GetPlayerPawn` 0))
  (bind _returnvalue_2 (`GameplayStatics.GetPlayerController` 0))
  (`Actor.DisableInput` _returnvalue _returnvalue_2)
  (`KismetSystemLibrary.Delay` 1.5)
  (`Actor.EnableInput` _returnvalue _returnvalue_2))

(event `IsGetAllCoins`
  (params (CurrentLevelID_Param :type Integer))
  (bind _fadewidget (`self.FadeWidget`))
  (bind _currentcoinnum (`self.CurrentCoinNum`))
  ;[1 1 1] 해당 레벨 코인을 다 획득했는지? 클리어조건
  (switch `int` CurrentLevelID_Param
    (:`1`
      (if (== (`self.Level1_TargetCoinNum`) _currentcoinnum)
        ;[1 1 1] 다음레벨로 이동
        (`self.ActivateLevel` 2)
        (set `self.CurrentCoinNum` 0 :!label _label)
        (`UserWidget.AddToViewport` _fadewidget 0)
        (`/Game/UI/WBP_FadeAnimWidget.PlayFadeOut` _fadewidget)
        (`self.ResetCurrentLevel`)))
    (:`2`
      (if (== (`self.Level2_TargetCoinNum`) _currentcoinnum)
        (`self.ActivateLevel` 3)
        (goto _label)))
    (:`3`
      (if (== (`self.Level3_TargetCoinNum`) _currentcoinnum)
        (`self.ActivateLevel` 4)
        (goto _label)))
    (:`4`
      (if (== (`self.Level4_TargetCoinNum`) _currentcoinnum)
        (`RXPuzzelEventManageComponent.EndPuzzelMode` (`Actor.GetComponentByClass` (`self.GetOwner`) "/Game/Blueprints/Puzzel/BP_PuzzelEventManageComponent.BP_PuzzelEventManageComponent_C"))
        ;[1 1 1] 게임 인스턴스에 클리어 조건 상태 전달
        (bind _asrxgame_instance (cast `RXGameInstance` (`GameplayStatics.GetGameInstance`)))
        (`RXGameInstance.SetPuzzelStatusAcquired` _asrxgame_instance "TimingPuzzel")))))

(event `self.ReceiveBeginPlay`
  (set `self.CurrentLevelID` 1)
  (set `self.CurrentCoinNum` 0)
  ;[1 1 1] 해당 레벨의 목표 코인 갯수 설정 , 이 갯수와 동일하게 코인오브젝트를 배치해야함!
  (`|ExecutionSequence`
    (:`then_0`
      (set `self.Level1_TargetCoinNum` 2))
    (:`then_1`
      (set `self.Level2_TargetCoinNum` 3))
    (:`then_2`
      (set `self.Level3_TargetCoinNum` 4))
    (:`then_3`
      (set `self.Level4_TargetCoinNum` 6))))

(event `self.ResetCurrentLevel`
  (set `self.CurrentCoinNum` 0)
  (`parent.ResetCurrentLevel`)
  (`self.DisablePlayerInput`)
  (`self.CheckLevelState`))

(event `CheckLevelState`
  ;[1 1 1] 해당 Level이 시작됨을 체크해주는 함수 : 각 BombTile 에 변수를 SET해 Branch 체크로 활용함
  (switch `int` (`self.CurrentLevelID`)
    (:`1`
      (bind _outactors (`GameplayStatics.GetAllActorsWithTag` "TimingPuzzelLevel1"))
      (for _array_element _outactors
        (bind _asbp_puzzel_timing_bomb_tile (cast `/Game/Blueprints/Puzzel/TimingPuzzel/BP_Puzzel_TimingBombTile` _array_element))
        (set `/Game/Blueprints/Puzzel/TimingPuzzel/BP_Puzzel_TimingBombTile.bIsLevelStarted` true _asbp_puzzel_timing_bomb_tile)))
    (:`2`
      (bind _outactors_2 (`GameplayStatics.GetAllActorsWithTag` "TimingPuzzelLevel2"))
      (for _array_element_2 _outactors_2
        (bind _asbp_puzzel_timing_bomb_tile_2 (cast `/Game/Blueprints/Puzzel/TimingPuzzel/BP_Puzzel_TimingBombTile` _array_element_2))
        (set `/Game/Blueprints/Puzzel/TimingPuzzel/BP_Puzzel_TimingBombTile.bIsLevelStarted` true _asbp_puzzel_timing_bomb_tile_2)))
    (:`3`
      (bind _outactors_3 (`GameplayStatics.GetAllActorsWithTag` "TimingPuzzelLevel3"))
      (for _array_element_3 _outactors_3
        (bind _asbp_puzzel_timing_bomb_tile_3 (cast `/Game/Blueprints/Puzzel/TimingPuzzel/BP_Puzzel_TimingBombTile` _array_element_3))
        (set `/Game/Blueprints/Puzzel/TimingPuzzel/BP_Puzzel_TimingBombTile.bIsLevelStarted` true _asbp_puzzel_timing_bomb_tile_3)))
    (:`4`
      (bind _outactors_4 (`GameplayStatics.GetAllActorsWithTag` "TimingPuzzelLevel4"))
      (for _array_element_4 _outactors_4
        (bind _asbp_puzzel_timing_bomb_tile_4 (cast `/Game/Blueprints/Puzzel/TimingPuzzel/BP_Puzzel_TimingBombTile` _array_element_4))
        (set `/Game/Blueprints/Puzzel/TimingPuzzel/BP_Puzzel_TimingBombTile.bIsLevelStarted` true _asbp_puzzel_timing_bomb_tile_4)))))
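; Puzzle event manager component that switches the player into and out of puzzle mode, extending a C++ parent that handles camera and player state.
; On BeginPlay it creates a fade widget and finds the level's start and end tiles by class.
; Starting swaps Enhanced Input to the puzzle mapping context, plays the fade and highlights both tiles.
; Ending restores default input, fades, destroys both tiles and notifies the owning BP_Puzzel_Parent.
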(event `self.ReceiveBeginPlay`
  ;[1 1 1] 쓰일 변수들 초기화 페이드위젯, 타일들
  (bind _returnvalue (`|CreateWidget` "/Game/UI/WBP_FadeAnimWidget.WBP_FadeAnimWidget_C"))
  (set `self.FadeWiget` _returnvalue)
  (bind _returnvalue_2 (`GameplayStatics.GetActorOfClass` "/Game/Blueprints/Puzzel/BP_Puzzel_StartTile.BP_Puzzel_StartTile_C"))
  (set `self.PuzzelStartTile` _returnvalue_2)
  (bind _returnvalue_3 (`GameplayStatics.GetActorOfClass` "/Game/Blueprints/Puzzel/BP_Puzzel_EndTile.BP_Puzzel_EndTile_C"))
  (set `self.PuzzelEndTile` _returnvalue_3))

(event `self.StartPuzzelMode`
  (bind _fadewiget (`self.FadeWiget`))
  ;[1 1 1] 퍼즐모드 시작 : BlueprintNativeEvent
  (bind _asrxplayer_controller (cast `RXPlayerController` (`GameplayStatics.GetPlayerController` 0)))
  (bind _returnvalue (pcsubsystem `EnhancedInputLocalPlayerSubsystem` _asrxplayer_controller))
  ;[1 1 1] 컨트롤러 퍼즐전용으로 교체
  (`EnhancedInputSubsystemInterface.RemoveMappingContext` _returnvalue "/Game/Input/IMC_Default.IMC_Default" (struct))
  (`EnhancedInputSubsystemInterface.AddMappingContext` _returnvalue "/Game/Input/IMC_Puzzel.IMC_Puzzel" 0 (struct))
  ;[1 1 1] 페이드이벤트발생
  (`UserWidget.AddToViewport` _fadewiget 0)
  (`/Game/UI/WBP_FadeAnimWidget.PlayFadeOut` _fadewiget)
  ;[1 1 1] CPP 부모호출 : 카메라셋팅, 플레이어 퍼즐이벤트 진입
  (`parent.StartPuzzelMode`)
  ;[1 1 1] 퍼즐이벤트 시작 : 퍼즐시작, 종료타일 색 활성화
  (`/Game/Blueprints/Puzzel/BP_Puzzel_StartTile.SetActiveColor` (`self.PuzzelStartTile`))
  (`/Game/Blueprints/Puzzel/BP_Puzzel_EndTile.SetActiveColor` (`self.PuzzelEndTile`)))

(event `self.EndPuzzelMode`
  (bind _fadewiget (`self.FadeWiget`))
  ;[1 1 1] 퍼즐모드 해제 : BlueprintNativeEvent
  (bind _asrxplayer_controller (cast `RXPlayerController` (`GameplayStatics.GetPlayerController` 0)))
  (bind _returnvalue (pcsubsystem `EnhancedInputLocalPlayerSubsystem` _asrxplayer_controller))
  (`EnhancedInputSubsystemInterface.RemoveMappingContext` _returnvalue "/Game/Input/IMC_Puzzel.IMC_Puzzel" (struct))
  (`EnhancedInputSubsystemInterface.AddMappingContext` _returnvalue "/Game/Input/IMC_Default.IMC_Default" 0 (struct))
  (`UserWidget.AddToViewport` _fadewiget 0)
  (`/Game/UI/WBP_FadeAnimWidget.PlayFadeOut` _fadewiget)
  ;[1 1 1] CPP 부모호출 : 카메라셋팅, 플레이어 퍼즐이벤트 진입해제
  (`parent.EndPuzzelMode`)
  ;[1 1 1] 퍼즐이벤트 종료 : 퍼즐시작, 종료타일 삭제
  (`Actor.K2_DestroyActor` (`self.PuzzelStartTile`))
  (`Actor.K2_DestroyActor` (`self.PuzzelEndTile`))
  (bind _asbp_puzzel_parent (cast `/Game/Blueprints/Puzzel/BP_Puzzel_Parent` (`self.GetOwner`)))
  (`RXPuzzelBase.PuzzelEventFinish` _asbp_puzzel_parent))
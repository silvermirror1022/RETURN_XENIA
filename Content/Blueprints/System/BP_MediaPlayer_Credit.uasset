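; BP_MediaPlayer_Credit switches the sound between a movie and two audio components, apparently for the credits, judging by its name.
; PlayMovieSound binds the MediaPlayer to the MediaSound component, starts it and stops both audio components.
; StopMovieSound rebinds the player, stops MediaSound and fades both audio components back in.
; BeginPlay and the construction script are empty, so both events rely on outside callers.
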(event `self.ReceiveBeginPlay`)

(event `StopMovieSound`
  (`MediaSoundComponent.SetMediaPlayer` (`self.MediaSound`) (`self.MediaPlayer`))
  (`SynthComponent.Stop` (`self.MediaSound`))
  (`AudioComponent.FadeIn` (`self.Audio1`) 1.0 1.0 0.0 "Linear")
  (`AudioComponent.FadeIn` (`self.Audio`) 1.0 1.0 0.0 "Linear"))

(event `PlayMovieSound`
  ;[1 1 1] When Playing Movie, Excute Music Player To Media Sound
  (`MediaSoundComponent.SetMediaPlayer` (`self.MediaSound`) (`self.MediaPlayer`))
  (`SynthComponent.Start` (`self.MediaSound`))
  (`AudioComponent.Stop` (`self.Audio1`))
  (`AudioComponent.Stop` (`self.Audio`)))

(fn `UserConstructionScript`)
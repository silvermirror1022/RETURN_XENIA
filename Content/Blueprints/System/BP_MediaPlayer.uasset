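; BP_MediaPlayer is a system Blueprint that plays selected movies in full widgets with their audio.
; PlayInMenuWidget serves the main menu, while PlayWithWidget uses a Nonstop widget variant that, per its comment, lacks the menu's Back option.
; Both add their widget to the viewport, pass it the MovieList selection and start sound.
; Sound start and stop events bind the MediaPlayer to MediaSound before acting.
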(event `StopMovieSound`
  (`MediaSoundComponent.SetMediaPlayer` (`self.MediaSound`) (`self.MediaPlayer`))
  (`SynthComponent.Stop` (`self.MediaSound`)))

(event `PlayMovieSound`
  ;[1 1 1] When Playing Movie, Excute Music Player To Media Sound
  (`MediaSoundComponent.SetMediaPlayer` (`self.MediaSound`) (`self.MediaPlayer`))
  (`SynthComponent.Start` (`self.MediaSound`)))

(event `PlayWithWidget`
  (params (MovieList :type "/Game/Movies/E_MovieList Enum" :default "NewEnumerator0"))
  (bind _mediaplayerwidget_nonstop (`self.MediaPlayerWidget_Nonstop`))
  ;[1 1 1] 동적으로 접근하여 첫 메모리 출력함수 (메뉴창은 Back 존재) Here No
  (`UserWidget.AddToViewport` _mediaplayerwidget_nonstop 0)
  (`/Game/UI/WBP_MediaPlayer_NonStop.PlaySelectedMovie` _mediaplayerwidget_nonstop MovieList)
  (`self.PlayMovieSound`))

(event `PlayInMenuWidget`
  (params (`Movie List` :type "/Game/Movies/E_MovieList Enum" :default "NewEnumerator0"))
  (bind _mediaplayerwidget (`self.MediaPlayerWidget`))
  ;[1 1 1] 메인메뉴창에서 위젯 플레이하는 노드 함수
  (`UserWidget.AddToViewport` _mediaplayerwidget 0)
  (`/Game/UI/WBP_MediaPlayer.PlaySelectedMovie` _mediaplayerwidget `Movie List`)
  (`self.PlayMovieSound`))

(fn `UserConstructionScript`)
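; BP_Player is the player Blueprint, adding an unlockable red cloak appearance on top of its parent class.
; On BeginPlay it runs the parent logic, then asks RXGameInstance whether the "RedCloak" profile status is acquired.
; If so, it swaps in cape and hat materials on the ChaosCloth component and two Mesh material slots.
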(event `self.ReceiveBeginPlay`
  (`parent.ReceiveBeginPlay`)
  (bind _asrxgame_instance (cast `RXGameInstance` (`GameplayStatics.GetGameInstance`)))
  (if (`RXGameInstance.IsProfileStatusAcquired` _asrxgame_instance "RedCloak")
    (`PrimitiveComponent.SetMaterial` (`self.ChaosCloth`) 0 "/Game/Designer/Materials/MI_cape_A01.MI_cape_A01")
    (`PrimitiveComponent.SetMaterial` (`self.Mesh`) 1 "/Game/Designer/Materials/MI_NoahHat_A01.MI_NoahHat_A01")
    (`PrimitiveComponent.SetMaterial` (`self.Mesh`) 2 "/Game/Designer/Materials/MI_cape_A01.MI_cape_A01")))

(fn `UserConstructionScript`)
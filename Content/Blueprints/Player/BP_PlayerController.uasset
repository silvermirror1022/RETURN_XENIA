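; Player controller Blueprint that sets up player input and handles the reset after the player dies in a boss map.
; On BeginPlay it switches to game-only input and adds the IMC_Default Enhanced Input mapping context to player controller 0, cast to RXPlayerController.
; ResetPlayerInBossMap waits briefly, async loads the BossBeforeBattle asset, then opens that level using the loaded asset's display name.
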(event `ResetPlayerInBossMap`
  ;[1 1 1] 보스맵에서 플레이어 사망시 호출 함수
  (`KismetSystemLibrary.Delay` 2.0)
  (bind _object (`|LoadAsset` "/Game/Maps/BossMaps/BossBeforeBattle.BossBeforeBattle")
    (:`Completed`
      (`GameplayStatics.OpenLevel` (`KismetStringLibrary.Conv_StringToName` (`KismetSystemLibrary.GetDisplayName` _object))))))

(event `self.ReceiveBeginPlay`
  (`WidgetBlueprintLibrary.SetInputMode_GameOnly` self)
  (bind _asrxplayer_controller (cast `RXPlayerController` (`GameplayStatics.GetPlayerController` 0)))
  (`EnhancedInputSubsystemInterface.AddMappingContext` (pcsubsystem `EnhancedInputLocalPlayerSubsystem` _asrxplayer_controller) "/Game/Input/IMC_Default.IMC_Default" 0 (struct)))

(fn `UserConstructionScript`)
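; Trigger volume that switches the player's footsteps to water while they are inside it.
; Box overlap events cast the actor to RXPlayer, then set FootstepType on its ABP_Player anim instance to Water on begin overlap.
; End overlap always sets it to Dirt rather than restoring the previous surface type.
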(event `self.Box.OnComponentBeginOverlap`
  (params (OverlappedComponent :type "PrimitiveComponent Object Reference") (OtherActor :type "Actor Object Reference") (OtherComp :type "PrimitiveComponent Object Reference") (OtherBodyIndex :type Integer) (bFromSweep :type Boolean) (SweepResult :type "HitResult Structure (by ref)"))
  (bind _asrxplayer (cast `RXPlayer` OtherActor))
  (bind _asabp_player (cast `/Game/Animation/Player/ABP_Player` (`SkeletalMeshComponent.GetAnimInstance` (`Character.Mesh` _asrxplayer))))
  (set `/Game/Animation/Player/ABP_Player.FootstepType` "Water" _asabp_player))

(event `self.Box.OnComponentEndOverlap`
  (params (OverlappedComponent :type "PrimitiveComponent Object Reference") (OtherActor :type "Actor Object Reference") (OtherComp :type "PrimitiveComponent Object Reference") (OtherBodyIndex :type Integer))
  (bind _asrxplayer (cast `RXPlayer` OtherActor))
  (bind _asabp_player (cast `/Game/Animation/Player/ABP_Player` (`SkeletalMeshComponent.GetAnimInstance` (`Character.Mesh` _asrxplayer))))
  (set `/Game/Animation/Player/ABP_Player.FootstepType` "Dirt" _asabp_player))

(fn `UserConstructionScript`)
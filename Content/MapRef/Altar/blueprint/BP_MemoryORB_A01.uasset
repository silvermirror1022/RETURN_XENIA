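; BP_MemoryORB_A01 is a memory orb pickup that stays hidden until dropped.
; BeginPlay hides the sphere and collision components, and the droporb event shows them and sets the sphere's scale from the OrbScale timeline track, though that timeline is never run.
; An overlap that passes a cast, apparently to the main character, destroys the orb, creates a widget, calls RemoveVideo on it, adds it to the viewport and prints debug text.
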(event OnComponentBeginOverlap(colision)
  (params (OverlappedComponent :type Primitive%20Component%20Object%20Reference) (OtherActor :type Actor%20Object%20Reference) (OtherComp :type Primitive%20Component%20Object%20Reference) (OtherBodyIndex :type Integer) (bFromSweep :type Boolean) (SweepResult :type Hit%20Result%20Structure%20%28by%20ref%29))
  (bind _asbp_maincharacter (Utilities|Casting|CastTo OtherActor))
  (Variables|Default|SetAs%20BP%20Maincharacter 0 _asbp_maincharacter)
  (Actor|DestroyActor)
  (bind _returnvalue (UserInterface|CreateWidget 0))
  (CallFunction|RemoveVideo _returnvalue)
  (UserInterface|Viewport|AddtoViewport _returnvalue 0)
  (Development|PrintText "Hello"))

(event Custom|drop%20orb
  (bind _sphere (Variables|Default|GetSphere))
  (Rendering|SetVisibility _sphere true false)
  (Transformation|SetRelativeScale3D _sphere (Math|Conversions|ToVector(Float) (stale _새_트랙_0))))

(event EventBeginPlay
  (Rendering|SetVisibility (Variables|Default|GetSphere) false false))

(fn ConstructionScript)
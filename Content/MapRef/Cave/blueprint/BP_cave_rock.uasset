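; Cave rock puzzle actor whose step meshes move vertically when the player enters their trigger boxes.
; Box1, Box2 and Box3 each play a box-move sound and a timeline that drives SMStep2, SMStep3 and SMStep4 respectively toward fixed relative heights.
; Each update lerps from the step's current Z rather than a cached start, so motion compounds, and a timeline event plays the rock-move sound.
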(event `self.Box1.OnComponentBeginOverlap`
  (params (OverlappedComponent :type "PrimitiveComponent Object Reference") (OtherActor :type "Actor Object Reference") (OtherComp :type "PrimitiveComponent Object Reference") (OtherBodyIndex :type Integer) (bFromSweep :type Boolean) (SweepResult :type "HitResult Structure (by ref)"))
  (bind _sm_step2 (`self.SM_Step2`))
  (bind _returnvalue (`SceneComponent.GetRelativeTransform` _sm_step2))
  (cast `RXPlayer` OtherActor)
  (`GameplayStatics.PlaySound2D` "/Game/Audio/SFX/Puzzel/SFX_PuzzleBoxMove.SFX_PuzzleBoxMove" 1.0 1.0 0.0 null null)
  (bind (_direction _float) (`Timeline|Timeline`)
    (:`Update`
      (`SceneComponent.K2_SetRelativeLocation` _sm_step2 (`KismetMathLibrary.MakeVector` (.x (.location _returnvalue)) (.y (.location _returnvalue)) (`KismetMathLibrary.Lerp` (.z (.location _returnvalue)) 100.0 _float)) false false))
    (:`Event`
      (`GameplayStatics.PlaySound2D` "/Game/Audio/SFX/SFX_MoveRock.SFX_MoveRock" 1.0 1.0 0.0 null null))))

(event `self.Box2.OnComponentBeginOverlap`
  (params (OverlappedComponent :type "PrimitiveComponent Object Reference") (OtherActor :type "Actor Object Reference") (OtherComp :type "PrimitiveComponent Object Reference") (OtherBodyIndex :type Integer) (bFromSweep :type Boolean) (SweepResult :type "HitResult Structure (by ref)"))
  (bind _sm_step3 (`self.SM_Step3`))
  (bind _returnvalue (`SceneComponent.GetRelativeTransform` _sm_step3))
  (cast `RXPlayer` OtherActor)
  (`GameplayStatics.PlaySound2D` "/Game/Audio/SFX/Puzzel/SFX_PuzzleBoxMove.SFX_PuzzleBoxMove" 1.0 1.0 0.0 null null)
  (bind (_direction _float) (`Timeline|Timeline_0`)
    (:`Update`
      (`SceneComponent.K2_SetRelativeLocation` _sm_step3 (`KismetMathLibrary.MakeVector` (.x (.location _returnvalue)) (.y (.location _returnvalue)) (`KismetMathLibrary.Lerp` (.z (.location _returnvalue)) 500.0 _float)) false false))
    (:`Event`
      (`GameplayStatics.PlaySound2D` "/Game/Audio/SFX/SFX_MoveRock.SFX_MoveRock" 1.0 1.0 0.0 null null))))

(event `self.Box3.OnComponentBeginOverlap`
  (params (OverlappedComponent :type "PrimitiveComponent Object Reference") (OtherActor :type "Actor Object Reference") (OtherComp :type "PrimitiveComponent Object Reference") (OtherBodyIndex :type Integer) (bFromSweep :type Boolean) (SweepResult :type "HitResult Structure (by ref)"))
  (bind _sm_step4 (`self.SM_Step4`))
  (bind _returnvalue (`SceneComponent.GetRelativeTransform` _sm_step4))
  (cast `RXPlayer` OtherActor)
  (`GameplayStatics.PlaySound2D` "/Game/Audio/SFX/Puzzel/SFX_PuzzleBoxMove.SFX_PuzzleBoxMove" 1.0 1.0 0.0 null null)
  (bind (_direction _float) (`Timeline|Timeline_1`)
    (:`Update`
      (`SceneComponent.K2_SetRelativeLocation` _sm_step4 (`KismetMathLibrary.MakeVector` (.x (.location _returnvalue)) (.y (.location _returnvalue)) (`KismetMathLibrary.Lerp` (.z (.location _returnvalue)) 700.0 _float)) false false))
    (:`Event`
      (`GameplayStatics.PlaySound2D` "/Game/Audio/SFX/SFX_MoveRock.SFX_MoveRock" 1.0 1.0 0.0 null null))))

(fn `UserConstructionScript`)